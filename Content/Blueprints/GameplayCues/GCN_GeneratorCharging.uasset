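; Gameplay cue notify that handles the looping audio for generator charging.
; When applied, it finds a BP_Generator via GetActorOfClass rather than the cue target, spawns a sound attached to its root, stores the audio component and prints a debug message.
; On removal, it stops and destroys that component if valid, then clears the reference.
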(event EventOnApplication
  (params (Target :type Actor%20Object%20Reference) (Parameters :type Gameplay%20Cue%20Parameters%20Structure%20%28by%20ref%29) (SpawnResults :type Gameplay%20Cue%20Notify%20Spawn%20Result%20Structure%20%28by%20ref%29))
  (bind _returnvalue (Actor|GetActorOfClass 0 "/Game/Blueprints/Systems/BP_Generator.BP_Generator_C"))
  (bind _returnvalue_2 (Audio|SpawnSoundAttached 0 (Variables|/Script/Engine.Actor|GetRootComponent _returnvalue) "None" "0, 0, 0" "0, 0, 0" "KeepRelativeOffset" false 1.0 1.0 0.0 0 0 false))
  (Variables|Default|SetGenChargeLoopAudioComponent _returnvalue_2)
  (Development|PrintString 0 "Loop start" true true "(R=0.000000,G=1.000000,B=0.450759,A=1.000000)"))

(event EventOnLoopingStart
  (params (Target :type Actor%20Object%20Reference) (Parameters :type Gameplay%20Cue%20Parameters%20Structure%20%28by%20ref%29) (SpawnResults :type Gameplay%20Cue%20Notify%20Spawn%20Result%20Structure%20%28by%20ref%29)))

(event EventOnRecurring
  (params (Target :type Actor%20Object%20Reference) (Parameters :type Gameplay%20Cue%20Parameters%20Structure%20%28by%20ref%29) (SpawnResults :type Gameplay%20Cue%20Notify%20Spawn%20Result%20Structure%20%28by%20ref%29)))

(event EventOnRemoval
  (params (Target :type Actor%20Object%20Reference) (Parameters :type Gameplay%20Cue%20Parameters%20Structure%20%28by%20ref%29) (SpawnResults :type Gameplay%20Cue%20Notify%20Spawn%20Result%20Structure%20%28by%20ref%29))
  (Utilities|IsValid (Variables|Default|GetGenChargeLoopAudioComponent)
    (:Is%20Valid
      (Audio|Components|Audio|Stop (Variables|Default|GetGenChargeLoopAudioComponent))
      (Components|DestroyComponent (Variables|Default|GetGenChargeLoopAudioComponent))
      (Variables|Default|SetGenChargeLoopAudioComponent 0))))

(fn ConstructionScript)