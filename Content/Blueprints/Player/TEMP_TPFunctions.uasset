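; Temporary player Blueprint holding teleport functions that glide the character between two points while hidden, like a dash.
; StartTeleportLerp hides the body components, plays dash audio and starts a fast looping timer instead of using Tick.
; Each timer call runs PerformTeleport, which advances elapsed time and lerps actor location without sweep.
; At full alpha it restores visibility, plays landing audio and clears the timer; elapsed time is not reset here.
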(event Custom|StartTeleportLerp
  (params (TP_StartLocation :type Vector) (TP_TargetLocation :type Vector))
  ;[0 0.7865 0.1973 0.5] Handle teleport lerp
  (CallFunction|SetTeleportHidden true)
  (Audio|Components|Audio|Play (Variables|Default|GetDashAudio) 0.0)
  (bind _returnvalue (Utilities|Time|SetTimerbyEvent (delegate Custom|UpdateTPLerp) 0.01 true))
  (Variables|Default|SetTP_TimerHandle _returnvalue))

(event Custom|UpdateTPLerp
  ;[0 0.7865 0.1973 0.5] Handle teleport lerp
  (CallFunction|PerformTeleport (stale Custom|StartTeleportLerp TP_StartLocation) (stale Custom|StartTeleportLerp TP_TargetLocation)))

(event EventBeginPlay)

(event Collision|EventActorBeginOverlap
  (params (OtherActor :type Actor%20Object%20Reference)))

(event EventTick
  (params (DeltaSeconds :type Float%20%28single-precision%29)))

(fn ConstructionScript)

(fn SetTeleportHidden
  (params (IsHidden :type Boolean))
  (if IsHidden
    (Rendering|SetVisibility (Variables|Character|GetMesh) false false)
    (Rendering|SetVisibility (Variables|Default|GetBoosters) false false)
    (Rendering|SetVisibility (Variables|Default|GetThermon) false false)
    (Rendering|SetVisibility (Variables|Default|GetSpringArm) false false)
    (Rendering|SetVisibility (Variables|Collision|GetCapsuleComponent) false false)
    (else
      (Rendering|SetVisibility (Variables|Character|GetMesh) true false)
      (Rendering|SetVisibility (Variables|Default|GetBoosters) true false)
      (Rendering|SetVisibility (Variables|Default|GetThermon) true false)
      (Rendering|SetVisibility (Variables|Default|GetSpringArm) true false)
      (Rendering|SetVisibility (Variables|Collision|GetCapsuleComponent) true false))))

(fn PerformTeleport
  (params (StartLocation :type Vector) (TargetLocation :type Vector))
  (Variables|Default|SetTeleportElapsedTime (+ (Variables|Default|GetTeleportElapsedTime) (Variables|Default|GetTeleportUpdateRate)))
  (Variables|Default|SetAlpha (/ (Variables|Default|GetTeleportElapsedTime) (Variables|Default|GetTeleportDuration)))
  (Transformation|SetActorLocation (Math|Vector|Lerp(Vector) StartLocation TargetLocation (Math|Float|Clamp(Float) (/ (Variables|Default|GetTeleportElapsedTime) (Variables|Default|GetTeleportDuration)))) false false)
  (if (>= (Variables|Default|GetAlpha) 1.0)
    (CallFunction|SetTeleportHidden false)
    ;[0.15 0.15 0.15 0.5] TP SFX
    (Audio|Components|Audio|Play (Variables|Default|GetLandingAudio) 0.0)
    (Utilities|Time|ClearandInvalidateTimerbyHandle (Variables|Default|GetTP_TimerHandle))))