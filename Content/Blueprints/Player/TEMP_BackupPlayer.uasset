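; Player character Blueprint (named as a temp backup) for action combat built on the Gameplay Ability System.
; Enhanced Input drives movement, camera, jump, dash and UI; BeginPlay grants abilities and initializes health and heat drain.
; Hitbox callbacks deal damage via effects, launch the player and add heat on enemy hits.
; It also manages slotted pickup abilities, enemy tokens, death-to-menu, and overlay-material flashes stepped by delayed re-triggering events.
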(event Custom|Event_ControlMaterialFlash
  ;[0.15 0.15 0.15 0.5] Control color change on hit
  (if (Variables|Default|GetFadeIn)
    (CallFunction|ColorFlashonHit)
    (Utilities|FlowControl|Delay 0.05)
    (CallFunction|EventControlMaterialFlash)
    (else
      (CallFunction|ColorFlashonHit)
      (Utilities|FlowControl|Delay 0.05)
      (if (Variables|Default|GetFade%20in%20Progress)
        (CallFunction|EventControlMaterialFlash)))))

(event Custom|HitboxHitActorsDelegate_Event
  (params (HitActors :type Array%20of%20Actor%20Object%20References) (HitboxData :type Hitbox%20Data%20Structure))
  ;[0.15 0.15 0.15 0.5] Bind on Hit Events
  (for _array_element HitActors
    (CallFunction|HitActor _array_element HitboxData)))

(event Custom|Event_PlayerDeath
  ;[0.1071 0.06027 0.15 0.5] Player death
  (CallFunction|ActivateHitFeedback)
  (bind _hasdied (CallFunction|CheckforDeath))
  (if _hasdied
    (Utilities|FlowControl|Delay 3.0) ; Delay loading menu to allow for other events to conduct
    (Game|OpenLevel(byObjectReference) "/Game/Maps/Build/MenuScene.MenuScene")))

(event Custom|Event_UpgradeEffect
  ;[0.15 0.15 0.15 0.5] Upgrade Effect
  (if (Variables|Default|GetEquipEffectFadeIn)
    (CallFunction|EquipEffectGlow)
    (Utilities|FlowControl|Delay 0.05)
    (CallFunction|EventUpgradeEffect)
    (else
      (CallFunction|EquipEffectGlow)
      (Utilities|FlowControl|Delay 0.05)
      (if (Variables|Default|GetEquipEffectFadeInProgress)
        (CallFunction|EventUpgradeEffect)))))

(event Input|EnhancedActionEvents|EnhancedInputActionIA_MoveForward
  (params (ActionValue :type Float%20%28double-precision%29) (ElapsedSeconds :type Float%20%28double-precision%29) (TriggeredSeconds :type Float%20%28double-precision%29) (InputAction :type Input%20Action%20Object%20Reference :default "/Game/Inputs/IA_MoveForward.IA_MoveForward"))
  ;[0.09152 0.15 0.07935 0.5] Movement
  (:Triggered
    (if (not (GameplayTags|HasAnyMatchingGameplayTags (Variables|Default|GetPlayerAbilitySystemComp) (Variables|Default|GetHeavyAttackTags))) :!label _label
      (Pawn|Input|AddMovementInput (Math|Vector|GetForwardVector (Math|Rotator|MakeRotator 0.0 0.0 (.yaw (Pawn|GetControlRotation :!class /Script/Engine.Pawn)))) ActionValue false)))
  (:Ongoing
    (goto _label)))

(event Input|EnhancedActionEvents|EnhancedInputActionIA_MoveBackwards
  (params (ActionValue :type Float%20%28double-precision%29) (ElapsedSeconds :type Float%20%28double-precision%29) (TriggeredSeconds :type Float%20%28double-precision%29) (InputAction :type Input%20Action%20Object%20Reference :default "/Game/Inputs/IA_MoveBackwards.IA_MoveBackwards"))
  ;[0.09152 0.15 0.07935 0.5] Movement
  (:Triggered
    (if (not (GameplayTags|HasAnyMatchingGameplayTags (Variables|Default|GetPlayerAbilitySystemComp) (Variables|Default|GetHeavyAttackTags))) :!label _label
      (Pawn|Input|AddMovementInput (* (Math|Vector|GetForwardVector (Math|Rotator|MakeRotator 0.0 0.0 (.yaw (Pawn|GetControlRotation :!class /Script/Engine.Pawn)))) -1.0) ActionValue false)))
  (:Ongoing
    (goto _label)))

(event Input|EnhancedActionEvents|EnhancedInputActionIA_CameraControl
  (params (ActionValue :type Vector%202D%20Structure) (ElapsedSeconds :type Float%20%28double-precision%29) (TriggeredSeconds :type Float%20%28double-precision%29) (InputAction :type Input%20Action%20Object%20Reference :default "/Game/Inputs/IA_CameraControl.IA_CameraControl"))
  (bind _looksensitivity (Variables|Default|GetLookSensitivity))
  ;[0.07734 0.15 0.08459 0.5] Camera Control
  (Pawn|Input|AddControllerYawInput (* (.x ActionValue) _looksensitivity))
  (Pawn|Input|AddControllerPitchInput (* (.y ActionValue) _looksensitivity)))

(event Input|EnhancedActionEvents|EnhancedInputActionIA_Slide
  (params (ActionValue :type Boolean) (ElapsedSeconds :type Float%20%28double-precision%29) (TriggeredSeconds :type Float%20%28double-precision%29) (InputAction :type Input%20Action%20Object%20Reference :default "/Game/Inputs/IA_Slide.IA_Slide"))
  (bind _charactermovement (Variables|Character|GetCharacterMovement))
  (bind _returnvalue (AI|Components|NavMovement|IsMovingonGround _charactermovement))
  ;[0.1709 0.5521 0.1553 0.5] Dash Ability
  (:Started
    ;;[0.15 0.15 0.15 0.5] If Dash Hold Not Allowed, Dash and Apply Cooldown Immediately
    (if _returnvalue
      (if (not (Variables|Default|GetisDashing))
        (bind _returnvalue_2 (Class|AbilitySystemComponent|TryActivateAbility (Variables|Default|GetPlayerAbilitySystemComp) (Variables|Default|GetdashAbility) true))
        (if _returnvalue_2
          (Variables|Default|SetisDashing true)
          (if (not (Variables|Default|GetallowDashHold))
            (Utilities|FlowControl|Delay (Variables|Default|GetdashDuration))
            (CallFunction|ApplyDashCooldown))))))
  (:Ongoing
    ;;[0.15 0.15 0.15 0.5] Dash
    (if _returnvalue
      (if (Variables|Default|GetisDashing)
        (if (Variables|Default|GetallowDashHold)
          (Class|AbilitySystemComponent|TryActivateAbility (Variables|Default|GetPlayerAbilitySystemComp) (Variables|Default|GetdashAbility) true)))))
  (:Completed
    ;;[0.15 0.15 0.15 0.5] If Dash Hold Allowed, Wait Until Release To Apply Cooldown
    (if (Variables|Default|GetisDashing)
      (if (Variables|Default|GetallowDashHold)
        (CallFunction|ApplyDashCooldown)))))

(event Input|EnhancedActionEvents|EnhancedInputActionIA_MoveRight
  (params (ActionValue :type Float%20%28double-precision%29) (ElapsedSeconds :type Float%20%28double-precision%29) (TriggeredSeconds :type Float%20%28double-precision%29) (InputAction :type Input%20Action%20Object%20Reference :default "/Game/Inputs/IA_MoveRight.IA_MoveRight"))
  ;[0.09152 0.15 0.07935 0.5] Movement
  (:Triggered
    (if (not (GameplayTags|HasAnyMatchingGameplayTags (Variables|Default|GetPlayerAbilitySystemComp) (Variables|Default|GetHeavyAttackTags))) :!label _label
      (Pawn|Input|AddMovementInput (Math|Vector|GetRightVector (Math|Rotator|MakeRotator 0.0 0.0 (.yaw (Pawn|GetControlRotation :!class /Script/Engine.Pawn)))) ActionValue false)))
  (:Ongoing
    (goto _label)))

(event Input|EnhancedActionEvents|EnhancedInputActionIA_MoveLeft
  (params (ActionValue :type Float%20%28double-precision%29) (ElapsedSeconds :type Float%20%28double-precision%29) (TriggeredSeconds :type Float%20%28double-precision%29) (InputAction :type Input%20Action%20Object%20Reference :default "/Game/Inputs/IA_MoveLeft.IA_MoveLeft"))
  ;[0.09152 0.15 0.07935 0.5] Movement
  (:Triggered
    (if (not (GameplayTags|HasAnyMatchingGameplayTags (Variables|Default|GetPlayerAbilitySystemComp) (Variables|Default|GetHeavyAttackTags))) :!label _label
      (Pawn|Input|AddMovementInput (* (Math|Vector|GetRightVector (Math|Rotator|MakeRotator 0.0 0.0 (.yaw (Pawn|GetControlRotation :!class /Script/Engine.Pawn)))) -1.0) ActionValue false)))
  (:Ongoing
    (goto _label)))

(event Input|EnhancedActionEvents|EnhancedInputActionIA_Pause
  (params (ActionValue :type Boolean) (ElapsedSeconds :type Float%20%28double-precision%29) (TriggeredSeconds :type Float%20%28double-precision%29) (InputAction :type Input%20Action%20Object%20Reference :default "/Game/Inputs/IA_Pause.IA_Pause"))
  ;[0.15 0.15 0.15 0.5] Pause
  (:Started
    (Default|OpenPauseMenu (Variables|Default|GetHUD))))

(event Input|EnhancedActionEvents|EnhancedInputActionIA_Interact
  (params (ActionValue :type Boolean) (ElapsedSeconds :type Float%20%28double-precision%29) (TriggeredSeconds :type Float%20%28double-precision%29) (InputAction :type Input%20Action%20Object%20Reference :default "/Game/Inputs/IA_Interact.IA_Interact"))
  (bind _nearbyupgrade (Variables|Default|GetNearbyUpgrade))
  ;[0.15 0.15 0.15 0.5] Interact - Equip Upgrade if one is nearby
  (Utilities|IsValid _nearbyupgrade
    (:Is%20Valid
      (Default|OpenItemEquipUI _nearbyupgrade))))

(event Input|EnhancedActionEvents|EnhancedInputActionIA_CameraSwap
  (params (ActionValue :type Boolean) (ElapsedSeconds :type Float%20%28double-precision%29) (TriggeredSeconds :type Float%20%28double-precision%29) (InputAction :type Input%20Action%20Object%20Reference :default "/Game/Inputs/IA_CameraSwap.IA_CameraSwap"))
  (bind _charactermovementcomp (Variables|Default|GetCharacterMovementComp))
  (bind _charactermovementcomp_2 (Variables|Default|GetCharacterMovementComp))
  ;[0.06447 0.15 0.04219 0.5] Changing Camera Angle to Over the Shoulder and Back
  (if (Variables|Default|GetCameraSwapped)
    (Transformation|SetRelativeLocation (Variables|Default|GetSpringArm) "0.000000,0.000000,70.000000" true false)
    (Variables|/Script/Engine.CharacterMovementComponent|SetbOrientRotationToMovement _charactermovementcomp true)
    (Variables|/Script/Engine.CharacterMovementComponent|SetbUseControllerDesiredRotation _charactermovementcomp false)
    (Variables|Default|SetCameraSwapped false)
    (else
      (Transformation|SetRelativeLocation (Variables|Default|GetSpringArm) "140.000000,-110.000000,30.000000" true false)
      (Variables|/Script/Engine.CharacterMovementComponent|SetbOrientRotationToMovement _charactermovementcomp_2 false)
      (Variables|/Script/Engine.CharacterMovementComponent|SetbUseControllerDesiredRotation _charactermovementcomp_2 true)
      (Variables|Default|SetCameraSwapped true))))

(event Input|EnhancedActionEvents|EnhancedInputActionIA_OpenInventory
  (params (ActionValue :type Boolean) (ElapsedSeconds :type Float%20%28double-precision%29) (TriggeredSeconds :type Float%20%28double-precision%29) (InputAction :type Input%20Action%20Object%20Reference :default "/Game/Inputs/IA_OpenInventory.IA_OpenInventory"))
  ;[0.15 0.15 0.15 0.5] Open Inventory
  (:Started
    (Default|ToggleInventoryUI (Variables|Default|GetHUD))))

(event Input|EnhancedActionEvents|EnhancedInputActionIA_ShoulderSwap
  (params (ActionValue :type Boolean) (ElapsedSeconds :type Float%20%28double-precision%29) (TriggeredSeconds :type Float%20%28double-precision%29) (InputAction :type Input%20Action%20Object%20Reference :default "/Game/Inputs/IA_ShoulderSwap.IA_ShoulderSwap"))
  ;[0.09468 0.15 0.07978 0.5] Ability to Swap Between Shoulders During Gameplay
  (if (Variables|Default|GetCameraSwapped)
    (if (Variables|Default|GetSwappedShoulder)
      (Transformation|SetRelativeLocation (Variables|Default|GetSpringArm) "140.000000,-110.000000,30.000000" true false)
      (Variables|Default|SetSwappedShoulder false)
      (else
        (Transformation|SetRelativeLocation (Variables|Default|GetSpringArm) "140.000000,110.000000,30.000000" true false)
        (Variables|Default|SetSwappedShoulder true)))))

(event Input|EnhancedActionEvents|EnhancedInputActionIA_Jump
  (params (ActionValue :type Boolean) (ElapsedSeconds :type Float%20%28double-precision%29) (TriggeredSeconds :type Float%20%28double-precision%29) (InputAction :type Input%20Action%20Object%20Reference :default "/Game/Inputs/IA_Jump.IA_Jump"))
  (bind _allowdashduringjump (Variables|Default|GetallowDashDuringJump))
  (bind _isdashing (Variables|Default|GetisDashing))
  (bind _returnvalue (not _isdashing))
  (bind _returnvalue_2 (or _returnvalue _allowdashduringjump))
  ;[0.09152 0.15 0.07935 0.5] Movement
  (:Started
    (if (not (GameplayTags|HasAnyMatchingGameplayTags (Variables|Default|GetPlayerAbilitySystemComp) (Variables|Default|GetHeavyAttackTags)))
      (if _returnvalue_2
        (Character|Jump))))
  (:Completed
    (if _returnvalue_2
      (Character|StopJumping))))

(event EventTick
  (params (DeltaSeconds :type Float%20%28single-precision%29))
  (CallFunction|CheckIsGrounded)
  (CallFunction|HandleInvulnCooldown DeltaSeconds)
  (CallFunction|HandleHeatBurnDisable)
  ;[0.15 0.15 0.15 0.5] Handle Physics Application Cooldown - Bandaid Fix
  (if (Variables|Default|GetAttackPhysicsAppliedThisFrame)
    (Utilities|FlowControl|Delay 0.2)
    (Variables|Default|SetAttackPhysicsAppliedThisFrame false)))

(event Collision|EventActorBeginOverlap
  (params (OtherActor :type Actor%20Object%20Reference)))

(event EventBeginPlay
  (bind _returnvalue (Game|GetPlayerController 0))
  (bind _playerabilitysystemcomp (Variables|Default|GetPlayerAbilitySystemComp))
  (bind _mesh (Variables|Character|GetMesh))
  (bind _playerabilitysystemcomp_2 (Variables|Default|GetPlayerAbilitySystemComp))
  (bind _returnvalue_2 (PlayerController|LocalPlayerSubsystems|GetEnhancedInputLocalPlayerSubsystem _returnvalue))
  (Utilities|FlowControl|Sequence
    (:then_0
      ;[0.15 0.15 0.15 0.5] Bind on Hit Events
      (EventDispatchers|AssignHitboxHitActorsDelegate (Variables|Default|GetAttackHitboxManager) (delegate Custom|HitboxHitActorsDelegate_Event))
      (EventDispatchers|BindEventtoOnDeath (delegate Custom|Event_PlayerDeath)))
    (:then_1
      (bind _returnvalue_3 (GameplayAbilities|GiveAbility (Variables|Default|GetPlayerAbilitySystemComp) "/Game/Blueprints/Player/GAS/Abilities/GA_ActivateGenerator.GA_ActivateGenerator_C" 1 -1))
      (Variables|Default|SetActivateGeneratorAbility _returnvalue_3)
      (GameplayEffects|ApplyGameplayEffectToSelf :self _playerabilitysystemcomp_2 :GameplayEffectClass "/Game/Blueprints/Player/GAS/Effects/Heat/GE_ConstantHeatDrain.GE_ConstantHeatDrain_C" :Level 1.0)
      ;[0.15 0.15 0.15 0.5] Temporary assignment of health
      (bind _returnvalue_4 (Ability|GameplayEffect|AssignTagSetbyCallerMagnitude (GameplayEffects|MakeOutgoingSpec :self _playerabilitysystemcomp_2 :GameplayEffectClass "/Game/Blueprints/Enemies/Effects/GE_InitializeHealth.GE_InitializeHealth_C") "(TagName=\"Health.Initialize\")" (Variables|Default|GetBaseHealth)))
      (GameplayEffects|ApplyGameplayEffectSpecToSelf (Variables|Default|GetPlayerAbilitySystemComp) _returnvalue_4)
      ;[0.15 0.15 0.15 0.5] Set Up Abilities
      (bind _returnvalue_5 (GameplayAbilities|GiveAbility _playerabilitysystemcomp "/Game/Blueprints/Player/GAS/Abilities/GA_Dash.GA_Dash_C" 0 -1))
      (Variables|Default|SetdashAbility _returnvalue_5)
      (bind _returnvalue_6 (GameplayAbilities|GiveAbility _playerabilitysystemcomp "/Game/Blueprints/Player/GAS/Abilities/HeatBurn/GA_ActivateHeatBurn.GA_ActivateHeatBurn_C" 0 -1))
      (Variables|Default|SetHeatBurnAbility _returnvalue_6)
      ;[0.15 0.15 0.15 0.5] Set Up Input
      (Utilities|IsValid _returnvalue_2
        (:Is%20Valid
          (Input|AddMappingContext _returnvalue_2 "/Game/Inputs/IMC_PlayerInputMapping.IMC_PlayerInputMapping" 0 "(bIgnoreAllPressedKeysUntilRelease=True,bForceImmediately=False,bNotifyUserSettings=False)")
          ;[0.15 0.15 0.15 0.5] Overlay Effect Shaders
          (CallFunction|AssignHitFlashMat _mesh)
          (CallFunction|AssignEquipEffectMat _mesh))))))

(fn ConstructionScript)

(fn ApplyDashCooldown
  (GameplayEffects|ApplyGameplayEffectToSelf :self (Variables|Default|GetPlayerAbilitySystemComp) :GameplayEffectClass "/Game/Blueprints/Player/GAS/Effects/GE_DashCooldown.GE_DashCooldown_C")
  (Variables|/Script/Engine.CharacterMovementComponent|SetGroundFriction (Variables|Character|GetCharacterMovement) (Variables|Default|GetdefaultFriction))
  (Variables|Default|SetisDashing false))

(fn SetNearbyUpgrade
  (params (Upgrade :type BP%20Equipable%20Item%20Object%20Reference))
  (Variables|Default|SetNearbyUpgrade Upgrade))

(fn CreateLightHitbox
  (Class|AbilitySystemComponent|TryActivateAbility (Variables|Default|GetPlayerAbilitySystemComp) (Variables|Default|GetlightAttack) true))

(fn CreateHeavyGroundHitbox
  (Class|AbilitySystemComponent|TryActivateAbility (Variables|Default|GetPlayerAbilitySystemComp) (Variables|Default|GetheavyGroundAttack) true))

(fn CreateHeavyAirHitbox
  (Class|AbilitySystemComponent|TryActivateAbility (Variables|Default|GetPlayerAbilitySystemComp) (Variables|Default|GetheavyAirAttack) true))

(fn TryActivateGenerator
  (bind _returnvalue (Class|AbilitySystemComponent|TryActivateAbility (Variables|Default|GetPlayerAbilitySystemComp) (Variables|Default|GetActivateGeneratorAbility) true))
  (return _returnvalue))

(fn DealDamagetoHitActor
  (params (HitActor :type Actor%20Object%20Reference) (Damage :type Float%20%28double-precision%29))
  (bind _returnvalue (Ability|GameplayEffect|AssignTagSetbyCallerMagnitude (GameplayEffects|MakeOutgoingSpec :self (Variables|Default|GetPlayerAbilitySystemComp) :GameplayEffectClass "/Game/Blueprints/Player/GAS/Effects/GE_ApplyDamageToTarget.GE_ApplyDamageToTarget_C" :Level 1.0) "(TagName=\"Damage.Apply\")" Damage))
  (GameplayEffects|ApplyGameplayEffectSpecToTarget (Variables|Default|GetPlayerAbilitySystemComp) _returnvalue (Ability|GetAbilitySystemComponent HitActor))
  (return))

(fn GainHeat
  (bind _playerabilitysystemcomp (Variables|Default|GetPlayerAbilitySystemComp))
  (bind _returnvalue (Ability|GameplayEffect|AssignTagSetbyCallerMagnitude (GameplayEffects|MakeOutgoingSpec :self _playerabilitysystemcomp :GameplayEffectClass "/Game/Blueprints/Player/GAS/Effects/Heat/GE_AddOrSubtractHeat.GE_AddOrSubtractHeat_C" :Level 1.0) "(TagName=\"Heat.Add\")" (Variables|Default|GetHeatGainOnHit)))
  (GameplayEffects|ApplyGameplayEffectSpecToSelf _playerabilitysystemcomp _returnvalue))

(fn ActivateAerialHitPhysics
  (params (PlayerLaunchForce :type Vector))
  ;[0.15 0.15 0.15 0.5] Only Apply Aerial Physics If Not Grounded
  (if (Variables|Default|GetIsGrounded)
    ;[0.15 0.15 0.15 0.5] Launch Character While Grounded if Launch Force Isn't Zero
    (if (not (Math|Vector|VectorIsZero PlayerLaunchForce))
      (Character|LaunchCharacter PlayerLaunchForce false true :!label _label))
    (else
      (GameplayEffects|ApplyGameplayEffectToSelf :self (Variables|Default|GetPlayerAbilitySystemComp) :GameplayEffectClass "/Game/Blueprints/Player/GAS/Effects/GE_ApplyAerialHitPhysics.GE_ApplyAerialHitPhysics_C" :Level 1.0)
      (goto _label))))

(fn HitActor
  (params (Actor :type Object%20Object%20Reference) (HitboxData :type Hitbox%20Data%20Structure))
  (bind (_positionoffset _height _radius _rotation _knockbackdirection _knockbackforce _damage _stuntime _playerlaunchforce) (Utilities|Struct|BreakHitboxData HitboxData))
  (bind _output_get (Variables|Default|SetDamage _damage))
  (Development|PrintString (Utilities|String|ToString(Float) (* _output_get (.ReturnValue (Class|AbilitySystemComponent|GetGameplayAttributeValue (Ability|GetAbilitySystemComponent 0) "(AttributeName=\"DamageMultiplier\",Attribute=/Script/Coldsnap.PlayerMovementAttributeSet:DamageMultiplier,AttributeOwner=\"/Script/CoreUObject.Class'/Script/Coldsnap.PlayerMovementAttributeSet'\")")))) true true "(R=0.947236,G=1.000000,B=0.000000,A=1.000000)")
  (bind _ashittable (Utilities|Casting|CastToHittable Actor)
    (:then
      (Class|Hittable|Hit _ashittable (* _output_get (.ReturnValue (Class|AbilitySystemComponent|GetGameplayAttributeValue (Ability|GetAbilitySystemComponent 0) "(AttributeName=\"DamageMultiplier\",Attribute=/Script/Coldsnap.PlayerMovementAttributeSet:DamageMultiplier,AttributeOwner=\"/Script/CoreUObject.Class'/Script/Coldsnap.PlayerMovementAttributeSet'\")"))) (Math|Vector|RotateVector (* _knockbackdirection _knockbackforce) (Transformation|GetWorldRotation (Variables|Default|GetCapsuleComponent))))
      (bind _asactor (Utilities|Casting|CastToActor Actor))
      (CallFunction|DealDamagetoHitActor _asactor (* _output_get (.ReturnValue (Class|AbilitySystemComponent|GetGameplayAttributeValue (Ability|GetAbilitySystemComponent 0) "(AttributeName=\"DamageMultiplier\",Attribute=/Script/Coldsnap.PlayerMovementAttributeSet:DamageMultiplier,AttributeOwner=\"/Script/CoreUObject.Class'/Script/Coldsnap.PlayerMovementAttributeSet'\")"))))
      ;[0.15 0.15 0.15 0.5] Only Apply On Hit Physics If hasn't been applied this frame
      (if (Variables|Default|GetAttackPhysicsAppliedThisFrame)
        _
        (else
          (CallFunction|ActivateAerialHitPhysics _playerlaunchforce)
          (Variables|Default|SetAttackPhysicsAppliedThisFrame true)
          (Audio|Components|Audio|Play (Variables|Default|GetEnemyHitAudio) 0.0)))
      ;[0.15 0.15 0.15 0.5] Check to Gain Heat - Eventually Should be Implemented in Hit Implementation for Enemies
      (Utilities|Casting|CastToEnemy _asactor)
      (CallFunction|GainHeat))
    (:CastFailed
      (Development|PrintString (LocalVariables|GetWarningText)))))

(fn GetSkeletalMesh
  (return (Variables|Character|GetMesh)))

(fn CheckIsGrounded
  (bind _charactermovementcomp (Variables|Default|GetCharacterMovementComp))
  (bind _playerabilitysystemcomp (Variables|Default|GetPlayerAbilitySystemComp))
  (bind _returnvalue (AI|Components|NavMovement|IsMovingonGround _charactermovementcomp))
  ;[0.15 0.15 0.15 0.5] Check If Grounded State has changed from last frame
  (if (not (== _returnvalue (Variables|Default|GetIsGrounded)))
    ;[0.15 0.15 0.15 0.5] If grounded state changed, update gameplay tags
    (bind _output_get (Variables|Default|SetIsGrounded _returnvalue))
    (if _output_get
      (GameplayEffects|RemoveActiveEffectswithGrantedTags _playerabilitysystemcomp "(GameplayTags=((TagName=\"Player.Airborne\")))")
      (Animation|StopAnimMontage (Animation|GetCurrentMontage :!class /Script/Engine.Character))
      (else
        (GameplayEffects|ApplyGameplayEffectToSelf :self _playerabilitysystemcomp :GameplayEffectClass "/Game/Blueprints/Player/GAS/Effects/GE_Airborne.GE_Airborne_C")))))

(fn SetInvulnerable
  (Variables|Default|SetInvulnerable true)
  (Variables|Default|SetInvulnTimer (Variables|Default|GetInvulnTime)))

(fn HandleInvulnCooldown
  (params (DeltaTime :type Float%20%28double-precision%29))
  (if (Variables|Default|GetInvulnerable)
    (Variables|Default|SetInvulnTimer (- (Variables|Default|GetInvulnTimer) DeltaTime))
    (if (<= (Variables|Default|GetInvulnTimer) 0.0)
      (Variables|Default|SetInvulnerable false))))

(fn TryActivateEquipableAbility
  (params (AbilitySlot :type Integer))
  (bind _equipableabilities (Variables|Default|GetEquipableAbilities))
  (bind (_value _returnvalue) (Utilities|Map|Find _equipableabilities AbilitySlot))
  (if _returnvalue
    (Class|AbilitySystemComponent|TryActivateAbility (Variables|Default|GetPlayerAbilitySystemComp) _value true)
    (else
      (Development|PrintString (Utilities|String|Append (LocalVariables|GetEmptySlotWarning) (Utilities|String|ToString(Integer) AbilitySlot))))))

(fn AddEquipableAbility
  (params (AbilitySlot :type Integer) (AbilityClassToAdd :type Gameplay%20Ability%20Class%20Reference) (PickupTransform :type Transform))
  (bind _equipableabilities (Variables|Default|GetEquipableAbilities))
  (bind (_value _returnvalue) (Utilities|Map|Find _equipableabilities AbilitySlot))
  ;[0.15 0.15 0.15 0.5] Remove Ability In This Slot If It Exists
  (if _returnvalue
    (CallFunction|DropReplacedAbility _value PickupTransform)
    (Utilities|Map|Remove _equipableabilities AbilitySlot))
  ;[0.15 0.15 0.15 0.5] Add New Ability
  (bind _returnvalue_2 (GameplayAbilities|GiveAbility (Variables|Default|GetPlayerAbilitySystemComp) AbilityClassToAdd 0 -1))
  (Utilities|Map|Add _equipableabilities AbilitySlot _returnvalue_2))

(fn DropReplacedAbility
  (params (DropppedAbility :type Gameplay%20Ability%20Spec%20Handle%20Structure) (NewPickupTransform :type Transform))
  (bind _asequipable_ability (Utilities|Casting|CastToEquipableAbility (.ReturnValue (Ability|GameplayAbility|GetGameplayAbilityfromSpecHandle (Variables|Default|GetPlayerAbilitySystemComp) DropppedAbility))))
  (bind _asactor (Utilities|Casting|CastToActorClass (Variables|/Script/Coldsnap.EquipableAbility|GetPickupActor _asequipable_ability)))
  (Game|SpawnActorfromClass _asactor NewPickupTransform "AlwaysSpawn" "MultiplyWithRoot" 0 0))

(fn CheckforPickupsinRange
  (bind _capsulecomponent (Variables|Default|GetCapsuleComponent))
  (bind _returnvalue (Transformation|GetWorldLocation _capsulecomponent))
  ;[0.15 0.15 0.15 0.5] Check for Upgrade In Pick Up Range (Called when an upgrade is equipped)
  (bind (_outactors _returnvalue_2) (Collision|SphereOverlapActors _returnvalue 1.8e+02 (LocalVariables|GetSphereCastObjectTypes) "/Game/Blueprints/Items/EquipableAbilityPickups/BP_BaseEquipableAbilityPickup.BP_BaseEquipableAbilityPickup_C")) ; Sphere radius should match equipable item pickup range - should eventually be direct reference
  (if _returnvalue_2
    (bind _asbp_equipable_item (Utilities|Casting|CastToBP_EquipableItem (.ReturnValue (Actor|FindNearestActor _returnvalue _outactors))))
    (Default|SetNearbyEquipableforPlayer _asbp_equipable_item self)))

(fn CheckforDeath
  (if (<= (.ReturnValue (Ability|Attribute|GetFloatAttributefromAbilitySystemComponent (Variables|Default|GetPlayerAbilitySystemComp) "(AttributeName=\"Health\",Attribute=/Script/Coldsnap.HealthAttributeSet:Health,AttributeOwner=\"/Script/CoreUObject.Class'/Script/Coldsnap.HealthAttributeSet'\")")) 0.0)
    (if (Variables|Default|GetisDead) ; Prevent multiple firings of death-related events
      _
      (else
        (Variables|Default|SetisDead true)
        (return true))))
  (return false))

(fn ActivateHitFeedback
  (Components|Activation|Activate (Variables|Default|GetNiagara) false)
  (Variables|Default|SetFade%20in%20Progress true)
  (Variables|Default|SetFadeIn true)
  (CallFunction|EventControlMaterialFlash)
  (Camera|PlayWorldCameraShake "/Game/Blueprints/Player/BP_CamShakeOnHit.BP_CamShakeOnHit_C" (Transformation|GetActorLocation) 0.0 1e+03)
  (Audio|Components|Audio|Play (Variables|Default|GetDamageAudio) 0.0))

(fn ColorFlashonHit
  (bind _hitflashmat (Variables|Default|GetHitFlashMat))
  (bind _fadeinterval (LocalVariables|GetFadeInterval))
  (bind _returnvalue (Rendering|Material|GetScalarParameterValue (Variables|Default|GetHitFlashMat) "Opacity_param" :!class /Script/Engine.MaterialInstanceDynamic))
  ;[0.15 0.15 0.15 0.5] Check if event should continue running
  (Utilities|IsValid (Variables|Default|GetHitFlashMat)
    (:Is%20Valid
      (if (Variables|Default|GetFade%20in%20Progress)
        (if (Variables|Default|GetFadeIn) ; Check if fading in or out
          ;[0.15 0.15 0.15 0.5] Set opacity
          (Rendering|Material|SetScalarParameterValue _hitflashmat "Opacity_param" (+ _returnvalue _fadeinterval) :!class /Script/Engine.MaterialInstanceDynamic)
          (if (>= (+ _returnvalue _fadeinterval) 1.0) ; Check if fade is over
            (Variables|Default|SetFadeIn false))
          (else
            (Rendering|Material|SetScalarParameterValue _hitflashmat "Opacity_param" (- _returnvalue _fadeinterval) :!class /Script/Engine.MaterialInstanceDynamic)
            (if (<= (- _returnvalue _fadeinterval) 0.0) ; Check if fade is over
              (Variables|Default|SetFade%20in%20Progress false))))
        (bind _returnvalue_2 (Rendering|Material|GetScalarParameterValue (Variables|Default|GetHitFlashMat) "Opacity_param" :!class /Script/Engine.MaterialInstanceDynamic))))
    (:Is%20Not%20Valid
      (Development|PrintString "Invalid material"))))

(fn ControlSensitivity)

(fn UpdateInventoryUI
  (Default|UpdateInventoryText (Variables|/Game/Blueprints/UI/BP_HUD.BP_HUD_C|GetInventoryUI (Variables|Default|GetHUD))))

(fn HandleHeatBurnDisable
  (bind _playerabilitysystemcomp (Variables|Default|GetPlayerAbilitySystemComp))
  (if (Variables|Default|GetIsBurningHeat)
    (if (<= (.ReturnValue (Class|AbilitySystemComponent|GetGameplayAttributeValue _playerabilitysystemcomp "(AttributeName=\"Heat\",Attribute=/Script/Coldsnap.HeatAttributeSet:Heat,AttributeOwner=\"/Script/CoreUObject.Class'/Script/Coldsnap.HeatAttributeSet'\")")) 0.0)
      (Ability|CancelAbility (.ReturnValue (Ability|GameplayAbility|GetGameplayAbilityfromSpecHandle _playerabilitysystemcomp (Variables|Default|GetHeatBurnAbility)))))))

(fn GetHeatBurnAbilitySpecHandle
  (bind _playerabilitysystemcomp (Variables|Default|GetPlayerAbilitySystemComp))
  (for _array_element (Variables|/Script/Coldsnap.PlayerAbilitySystemComponent|GetMappedAbilitySpecHandles _playerabilitysystemcomp)
    (if (== (Utilities|GetClass (.ReturnValue (Ability|GameplayAbility|GetGameplayAbilityfromSpecHandle _playerabilitysystemcomp _array_element))) "/Game/Blueprints/Player/GAS/Abilities/HeatBurn/GA_ActivateHeatBurn.GA_ActivateHeatBurn_C")
      (Variables|Default|SetHeatBurnAbility _array_element))))

(fn AssignHitFlashMat
  (params (SkeletalMeshOnActor :type Skeletal%20Mesh%20Component%20Object%20Reference))
  (bind _returnvalue (Rendering|Material|CreateDynamicMaterialInstance "/Game/Art/Characters/SmallEnemy/Textures/Test/M_EnemyHitDynamic.M_EnemyHitDynamic" "Hit_Highlight_Inst" "None" :!class /Script/Engine.KismetMaterialLibrary))
  (bind _output_get (Variables|Default|SetHitFlashMat _returnvalue))
  (Rendering|Material|SetOverlayMaterial SkeletalMeshOnActor _output_get :!class /Script/Engine.MeshComponent)
  (return SkeletalMeshOnActor))

(fn AssignEquipEffectMat
  (params (SkeletalMeshOnActor :type Skeletal%20Mesh%20Component%20Object%20Reference))
  (bind _returnvalue (Rendering|Material|CreateDynamicMaterialInstance "/Game/Art/Environment/DesignAssets/Shaders/MI_UpgradeEffect_Inst.MI_UpgradeEffect_Inst" "Equip_Effect_Inst" "None" :!class /Script/Engine.KismetMaterialLibrary))
  (bind _output_get (Variables|Default|SetEquipEffectMat _returnvalue))
  (Rendering|Material|SetOverlayMaterial SkeletalMeshOnActor _output_get :!class /Script/Engine.MeshComponent)
  (return SkeletalMeshOnActor))

(fn EquipEffectGlow
  (bind _equipeffectmat (Variables|Default|GetEquipEffectMat))
  (bind _equipeffectmat_2 (Variables|Default|GetEquipEffectMat))
  (bind _fadeinterval (LocalVariables|GetFadeInterval))
  (bind _returnvalue (Rendering|Material|GetScalarParameterValue _equipeffectmat "Opacity" :!class /Script/Engine.MaterialInstanceDynamic))
  ;[0.15 0.15 0.15 0.5] Check if event should continue running
  (Utilities|IsValid _equipeffectmat
    (:Is%20Valid
      (if (Variables|Default|GetEquipEffectFadeInProgress)
        (if (Variables|Default|GetEquipEffectFadeIn) ; Check if fading in or out
          ;[0.15 0.15 0.15 0.5] Set opacity
          (Rendering|Material|SetScalarParameterValue _equipeffectmat_2 "Opacity" (+ _returnvalue _fadeinterval) :!class /Script/Engine.MaterialInstanceDynamic)
          (if (>= (+ _returnvalue _fadeinterval) 1.0) ; Check if fade is over
            (Variables|Default|SetEquipEffectFadeIn false))
          (else
            (Rendering|Material|SetScalarParameterValue _equipeffectmat_2 "Opacity" (- _returnvalue _fadeinterval) :!class /Script/Engine.MaterialInstanceDynamic)
            (if (<= (- _returnvalue _fadeinterval) 0.0) ; Check if fade is over
              (Variables|Default|SetEquipEffectFadeInProgress false)
              (Rendering|Material|SetOverlayMaterial (Variables|Character|GetMesh) (Variables|Default|GetHitFlashMat) :!class /Script/Engine.MeshComponent))))
        (bind _returnvalue_2 (Rendering|Material|GetScalarParameterValue (Variables|Default|GetEquipEffectMat) "Opacity" :!class /Script/Engine.MaterialInstanceDynamic))
        (Development|PrintString (Utilities|String|ToString(Float) _returnvalue_2) true true "(R=1.000000,G=0.485410,B=0.038231,A=1.000000)")
        (else
          (Development|PrintString "Invalid material" :!label _label))))
    (:Is%20Not%20Valid
      (goto _label))))

(fn TryActivateDrill
  (bind _returnvalue (Class|AbilitySystemComponent|TryActivateAbility (Variables|Default|GetPlayerAbilitySystemComp) (Variables|Default|GetActivateDrill) true))
  (return _returnvalue))

(fn ChangeTokenAmount
  (params (ChangeVal :type Integer))
  (if (<= (+ ChangeVal (Variables|Default|GetEnemyTokens)) (Variables|Default|GetMaxTokens))
    (Variables|Default|SetEnemyTokens (+ ChangeVal (Variables|Default|GetEnemyTokens)))
    (else
      (Variables|Default|SetEnemyTokens (Variables|Default|GetMaxTokens)))))

(fn AsPlayerCharacter
  (return self))