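; Gameplay ability that teleports the player character forward along the horizontal facing, over a distance derived from its dash duration and force.
; A capsule trace stops short of obstacles, then a ground line trace sets the landing height or rejects the spot.
; After commit, it hands movement to the character's StartTeleportLerp and immediately restores capsule collision and ends.
; Its own timer-style PerformTeleport lerp is never called here.
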(event Ability|EventActivateAbility
  ;[0.8698 0.154 0.1685 0.5] Getting References
  (bind _output_get (Variables|Default|SetActor (Ability|GetOwningActorfromActorInfo)))
  (Variables|Default|SetStartLocation (Transformation|GetActorLocation _output_get))
  (bind _asbp_player_character (Utilities|Casting|CastToBP_PlayerCharacter (Variables|Default|GetActor))
    (:then
      (Variables|Default|SetPlayer _asbp_player_character)
      ;[0.8438 0.8122 0.2197 0.5] Getting teleport distance
      (bind _teleportdistance (CallFunction|GetTeleportDistance (Variables|Default|GetPlayer)))
      (if (>= _teleportdistance 0.0)
        ;[0.1763 0.8698 0.1042 0.5] Finding teleport destination
        (bind (_validlocationfound _finallocation) (CallFunction|FindTeleportDestination _teleportdistance))
        (Variables|Default|SetFinal%20Location _finallocation)
        (if _validlocationfound
          (Variables|/Game/Blueprints/Player/BP_PlayerCharacter.BP_PlayerCharacter_C|SetTeleportElapsedTime (Variables|Default|GetPlayer) 0.0)
          ;[0.2109 0.1989 0.7344 0.5] Committing ability
          (bind _returnvalue (Ability|CommitAbility))
          (if _returnvalue
            (Collision|SetCollisionEnabled (Variables|/Script/Engine.Character|GetCapsuleComponent (Variables|Default|GetPlayer)) "NoCollision")
            (Components|Movement|StopMovementImmediately (Variables|/Script/Engine.Character|GetCharacterMovement (Variables|Default|GetPlayer)))
            ;[0.03597 0.0371 0.2656 0.5] Performing teleport
            (Default|StartTeleportLerp (Variables|Default|GetPlayer) (Variables|Default|GetStartLocation) (Variables|Default|GetFinal%20Location))
            (Collision|SetCollisionEnabled (Variables|/Script/Engine.Character|GetCapsuleComponent (Variables|Default|GetPlayer)) "QueryAndPhysics")
            ;[0.1251 0.7979 0.8281 0.8261] Ending ability
            (Ability|EndAbility)
            (else
              (Development|PrintString "Commit failed, end ability" true true "(R=1.000000,G=0.000000,B=0.015317,A=1.000000)")
              (Ability|EndAbility)))
          (else
            (Development|PrintString "No valid destination, end ability" true true "(R=1.000000,G=0.000000,B=0.015317,A=1.000000)")
            (Ability|EndAbility)))
        (else
          (Development|PrintString "Teleport distance 0 or less, end ability" true true "(R=1.000000,G=0.000000,B=0.015317,A=1.000000)")
          (Ability|EndAbility))))
    (:CastFailed
      (Development|PrintString "Player character invalid, end ability" true true "(R=1.000000,G=0.000000,B=0.015317,A=1.000000)")
      (Ability|EndAbility))))

(event Ability|EventOnEndAbility
  (params (bWasCancelled :type Boolean)))

(fn GetTeleportDistance
  (params (Player :type BP%20Player%20Character%20Object%20Reference))
  (Development|PrintString "TP distance found" true true "(R=0.634122,G=0.000495,B=1.000000,A=1.000000)")
  (return (* (Variables|/Script/Coldsnap.PlayerCharacter|GetdashDuration Player) (Math|Vector|VectorLength (Variables|/Script/Coldsnap.PlayerCharacter|GetdashForce Player)))))

(fn FindTeleportDestination
  (params (TeleportDistance :type Float%20%28double-precision%29))
  (bind _actor (Variables|Default|GetActor))
  (bind _player (Variables|Default|GetPlayer))
  (bind _returnvalue (Transformation|GetActorForwardVector _actor))
  (bind _capsulecomponent (Variables|/Script/Engine.Character|GetCapsuleComponent _player))
  (bind (_x _y) (Math|Vector|BreakVector _returnvalue))
  ;[0.8698 0.154 0.1685 0.5] Setting up references
  (LocalVariables|SetTeleportDistanceRef TeleportDistance)
  (Utilities|Array|Add (LocalVariables|GetActorsToIgnore) (Variables|Default|GetPlayer))
  (LocalVariables|SetForwardDirection (Math|Vector|Normalize (Math|Vector|MakeVector _x _y 0.0)))
  ;[0.7708 0.2694 0.06825 0.5] Adjusting start location
  (Variables|Default|SetStartLocation (+ (Variables|Default|GetStartLocation) (Math|Vector|MakeVector 0.0 0.0 (Variables|Default|GetFowardTraceLift))))
  ;[0.8229 0.4857 0.1286] Calculating desired location
  (LocalVariables|SetDesiredLocation (+ (+ (Variables|Default|GetStartLocation) (* (LocalVariables|GetForwardDirection) (LocalVariables|GetTeleportDistanceRef))) (Math|Vector|MakeVector 0.0 0.0 (Variables|Default|GetFowardTraceLift))))
  ;[0.8438 0.8122 0.2197 0.5] Getting capsule dimensions
  (LocalVariables|SetCapsuleRadius (Components|Capsule|GetScaledCapsuleRadius _capsulecomponent))
  (LocalVariables|SetCapsuleHalfHeight (Components|Capsule|GetScaledCapsuleHalfHeight _capsulecomponent))
  ;[0.1763 0.8698 0.1042 0.5] Perofrming capsule trace to see if the teleport location will run into a obstacle
  (bind (_outhit _returnvalue_2) (Collision|CapsuleTraceByChannel (Variables|Default|GetStartLocation) (LocalVariables|GetDesiredLocation) (LocalVariables|GetCapsuleRadius) (LocalVariables|GetCapsuleHalfHeight) "TraceTypeQuery1" false (LocalVariables|GetActorsToIgnore) "None"))
  (if _returnvalue_2 ; Did the trace hit something?
    ;;[0.1251 0.7979 0.8281 0.8261] If player hits something, teleport player to just in front of it
    (LocalVariables|SetCandidateLocation (- (.Location (Collision|BreakHitResult _outhit)) (* (LocalVariables|GetForwardDirection) (LocalVariables|GetCapsuleRadius))))
    (else
      ;;[0.03597 0.0371 0.2656 0.5] If nothing is hit, use desired location as candidate location
      (LocalVariables|SetCandidateLocation (LocalVariables|GetDesiredLocation))))
  ;[0.7812 0.2645 0.7261] Getting ground trace start and end depending on candidate location
  (LocalVariables|SetGroundTraceStart (+ (LocalVariables|GetCandidateLocation) (Math|Vector|MakeVector 0.0 0.0 (LocalVariables|GetGroundTraceHeight))))
  (LocalVariables|SetGroundTraceEnd (- (LocalVariables|GetCandidateLocation) (Math|Vector|MakeVector 0.0 0.0 (LocalVariables|GetGroundTraceDepth))))
  ;[0.3903 0.1348 0.5625 0.5] Performing ground trace
  (bind (_outhit_2 _returnvalue_3) (Collision|LineTraceByChannel (LocalVariables|GetGroundTraceStart) (LocalVariables|GetGroundTraceEnd) "TraceTypeQuery1" false (LocalVariables|GetActorsToIgnore) "None"))
  (if _returnvalue_3 ; Was ground found?
    (bind _output_get (LocalVariables|SetFinalTeleportLocation (+ (.ImpactPoint (Collision|BreakHitResult _outhit_2)) (Math|Vector|MakeVector 0.0 0.0 (LocalVariables|GetCapsuleHalfHeight)))))
    (Development|PrintString "VALID LOCATION FOUND" true true "(R=1.000000,G=0.000000,B=0.772921,A=1.000000)")
    (return true _output_get)
    (else
      (Development|PrintString "No ground")
      (return false "0, 0, 0"))))

(fn PerformTeleport
  (params (FinalTeleportLocation :type Vector) (ActorRotation :type Rotator))
  (Variables|Default|SetTeleportElapsedTime (+ (Variables|Default|GetTeleportElapsedTime) (Variables|Default|GetTeleportUpdateRate)))
  (LocalVariables|SetAlpha (/ (Variables|Default|GetTeleportElapsedTime) (Variables|Default|GetTeleportDuration)))
  (Development|PrintString "PERFORMING TP" true true "(R=0.103307,G=1.000000,B=0.000000,A=1.000000)")
  (Transformation|SetActorLocation (Variables|Default|GetPlayer) (Math|Vector|Lerp(Vector) (Variables|Default|GetStartLocation) (Variables|Default|GetFinal%20Location) (Math|Float|Clamp(Float) (/ (Variables|Default|GetTeleportElapsedTime) (Variables|Default|GetTeleportDuration)))) false false)
  (if (>= (LocalVariables|GetAlpha) 1.0)
    (Utilities|Time|ClearandInvalidateTimerbyHandle (Variables|Default|GetTimerHandle))
    (Development|PrintString "TP FINISHED")))