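; Gameplay ability that switches on the player character's heat burn state.
; On activation it sets the player's burning flag, applies the GE_NewHeatBurn effect to its owner and plays the heat burn audio.
; When the ability ends, it clears the flag and removes active effects granting the player's HeatBurn tags.
; Heat particle activation and deactivation nodes are present but disconnected, so they never run.
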(event Ability|EventActivateAbility
  (bind _returnvalue (Ability|GetOwningActorfromActorInfo))
  (bind _asbp_player_character (Utilities|Casting|CastToBP_PlayerCharacter _returnvalue))
  (bind _output_get (Variables|Default|SetPlayer _asbp_player_character))
  (Variables|/Game/Blueprints/Player/BP_PlayerCharacter.BP_PlayerCharacter_C|SetIsBurningHeat _output_get true)
  (GameplayEffects|ApplyGameplayEffectToSelf :self (Ability|GetAbilitySystemComponent _returnvalue) :GameplayEffectClass "/Game/Blueprints/Player/GAS/Effects/Heat/GE_NewHeatBurn.GE_NewHeatBurn_C")
  (Audio|Components|Audio|Play (Variables|/Game/Blueprints/Player/BP_PlayerCharacter.BP_PlayerCharacter_C|GetHeatBurnAudio (Variables|Default|GetPlayer)) 0.0))

(event Ability|EventOnEndAbility
  (params (bWasCancelled :type Boolean))
  (Variables|/Game/Blueprints/Player/BP_PlayerCharacter.BP_PlayerCharacter_C|SetIsBurningHeat (Variables|Default|GetPlayer) false)
  (GameplayEffects|RemoveActiveEffectswithGrantedTags (Ability|GetAbilitySystemComponent (Ability|GetOwningActorfromActorInfo)) "(GameplayTags=((TagName=\"Player.HeatBurn\")))"))