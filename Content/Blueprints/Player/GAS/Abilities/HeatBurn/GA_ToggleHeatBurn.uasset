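; Gameplay ability that toggles the player character's heat burn mode on or off.
; On activation it calls CallBurnMode, then checks the player's IsBurningHeat flag.
; If burning, it ends the burn mode ability instance found through its stored spec handle; otherwise it tries to activate that ability when heat is above zero.
; The toggle then ends itself, acting as a one-shot switch for the separate burn ability.
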(event Ability|EventActivateAbility
  (Default|CallBurnMode)
  (bind _asbp_player_character (Utilities|Casting|CastToBP_PlayerCharacter (Ability|GetOwningActorfromActorInfo)))
  (Variables|Default|SetPlayer _asbp_player_character)
  ;[0.276 0.01853 0.01294 0.6522] Check if burn mode is currently on or off
  (if (Variables|/Game/Blueprints/Player/BP_PlayerCharacter.BP_PlayerCharacter_C|GetIsBurningHeat (Variables|Default|GetPlayer))
    ;[0.276 0.01853 0.01294 0.6522] If in burn mode, cancel ability
    (if (.bIsInstance (Ability|GameplayAbility|GetGameplayAbilityfromSpecHandle (Variables|/Script/Coldsnap.PlayerCharacter|GetPlayerAbilitySystemComp (Variables|Default|GetPlayer)) (Variables|/Game/Blueprints/Player/BP_PlayerCharacter.BP_PlayerCharacter_C|GetBurnModeAbility (Variables|Default|GetPlayer))))
      (Ability|EndAbility (.ReturnValue (Ability|GameplayAbility|GetGameplayAbilityfromSpecHandle (Variables|/Script/Coldsnap.PlayerCharacter|GetPlayerAbilitySystemComp (Variables|Default|GetPlayer)) (Variables|/Game/Blueprints/Player/BP_PlayerCharacter.BP_PlayerCharacter_C|GetBurnModeAbility (Variables|Default|GetPlayer))))))
    (else
      ;[0.276 0.01853 0.01294 0.6522] If heat > 0, activate burn mode -otherwise end toggle ability
      (if (and (.bSuccessfullyFoundAttribute (Ability|Attribute|GetFloatAttributefromAbilitySystemComponent (Variables|/Script/Coldsnap.PlayerCharacter|GetPlayerAbilitySystemComp (Variables|Default|GetPlayer)) "(AttributeName=\"Heat\",Attribute=/Script/Coldsnap.HeatAttributeSet:Heat,AttributeOwner=\"/Script/CoreUObject.Class'/Script/Coldsnap.HeatAttributeSet'\")")) (> (.ReturnValue (Ability|Attribute|GetFloatAttributefromAbilitySystemComponent (Variables|/Script/Coldsnap.PlayerCharacter|GetPlayerAbilitySystemComp (Variables|Default|GetPlayer)) "(AttributeName=\"Heat\",Attribute=/Script/Coldsnap.HeatAttributeSet:Heat,AttributeOwner=\"/Script/CoreUObject.Class'/Script/Coldsnap.HeatAttributeSet'\")")) 0.0))
        (Class|AbilitySystemComponent|TryActivateAbility (Variables|/Script/Coldsnap.PlayerCharacter|GetPlayerAbilitySystemComp (Variables|Default|GetPlayer)) (Variables|/Game/Blueprints/Player/BP_PlayerCharacter.BP_PlayerCharacter_C|GetBurnModeAbility (Variables|Default|GetPlayer)) true))))
  (Ability|EndAbility))

(event Ability|EventOnEndAbility
  (params (bWasCancelled :type Boolean)))