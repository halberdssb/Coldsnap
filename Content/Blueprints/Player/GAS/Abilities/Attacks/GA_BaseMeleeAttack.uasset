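; Base Gameplay Ability for player melee attacks with a combo input window.
; On activation it flags the player as attacking, plays the attack montage and applies GE_AttackActive, then waits for montage duration plus the combo window.
; It broadcasts OnAttackStarted before binding to it, so a later attack ends this one early.
; Either ending stops the montage, removes the effect, resets hitbox ignored actors and ends the ability.
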(event Custom|OnAbilityEnd_Event
  ;[0.15 0.01057 0.001083 0.5] Attack Started Delegate
  (CallFunction|OnComboInputWindowEnd))

(event Ability|EventActivateAbility
  ;[0.007354 0.08234 0.15 0.5] Get Player Actor & Character References
  (bind (_player_actor_ref _player_character_ref) (CallFunction|GetPlayerReferences))
  (Variables|/Game/Blueprints/Player/BP_PlayerCharacter.BP_PlayerCharacter_C|SetIsAttacking _player_character_ref true)
  ;[0.15 0.01057 0.001083 0.5] Attack Started Delegate
  (Default|CallOnAttackStarted _player_character_ref)
  (EventDispatchers|AssignOnAttackStarted _player_character_ref (delegate Custom|OnAbilityEnd_Event))
  ;[0.0482 0.01957 0.15 0.5] Fire Attack Animation
  (bind _animduration (CallFunction|PlayAttackMontage _player_actor_ref))
  (bind _returnvalue (GameplayEffects|ApplyGameplayEffectToSelf :self (Ability|GetAbilitySystemComponent (Variables|Default|GetPlayerActor)) :GameplayEffectClass "/Game/Blueprints/Player/GAS/Effects/Attacks/Utility/GE_AttackActive.GE_AttackActive_C"))
  (Variables|Default|SetActiveAttackEffectHandle _returnvalue)
  ;[0.01462 0.15 0 0.5] Wait For Combo Input Before Ability Ends
  (Utilities|FlowControl|Delay (+ _animduration (Variables|Default|GetComboInputWindow)))
  (EventDispatchers|UnbindEventfromOnAttackStarted (Variables|Default|GetPlayerCharacterRef) (delegate Custom|OnAbilityEnd_Event))
  (CallFunction|OnComboInputWindowEnd)
  (Variables|/Game/Blueprints/Player/BP_PlayerCharacter.BP_PlayerCharacter_C|SetIsAttacking (Variables|Default|GetPlayerCharacterRef) false)
  (Development|PrintString "Hello" true true "(R=0.937612,G=0.070641,B=1.000000,A=1.000000)"))

(fn PlayAttackMontage
  (params (Player%20Actor :type Object%20Object%20Reference))
  (bind _asbp_player_character (Utilities|Casting|CastToBP_PlayerCharacter Player%20Actor))
  (bind _skeletal_mesh (Default|GetSkeletalMesh _asbp_player_character))
  (bind _returnvalue (Class|AnimInstance|MontagePlaywithBlendSettings (Components|SkeletalMesh|GetAnimInstance _skeletal_mesh) (Variables|Default|GetAttackAnimMontage) (LocalVariables|GetAttackBlendSettings) 1.0 "Duration" 0.0 true))
  (return _returnvalue))

(fn GABaseMeleeAttackAutoGenFunc)

(fn OnComboInputWindowEnd
  (bind _asbp_player_character (Utilities|Casting|CastToBP_PlayerCharacter (Variables|Default|GetPlayerActor)))
  (bind _skeletal_mesh (Default|GetSkeletalMesh _asbp_player_character))
  (Animation|Montage|MontageStop (Components|SkeletalMesh|GetAnimInstance _skeletal_mesh) 0.25 0)
  (GameplayEffects|RemoveActiveGameplayEffect (Ability|GetAbilitySystemComponent (Variables|Default|GetPlayerActor)) (Variables|Default|GetActiveAttackEffectHandle) -1)
  (Class|AttackHitboxManager|ResetIgnoredHitActors (Variables|/Script/Coldsnap.PlayerCharacter|GetAttackHitboxManager (Variables|Default|GetPlayerCharacterRef)))
  (Ability|EndAbility))

(fn GetPlayerReferences
  (bind _output_get (Variables|Default|SetPlayerActor (Components|GetOwner (Ability|GetAbilitySystemComponentfromActorInfo))))
  (bind _asbp_player_character (Utilities|Casting|CastToBP_PlayerCharacter _output_get)
    (:then
      (bind _output_get_2 (Variables|Default|SetPlayerCharacterRef _asbp_player_character)))
    (:CastFailed
      _))
  (return _output_get _output_get_2))