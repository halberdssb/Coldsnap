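; Gameplay Ability that spawns a BP_LavaPool actor on the ground beneath the avatar.
; On activation it commits the ability, then runs a vertical visibility line trace around the avatar's location to find the floor.
; The pool spawns at the hit point and the ability ends after a short delay; without a hit, it spawns at the avatar's location and ends immediately.
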(event Ability|EventActivateAbility
  (Development|PrintString "Spawn lava pool" true true "(R=0.718722,G=1.000000,B=0.000000,A=1.000000)" 1e+01)
  ;[0.8333 0.1259 0.1359 0.5] Set up
  (bind _returnvalue (Ability|CommitAbility))
  (if _returnvalue
    (Variables|Default|SetBaseLocation (Transformation|GetActorLocation (Ability|GetAvatarActorfromActorInfo)))
    ;[1 0.5143 0 0.3652] Perform ground trace
    (bind (_outhit _returnvalue_2) (Collision|LineTraceByChannel (+ (Variables|Default|GetBaseLocation) "0.000000,0.000000,100.000000") (- (Variables|Default|GetBaseLocation) "0.000000,0.000000,500.000000") "TraceTypeQuery1" false 0 "None"))
    ;[0.8438 0.8122 0.2197 0.5] Spawn lava pool
    (if _returnvalue_2
      (Game|SpawnActorfromClass :Class "/Game/Blueprints/Systems/LavaPool/BP_LavaPool.BP_LavaPool_C" :SpawnTransform (Math|Transform|MakeTransform (.Location (Collision|BreakHitResult _outhit))) :CollisionHandlingOverride "Undefined" :TransformScaleMethod "MultiplyWithRoot" :Instigator 0)
      (Utilities|FlowControl|Delay 0.2)
      (Ability|EndAbility)
      (else
        (Game|SpawnActorfromClass :Class "/Game/Blueprints/Systems/LavaPool/BP_LavaPool.BP_LavaPool_C" :SpawnTransform (Math|Transform|MakeTransform (Variables|Default|GetBaseLocation)) :CollisionHandlingOverride "Undefined" :TransformScaleMethod "MultiplyWithRoot" :Instigator 0)
        (Ability|EndAbility)))))

(event Ability|EventOnEndAbility
  (params (bWasCancelled :type Boolean)))

(fn GetReferences
  (bind _returnvalue (Actor|GetActorOfClass "/Game/Blueprints/Player/BP_PlayerCharacter.BP_PlayerCharacter_C"))
  (Variables|Default|SetPlayerRef _returnvalue))