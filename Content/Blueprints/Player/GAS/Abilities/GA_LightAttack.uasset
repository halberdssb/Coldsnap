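; GA_LightAttack is a Gameplay Ability for the player's light attack, built on a parent ability class.
; On activation it sets KnockbackDirection to the ASC owner's forward vector with an added upward bias.
; It then calls the parent's activation logic and ends the ability immediately after that call returns.
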(event Ability|EventActivateAbility
  (bind _returnvalue (Ability|GetAbilitySystemComponentfromActorInfo))
  (bind _returnvalue_2 (Components|GetOwner _returnvalue))
  (bind _returnvalue_3 (Transformation|GetActorForwardVector _returnvalue_2))
  (bind (_x _y _z) (Math|Vector|BreakVector _returnvalue_3))
  (Variables|Default|SetKnockback%20Direction (Math|Vector|MakeVector _x _y (+ _z 0.5)))
  (|CallParentFunction)
  (Ability|EndAbility))

(event Ability|EventOnEndAbility
  (params (bWasCancelled :type Boolean))
  (|CallParentFunction bWasCancelled) ; This node is disabled and will not be called.\nDrag off pins to build functionality.
)