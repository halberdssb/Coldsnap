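; Base GAS melee attack ability for the player, providing helpers for hit, knockback, damage and Heat gain.
; HitActor sends knockback through Hittable, applies damage via a SetByCaller effect, grants Heat for Enemy hits, then launches the player with an aerial-physics effect.
; Activation only computes a forward hitbox position; the loop calling HitActor is disconnected, and the ability never calls EndAbility.
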(event Ability|EventActivateAbility
  (bind _returnvalue (Ability|GetAbilitySystemComponentfromActorInfo))
  (bind _returnvalue_2 (Components|GetOwner _returnvalue))
  (bind _output_get (Variables|Default|SetPlayerActor _returnvalue_2))
  (bind _asbp_player_character (Utilities|Casting|CastToBP_PlayerCharacter _output_get))
  ;[0.15 0.15 0.15 0.5] Create Hitbox and Get Overlapped Hittables
  (CallFunction|GetHitboxOffsetinPlayerSpace (Variables|/Script/Engine.Actor|GetRootComponent _returnvalue_2)))

(event Ability|EventOnEndAbility
  (params (bWasCancelled :type Boolean)))

(fn GetHitboxOffsetinPlayerSpace
  (params (PlayerSceneComponent :type Scene%20Component%20Object%20Reference))
  (return (+ (Transformation|GetWorldLocation PlayerSceneComponent) (* (Math|Vector|VectorLength (Variables|Default|GetHitboxOffset)) (Math|Vector|Normalize (Math|Vector|GetForwardVector PlayerSceneComponent))))))

(fn ApplyKnockbacktoActor
  (params (Actor :type Object%20Object%20Reference))
  (bind _asknockbackable (Utilities|Casting|CastToKnockbackable Actor)
    (:then
      (Class|Knockbackable|ApplyKnockback _asknockbackable (Variables|Default|GetKnockback%20Direction) (Variables|Default|GetKnockback%20Force)))
    (:CastFailed
      (Development|PrintString (LocalVariables|GetWarningText)))))

(fn HitActor
  (params (Actor :type Object%20Object%20Reference) (KnockbackForce :type Vector))
  (bind _ashittable (Utilities|Casting|CastToHittable Actor)
    (:then
      (Class|Hittable|Hit _ashittable 0.0 KnockbackForce)
      (bind _asactor (Utilities|Casting|CastToActor Actor))
      (CallFunction|DealDamage _asactor)
      ;[0.15 0.15 0.15 0.5] Check to Gain Heat - Eventually Should be Implemented in Hit Implementation for Enemies
      (Utilities|Casting|CastToEnemy _asactor
        (:then
          (CallFunction|GainHeat (Ability|GetAbilitySystemComponent (Ability|GetOwningActorfromActorInfo))))
        (:CastFailed
          _))
      (CallFunction|ActivateAerialHitPhysics))
    (:CastFailed
      (Development|PrintString (LocalVariables|GetWarningText)))))

(fn DealDamage
  (params (HitActor :type Actor%20Object%20Reference))
  (bind _returnvalue (Ability|GameplayEffect|AssignTagSetbyCallerMagnitude (GameplayEffects|MakeOutgoingSpec :self (Ability|GetAbilitySystemComponent (Variables|Default|GetPlayerActor)) :GameplayEffectClass "/Game/Blueprints/Player/GAS/Effects/GE_ApplyDamageToTarget.GE_ApplyDamageToTarget_C" :Level 1.0) "(TagName=\"Damage.Apply\")" (Variables|Default|GetDamage)))
  (GameplayEffects|ApplyGameplayEffectSpecToTarget _returnvalue (Ability|TargetData|AbilityTargetDatafromActor HitActor))
  (Development|PrintString (Utilities|String|ToString(Float) (.ReturnValue (Ability|Attribute|GetFloatAttributefromAbilitySystemComponent (Ability|GetAbilitySystemComponent HitActor) "(AttributeName=\"Health\",Attribute=/Script/Coldsnap.HealthAttributeSet:Health,AttributeOwner=\"/Script/CoreUObject.Class'/Script/Coldsnap.HealthAttributeSet'\")"))))
  (return))

(fn GainHeat
  (params (PlayerAbilitySystem :type Ability%20System%20Component%20Object%20Reference))
  (bind _returnvalue (Ability|GameplayEffect|AssignTagSetbyCallerMagnitude (GameplayEffects|MakeOutgoingSpec :self PlayerAbilitySystem :GameplayEffectClass "/Game/Blueprints/Player/GAS/Effects/Heat/GE_AddOrSubtractHeat.GE_AddOrSubtractHeat_C" :Level 1.0) "(TagName=\"Heat.Add\")" 5e+01))
  (GameplayEffects|ApplyGameplayEffectSpecToSelf PlayerAbilitySystem _returnvalue))

(fn ActivateAerialHitPhysics
  (bind _asbp_player_character (Utilities|Casting|CastToBP_PlayerCharacter (Variables|Default|GetPlayerActor)))
  (Character|LaunchCharacter _asbp_player_character (Variables|Default|GetLaunchForce) false false)
  (Ability|ApplyGameplayEffectToOwner "/Game/Blueprints/Player/GAS/Effects/GE_ApplyAerialHitPhysics.GE_ApplyAerialHitPhysics_C"))