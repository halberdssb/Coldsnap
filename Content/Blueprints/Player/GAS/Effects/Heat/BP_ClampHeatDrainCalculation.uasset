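; Gameplay Effect magnitude calculation that limits heat drain around a minimum heat threshold.
; It reads a captured attribute, presumably Heat, using source and target tags, then adds the base drain value to test the result.
; A drain that would cross from at or above the threshold to below it returns zero rather than a partial amount.
; Otherwise, including when already below the threshold, the full base drain applies.
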(fn CalculateBaseMagnitude
  (params (Spec :type Gameplay%20Effect%20Spec%20Structure%20%28by%20ref%29))
  (bind _returnvalue (Class|GameplayModMagnitudeCalculation|GetCapturedAttributeMagnitude Spec "(AttributeName=\"Heat\",Attribute=/Script/Coldsnap.HeatAttributeSet:Heat,AttributeOwner=\"/Script/CoreUObject.Class'/Script/Coldsnap.HeatAttributeSet'\")" (Class|GameplayModMagnitudeCalculation|GetSourceActorTags Spec) (Class|GameplayModMagnitudeCalculation|GetTargetActorTags Spec)))
  (if (and (>= _returnvalue (LocalVariables|GetMinimumHeatThreshold)) (< (+ _returnvalue (LocalVariables|GetBaseHeatDrainValue)) (LocalVariables|GetMinimumHeatThreshold)))
    (return 0.0)
    (else
      (return (LocalVariables|GetBaseHeatDrainValue)))))