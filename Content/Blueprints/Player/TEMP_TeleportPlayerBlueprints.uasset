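; A temporary player Blueprint holding draft logic for a teleport ability built on the Gameplay Ability System.
; Unconnected event graph nodes print a debug message, clear the dash ability, then grant and try to activate GA_Teleport, but never run.
; CheckHasTeleport sets HasTeleportAbility to true when the ability system component has the Player.Teleporting tag, and never resets it.
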(fn ConstructionScript)

(fn CheckHasTeleport
  (if (GameplayTags|HasMatchingGameplayTag (Ability|GetAbilitySystemComponent 0) "(TagName=\"Player.Teleporting\")")
    (Variables|Default|SetHasTeleportAbility true)
    (else
      (return))))