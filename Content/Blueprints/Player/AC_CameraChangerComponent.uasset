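; Actor component that changes the owning player character's camera FOV while dashing.
; On BeginPlay it validates the owner and starts a looping timer that drives the FOV update in place of Tick.
; While dashing, the dot product of velocity direction and actor forward blends default toward target FOV, so it follows direction rather than speed.
; Constant-rate interpolation uses separate in and out speeds, returning to default when not dashing.
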(event Custom|UpdateFOV
  (bind _blueprint_character (Variables|Default|GetBlueprint%20Character))
  (bind _camera (Variables|/Game/Blueprints/Player/BP_PlayerCharacter.BP_PlayerCharacter_C|GetCamera _blueprint_character))
  ;[0.15 0.05469 0.05532 0.5] FOV Resets when not Dashing
  (if (Variables|/Game/Blueprints/Player/BP_PlayerCharacter.BP_PlayerCharacter_C|GetisDashing (Variables|Default|GetBlueprint%20Character))
    ;[0.05869 0.15 0.04688 0.5] FOV Increases with Movement Speed (FOVTarget is Limit)
    (Variables|Default|SetForwardAlpha (Math|Vector|DotProduct (Math|Vector|Normalize (Variables|/Script/Engine.MovementComponent|GetVelocity (Pawn|GetMovementComponent (Variables|Default|GetBlueprint%20Character)))) (Transformation|GetActorForwardVector (Variables|Default|GetBlueprint%20Character))))
    (Camera|SetFieldOfView _camera (Math|Interpolation|FInterptoConstant (Variables|/Script/Engine.CameraComponent|GetFieldOfView _camera) (Math|Float|Lerp (Variables|Default|GetFOVDefault) (Variables|Default|GetFOVTarget) (Variables|Default|GetForwardAlpha)) (Utilities|Time|GetWorldDeltaSeconds) (Variables|Default|GetInterp%20Speed%20IN)))
    (else
      (Camera|SetFieldOfView (Variables|/Game/Blueprints/Player/BP_PlayerCharacter.BP_PlayerCharacter_C|GetCamera (Variables|Default|GetBlueprint%20Character)) (Math|Interpolation|FInterptoConstant (Variables|/Script/Engine.CameraComponent|GetFieldOfView (Variables|/Game/Blueprints/Player/BP_PlayerCharacter.BP_PlayerCharacter_C|GetCamera (Variables|Default|GetBlueprint%20Character))) (Variables|Default|GetFOVDefault) (Utilities|Time|GetWorldDeltaSeconds) (Variables|Default|GetInterp%20Speed%20OUT))))))

(event EventBeginPlay
  ;[0.06953 0.08598 0.15 0.5] Check for Player Character
  (bind _playerchar (Class|BIPlayerCharacter|AsPlayerCharacter(Message) (Components|GetOwner)))
  (Utilities|IsValid _playerchar
    (:Is%20Valid
      (Variables|Default|SetBlueprint%20Character _playerchar)
      (bind _returnvalue (Utilities|Time|SetTimerbyEvent (delegate Custom|UpdateFOV) (Variables|Default|GetUpdateTimerTime) true))
      (Variables|Default|SetUpdateTimerHandle _returnvalue))
    (:Is%20Not%20Valid
      (Development|PrintString "Not valid character"))))