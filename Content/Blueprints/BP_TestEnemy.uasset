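; BP_TestEnemy is a test enemy driven by a State Tree AI that reacts to hits with a stun and an upward knockback.
; On BeginPlay it caches its AI controller and that controller's StateTreeAIComponent.
; The Hit event sends an Enemy.Stunned event to the State Tree and switches the capsule to physics simulation.
; It waits one tick before applying the knockback force, so physics is already active.
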(event EventBeginPlay
  (CallFunction|GetAIController)
  (CallFunction|GetStateTree))

(event EventHit
  ;[0.15 0.15 0.15 0.5] Send Stunned Event On Hit
  (Gameplay|StateTree|SendStateTreeEvent (Variables|Default|GetAIStateTree) (Utilities|Struct|MakeStateTreeEvent "(TagName=\"Enemy.Stunned\")") :!class /Script/GameplayStateTreeModule.StateTreeComponent)
  ;[0.15 0.15 0.15 0.5] Enable Physics and Apply Force Next Frame
  (CallFunction|EnablePhysics)
  (Utilities|FlowControl|DelayUntilNextTick)
  (Class|Knockbackable|ApplyKnockback "0.000000,0.000000,1.000000" 1e+05))

(fn ConstructionScript)

(fn GetStateTree
  (bind _aicontroller (Variables|Default|GetAIController))
  (bind _returnvalue (Actor|GetComponentbyClass _aicontroller "/Script/GameplayStateTreeModule.StateTreeAIComponent"))
  ;[0.15 0.15 0.15 0.5] Get State Tree Reference
  (Utilities|IsValid _returnvalue
    (:Is%20Valid
      (Variables|Default|SetAIStateTree _returnvalue))))

(fn GetAIController
  (bind _self self)
  (bind _returnvalue (AI|GetAIController _self))
  ;[0.15 0.15 0.15 0.5] Get AI Controller Reference
  (Utilities|IsValid _returnvalue
    (:Is%20Valid
      (Variables|Default|SetAIController _returnvalue))))

(fn EnablePhysics
  (Physics|SetSimulatePhysics (Variables|Default|GetCapsuleComponent) true))