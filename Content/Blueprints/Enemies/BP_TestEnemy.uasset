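; Test enemy that gets stunned and knocked back when hit, drops core upgrades and attacks the player on contact.
; Hits send a stun event to the AI controller's State Tree, enable capsule physics for next-tick knockback, apply damage and roll drops, which also run on death.
; Drops spawn each item to read its DropChance, then scatter or destroy it.
; A temporary collision binding activates the granted GAS attack ability.
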(event EventBeginPlay
  (CallFunction|GetAIController)
  (CallFunction|GetStateTree)
  (Utilities|Array|Add (Variables|Default|GetDroppableItems) "/Game/Blueprints/Upgrades/BP_AgileCoreUpgrade.BP_AgileCoreUpgrade_C")
  (Utilities|Array|Add (Variables|Default|GetDroppableItems) "/Game/Blueprints/Upgrades/BP_BouncyCoreUpgrade.BP_BouncyCoreUpgrade_C")
  (CallFunction|AssignAttackTypes))

(event EventHit
  (params (damage :type Float%20%28single-precision%29) (knockbackForce :type Vector :default "0, 0, 0"))
  ;[0.15 0.15 0.15 0.5] Send Stunned Event On Hit
  (Gameplay|StateTree|SendStateTreeEvent (Variables|Default|GetAIStateTree) (Utilities|Struct|MakeStateTreeEvent "(TagName=\"Enemy.Stunned\")") :!class /Script/GameplayStateTreeModule.StateTreeComponent)
  ;[0.15 0.15 0.15 0.5] Enable Physics and Apply Force Next Frame
  (CallFunction|EnablePhysics)
  (Utilities|FlowControl|DelayUntilNextTick)
  (Class|Knockbackable|ApplyKnockback knockbackForce 1.0)
  (Game|Damage|ApplyDamage 0 0.0 0 0)
  (CallFunction|DropItems))

(event Collision|EventHit
  (params (MyComp :type Primitive%20Component%20Object%20Reference) (Other :type Actor%20Object%20Reference) (OtherComp :type Primitive%20Component%20Object%20Reference) (bSelfMoved :type Boolean) (HitLocation :type Vector :default "0, 0, 0") (HitNormal :type Vector :default "0, 0, 0") (NormalImpulse :type Vector :default "0, 0, 0") (Hit :type Hit%20Result%20Structure%20%28by%20ref%29))
  (CallFunction|AttackPlayer Other (* (Variables|Default|GetKnockbackDirection) (Variables|Default|GetKnockbackForce))))

(event EventDropItemsonDeath
  (CallFunction|DropItems))

(fn ConstructionScript)

(fn GetStateTree
  (bind _aicontroller (Variables|Default|GetAIController))
  (bind _returnvalue (Actor|GetComponentbyClass _aicontroller "/Script/GameplayStateTreeModule.StateTreeAIComponent"))
  ;[0.15 0.15 0.15 0.5] Get State Tree Reference
  (Utilities|IsValid _returnvalue
    (:Is%20Valid
      (Variables|Default|SetAIStateTree _returnvalue))))

(fn GetAIController
  (bind _self self)
  (bind _returnvalue (AI|GetAIController _self))
  ;[0.15 0.15 0.15 0.5] Get AI Controller Reference
  (Utilities|IsValid _returnvalue
    (:Is%20Valid
      (Variables|Default|SetAIController _returnvalue))))

(fn EnablePhysics
  (Physics|SetSimulatePhysics (Variables|Default|GetCapsuleComponent) true))

(fn DropItems
  (for _array_element (Variables|Default|GetDroppableItems)
    (bind _output_get (Variables|Default|SetrandomDropValue (Math|Random|RandomFloatinRange 0.0 1.0)))
    (bind _returnvalue (Game|SpawnActorfromClass _array_element (Transformation|GetActorTransform) "AdjustIfPossibleButAlwaysSpawn" "MultiplyWithRoot" 0 0))
    (if (> (Variables|/Game/Blueprints/Upgrades/BP_Upgrade.BP_Upgrade_C|GetDropChance _returnvalue) _output_get)
      (Transformation|SetActorLocation _returnvalue (+ (Transformation|GetActorLocation _returnvalue) (* (Math|Random|RandomUnitVector) (Variables|Default|GetItem%20Drop%20RandomRadius))) false false)
      (else
        (Actor|DestroyActor _returnvalue)))))

(fn AttackPlayer
  (params (Other :type Actor%20Object%20Reference) (KnockbackForce :type Vector))
  (Utilities|Casting|CastToBP_PlayerCharacter Other) ; Check if enemy collided w/player
  (Class|AbilitySystemComponent|TryActivateAbility (Variables|Default|GetAbilitySystemComponent) (Variables|Default|GetBaseEnemyAttack) true))

(fn AssignAttackTypes
  (bind _returnvalue (GameplayAbilities|GiveAbility (Variables|Default|GetAbilitySystemComponent) "/Game/Blueprints/Enemies/Attacks/GA_BaseEnemyAttack.GA_BaseEnemyAttack_C" 0 -1))
  (Variables|Default|SetBaseEnemyAttack _returnvalue))