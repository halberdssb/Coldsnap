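; Base Gameplay Ability for enemy attacks that hits the player character on activation.
; Unless the player is invulnerable, it applies a damage effect with SetByCaller magnitude from the difficulty-scaling actor's ScaledDamage, plus on-hit invulnerability, then calls the player's hit handler.
; A comment flags scaled damage as broken.
; Knockback is passed but unused, EndAbility is never called, and the death-check and KillPlayer helpers are not called here.
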(event Ability|EventActivateAbility
  (Variables|Default|SetThisActor (Components|GetOwner (Ability|GetAbilitySystemComponentfromActorInfo)))
  (bind _returnvalue (Actor|GetActorOfClass "/Game/Blueprints/Player/BP_PlayerCharacter.BP_PlayerCharacter_C"))
  (CallFunction|HitPlayer _returnvalue (* (Variables|Default|GetKnockbackDirection) (Variables|Default|GetKnockbackForce))))

(event Ability|EventOnEndAbility
  (params (bWasCancelled :type Boolean)))

(fn HitPlayer
  (params (Player :type Actor%20Object%20Reference) (KnockbackForce :type Vector))
  ;[0.15 0.15 0.15 0.5] Correct way of decreasing health
  (bind _asbp_player_character (Utilities|Casting|CastToBP_PlayerCharacter Player))
  (if (not (Variables|/Game/Blueprints/Player/BP_PlayerCharacter.BP_PlayerCharacter_C|GetIsInvulnerable _asbp_player_character))
    (bind _returnvalue (Actor|GetActorOfClass "/Game/Blueprints/Systems/DifficultyScaling/BP_GameStateDiffScaling.BP_GameStateDiffScaling_C"))
    (Development|PrintString (Utilities|String|Append "Scaled damage: " (Utilities|String|ToString(Float) (Variables|/Game/Blueprints/Systems/DifficultyScaling/BP_GameStateDiffScaling.BP_GameStateDiffScaling_C|GetScaledDamage _returnvalue))) true true "(R=1.000000,G=0.000000,B=0.867379,A=1.000000)" 1e+01)
    ;;[0.15 0.15 0.15 0.5] FIX THIS - scaled damage not working from director - not doing damage
    (bind _returnvalue_2 (Ability|GameplayEffect|AssignTagSetbyCallerMagnitude (GameplayEffects|MakeOutgoingSpec :self (Ability|GetAbilitySystemComponent (Variables|Default|GetThisActor)) :GameplayEffectClass "/Game/Blueprints/Player/GAS/Effects/GE_ApplyDamageToTarget.GE_ApplyDamageToTarget_C" :Level 1.0) "(TagName=\"Damage.Apply\")" (Variables|/Game/Blueprints/Systems/DifficultyScaling/BP_GameStateDiffScaling.BP_GameStateDiffScaling_C|GetScaledDamage _returnvalue)))
    (GameplayEffects|ApplyGameplayEffectSpecToTarget _returnvalue_2 (Ability|TargetData|AbilityTargetDatafromActor _asbp_player_character))
    (GameplayEffects|ApplyGameplayEffectToTarget (Ability|TargetData|AbilityTargetDatafromActor _asbp_player_character) "/Game/Blueprints/Player/GAS/Effects/GE_OnHitInvulnerability.GE_OnHitInvulnerability_C" 1 1)
    (Default|SetInvulnerable _asbp_player_character)
    ;[0.15 0.15 0.15 0.5] \Check for player death
    (Default|CallOnPlayerHit _asbp_player_character)))

(fn [DELETE?]CheckforPlayerDeath
  (params (Player :type Actor%20Object%20Reference))
  (bind _asbp_player_character (Utilities|Casting|CastToBP_PlayerCharacter Player))
  (if (<= (.ReturnValue (Ability|Attribute|GetFloatAttributefromAbilitySystemComponent (Ability|GetAbilitySystemComponent _asbp_player_character) "(AttributeName=\"Health\",Attribute=/Script/Coldsnap.HealthAttributeSet:Health,AttributeOwner=\"/Script/CoreUObject.Class'/Script/Coldsnap.HealthAttributeSet'\")")) 0.0)
    (Default|CallOnPlayerHit _asbp_player_character)))

(fn KillPlayer
  (Game|OpenLevel(byObjectReference) "/Game/Maps/Dev/MainMenu_Test.MainMenu_Test"))