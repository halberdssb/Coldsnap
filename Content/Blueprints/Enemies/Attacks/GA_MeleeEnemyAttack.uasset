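; Gameplay ability for an enemy melee attack that targets the player character.
; On activation, it runs a sphere overlap at a hitbox offset relative to the owner's transform, filtered to BP_PlayerCharacter.
; A hit copies MeleeDamage into Damage and hands off to the parent ability's activation, while a miss ends the ability immediately.
; A debug sphere draw is left disconnected.
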(event Ability|EventActivateAbility
  (bind _returnvalue (Collision|SphereOverlapActors (Math|Transform|TransformLocation (Transformation|GetActorTransform (Components|GetOwner (Ability|GetAbilitySystemComponentfromActorInfo))) (Variables|Default|GetAttackHitboxOffset)) (Variables|Default|GetAttackRadius) (Variables|Default|GetHitObjectTypes) "/Game/Blueprints/Player/BP_PlayerCharacter.BP_PlayerCharacter_C"))
  (if _returnvalue
    (Variables|Default|SetDamage (Variables|Default|GetMeleeDamage))
    (|CallParentFunction)
    (else
      (Ability|EndAbility))))

(event Ability|EventOnEndAbility
  (params (bWasCancelled :type Boolean))
  (|CallParentFunction bWasCancelled))