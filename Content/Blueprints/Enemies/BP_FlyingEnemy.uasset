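; Flying bomb enemy that launches at the player and can be knocked back to stun enemies.
; A timeline sweeps the mesh along a spline whose last point snaps to the player's location at launch, then destroys the actor after a short delay.
; Hits from an attacking player enable physics and apply an impulse along the player's forward vector.
; Once reflected, hitting the final boss stuns it and the parent enemy.
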(event Custom|OnActorHit_Event
  (params (SelfActor :type Actor%20Object%20Reference) (OtherActor :type Actor%20Object%20Reference) (NormalImpulse :type Vector) (Hit :type Hit%20Result%20Structure%20%28by%20ref%29))
  (bind _asbp_player_character (Utilities|Casting|CastToBP_PlayerCharacter OtherActor)
    (:then
      ;[0.15 0.15 0.15 0.5] Hits player
      (if (Variables|/Game/Blueprints/Player/BP_PlayerCharacter.BP_PlayerCharacter_C|GetIsAttacking _asbp_player_character) ; Reflect back
        (CallFunction|EventHitBack)))
    (:CastFailed
      ;[0.15 0.15 0.15 0.5] Hit enemy
      (bind _asbp_final_boss (Utilities|Casting|CastToBP_FinalBoss OtherActor))
      (if (Variables|Default|GetCanStun)
        (Default|GetStunnedfromBomb (Variables|Default|GetParentEnemy))))))

(event Custom|Event_MoveObject
  (bind _spline (Variables|Default|GetSpline))
  ;[0.15 0.15 0.15 0.5] Launch bomb
  (Default|CallEventPlayHone)
  (CallFunction|MoveSplinetoPlayerPos)
  (Components|Timeline|SetPlayRate (Variables|Default|GetFlightMovement) (/ 1.0 (Variables|Default|GetLengthOfSpline)))
  (bind _newtrack_0 (Timeline|FlightMovement Play) ; Use timeline to move bomb
    (:Update
      ;[0.15 0.15 0.15 0.5] Move and set transform of bomb on spline
      (Transformation|SetWorldTransform (Variables|Character|GetMesh) (Math|Transform|MakeTransform (Spline|GetLocationatDistanceAlongSpline _spline (Math|Float|Lerp 0.0 (Spline|GetSplineLength _spline) (/ _newtrack_0 1.0)) "World") (Spline|GetRotationatDistanceAlongSpline _spline (Math|Float|Lerp 0.0 (Spline|GetSplineLength _spline) (/ _newtrack_0 1.0)) "World")) true false))
    (:Finished
      (Default|CallEventPlayHone)
      (Utilities|FlowControl|Delay 1.2) ; Let anim play
      (Actor|DestroyActor))))

(event Custom|Event_HitBack
  (bind _playerref (Variables|Default|GetPlayerRef))
  (bind _hitforce (Variables|Default|GetHitForce))
  (bind _returnvalue (Transformation|GetActorForwardVector _playerref))
  (bind _returnvalue_2 (Math|Vector|Normalize _returnvalue))
  (bind _returnvalue_3 (* _returnvalue_2 _hitforce))
  (bind (_x _y) (Math|Vector|BreakVector _returnvalue_3))
  ;[0.15 0.15 0.15 0.5] Hit back when hit by player
  (Physics|SetSimulatePhysics (Variables|Character|GetMesh) true) ; Allows bomb to be affected by physics\nOtherwise should not be to allow proper spline movement
  (Physics|AddImpulse (Variables|Character|GetMesh) (Math|Vector|MakeVector _x _y 1e+02) "None" false)
  (Variables|Default|SetCanStun true))

(event EventBeginPlay
  (|CallParentFunction)
  (Collision|BindEventtoOnActorHit (delegate Custom|OnActorHit_Event)))

(event Collision|EventActorBeginOverlap
  (params (OtherActor :type Actor%20Object%20Reference)))

(fn ConstructionScript
  (|CallParentFunction))

(fn MoveSplinetoPlayerPos
  (bind _spline (Variables|Default|GetSpline))
  (Spline|SetLocationatSplinePoint _spline (- (Spline|GetNumberOfSplinePoints _spline) 1) (Transformation|GetActorLocation (Variables|Default|GetPlayerRef)) "World" true))

(fn DebugTool
  (Utilities|Casting|CastToAIC_FlyingEnemy (AI|GetAIController 0)))