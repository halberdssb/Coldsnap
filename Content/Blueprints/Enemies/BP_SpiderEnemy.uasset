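; BP_SpiderEnemy is a spider enemy Blueprint built on a parent enemy class.
; On BeginPlay it sets up the hit-flash material on its skeletal mesh and registers that mesh as UsedSkeletalMesh before calling parent logic.
; Its DropItems function destroys the actor on death, with an alternative deactivation path left disconnected.
; The construction script only calls the parent, leaving dynamic material creation nodes unwired.
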(event EventBeginPlay
  (bind _skeletalmesh (Variables|Default|GetSkeletalMesh))
  (CallFunction|AssignHitFlashMat _skeletalmesh)
  (Variables|Default|SetUsedSkeletalMesh _skeletalmesh)
  (|CallParentFunction))

(event Collision|EventActorBeginOverlap
  (params (OtherActor :type Actor%20Object%20Reference)))

(event EventTick
  (params (DeltaSeconds :type Float%20%28single-precision%29)))

(fn ConstructionScript
  (|CallParentFunction))

(fn DropItems0
  (Actor|DestroyActor) ; On death, destroy actor in event that this is the method we want to take
)