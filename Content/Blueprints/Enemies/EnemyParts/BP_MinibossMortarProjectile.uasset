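; Miniboss mortar projectile that flies along a spline toward the player.
; A timeline sweeps the box along the spline at a rate set by LengthOfSpline, then plays VFX and destroys the actor.
; After a delay it moves the spline's last point to the player, then keeps refreshing it on timeline updates.
; Any hit plays VFX, but only a player hit calls ActivateMortarAttack on the miniboss and destroys the projectile.
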(event Custom|OnActorHit_Event
  (params (SelfActor :type Actor%20Object%20Reference) (OtherActor :type Actor%20Object%20Reference) (NormalImpulse :type Vector) (Hit :type Hit%20Result%20Structure%20%28by%20ref%29))
  (Components|Activation|Activate (Variables|Default|GetAttackVFX) false)
  (CallFunction|DestroyProjectile OtherActor))

(event Custom|MoveObject
  (bind _spline (Variables|Default|GetSpline))
  ;[0.15 0.01875 0.01875 0.5] COntrol movement of projectile object along a spline
  (Components|Timeline|SetPlayRate (Variables|Default|GetMoveAlongSpline) (/ 1.0 (Variables|Default|GetLengthOfSpline)))
  (bind _distance (Timeline|MoveAlongSpline Play)
    (:Update
      (Transformation|SetWorldTransform (Variables|Default|GetBox) (Math|Transform|MakeTransform (Spline|GetLocationatDistanceAlongSpline _spline (Math|Float|Lerp 0.0 (Spline|GetSplineLength _spline) (/ _distance 1.0)) "World") (Spline|GetRotationatDistanceAlongSpline _spline (Math|Float|Lerp 0.0 (Spline|GetSplineLength _spline) (/ _distance 1.0)) "World")) true false)
      ;[0.1173 0.04458 0.15 0.5] Find  player position once at apex of curve
      (Utilities|IsValid (Variables|Default|GetSpline) ; Prevent null errors after projectile is destroyed
        (:Is%20Valid
          (if (>= (Math|Float|Lerp 0.0 (Spline|GetSplineLength _spline) (/ _distance 1.0)) (* (Math|Float|Lerp 0.0 (Spline|GetSplineLength _spline) (/ _distance 1.0)) 0.66)) ; Check if past halfway point
            (if (not (Utilities|Operators|EqualEqual :B (Variables|Default|GetTargetPosition))) ; Check if player has been set already
              (CallFunction|GetPlayerPosition))))))
    (:Finished
      (Components|Activation|Activate (Variables|Default|GetAttackVFX) false)
      (Actor|DestroyActor))))

(event EventBeginPlay
  (EventDispatchers|BindEventtoOnActorHit (delegate Custom|OnActorHit_Event))
  (CallFunction|MoveObject)
  (Utilities|FlowControl|Delay (Variables|Default|GetLifetimeToGetPlayerPos))
  (CallFunction|GetPlayerPosition)
  (Transformation|SetAbsolute (Variables|Default|GetSpline) true false false))

(event EventTick
  (params (DeltaSeconds :type Float%20%28single-precision%29)))

(fn ConstructionScript)

(fn GetPlayerPosition
  (bind _returnvalue (Actor|GetActorOfClass "/Game/Blueprints/Player/BP_PlayerCharacter.BP_PlayerCharacter_C"))
  (Variables|Default|SetTargetPosition (Transformation|GetActorLocation _returnvalue))
  (CallFunction|ResetEndPtSpline))

(fn DestroyProjectile
  (params (HitActor :type Actor%20Object%20Reference))
  (if (Class|GameplayStatics|ObjectIsA HitActor "/Game/Blueprints/Player/BP_PlayerCharacter.BP_PlayerCharacter_C") ; Should do damage on collision with player, else ignore pawns
    (Default|ActivateMortarAttack (Variables|Default|GetEnemMiniboss))
    (Actor|DestroyActor)))

(fn ResetEndPtSpline
  (bind _spline (Variables|Default|GetSpline))
  (Spline|SetLocationatSplinePoint _spline (- (Spline|GetNumberOfSplinePoints _spline) 1) (Variables|Default|GetTargetPosition) "World" true))