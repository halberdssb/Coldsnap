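; Projectile fired by a ranged enemy that damages the player through the shooter's Gameplay Ability System.
; On hit it activates the attack VFX, and a player hit triggers the first ability on the stored Enemy's ability system component, then destroys the projectile.
; Hits on other actors also destroy it, except the shooter set through SetEnemy.
; Tick destroys it once it travels beyond DestroyDistance from its start position.
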(event Custom|OnActorHit_Event
  (params (SelfActor :type Actor%20Object%20Reference) (OtherActor :type Actor%20Object%20Reference) (NormalImpulse :type Vector) (Hit :type Hit%20Result%20Structure%20%28by%20ref%29))
  (Components|Activation|Activate (Variables|Default|GetAttackVFX) false)
  (CallFunction|DamagePlayer OtherActor))

(event EventBeginPlay
  (EventDispatchers|BindEventtoOnActorHit (delegate Custom|OnActorHit_Event))
  (Variables|Default|SetStartPos (Transformation|GetActorLocation)))

(event EventTick
  (params (DeltaSeconds :type Float%20%28single-precision%29))
  (CallFunction|DestroyAfterDistance))

(fn ConstructionScript)

(fn DamagePlayer
  (params (OverlappedObj :type Actor%20Object%20Reference))
  (bind _enemy (Variables|Default|GetEnemy))
  (bind _returnvalue (Ability|GetAbilitySystemComponent _enemy))
  (if (Class|GameplayStatics|ObjectIsA OverlappedObj "/Game/Blueprints/Player/BP_PlayerCharacter.BP_PlayerCharacter_C")
    (bind _outabilityhandles (Class|AbilitySystemComponent|GetAllAbilities _returnvalue))
    (Class|AbilitySystemComponent|TryActivateAbility _returnvalue (Utilities|Array|Get(acopy) _outabilityhandles) true) ; Activate the damage ability
    (Actor|DestroyActor)
    (elif (not (== OverlappedObj (Variables|Default|GetEnemy))) ; Check if hit actor is shooting enemy, otherwise destroy
      (Actor|DestroyActor))))

(fn SetEnemy
  (params (ThisEnemy :type BP%20Base%20Enemy%20Object%20Reference))
  (Variables|Default|SetEnemy ThisEnemy))

(fn DestroyAfterDistance
  (if (> (Math|Vector|Distance(Vector) (Variables|Default|GetStartPos) (Transformation|GetActorLocation)) (LocalVariables|GetDestroyDistance))
    (Actor|DestroyActor)))