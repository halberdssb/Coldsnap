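; Miniboss enemy Blueprint that can turn to face the player and fire a mortar attack.
; On BeginPlay it runs the parent setup and assigns a hit-flash material; while IsRotating is set, Tick blends its rotation halfway toward the player.
; ActivateMortarAttack triggers MortarAbility through the Ability System Component, ignoring its Ability input.
; The external ram event is a stub that only casts the AI controller, and the rotation-stop check is unconnected.
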(event Custom|Event_StartRam
  (bind _asaic_miniboss_enemy (Utilities|Casting|CastToAIC_MinibossEnemy (AI|GetAIController self))))

(event Custom|Event_SmoothTurn
  (params (Start :type Rotator) (RotateToFace :type Vector))
  (Transformation|SetActorRotation (Math|Rotator|Lerp(Rotator) Start (Math|Rotator|FindLookatRotation (Transformation|GetActorLocation) RotateToFace) 0.5 true)))

(event EventBeginPlay
  (|CallParentFunction)
  (CallFunction|AssignHitFlashMat (Variables|Character|GetMesh)))

(event Collision|EventActorBeginOverlap
  (params (OtherActor :type Actor%20Object%20Reference)))

(event EventTick
  (params (DeltaSeconds :type Float%20%28single-precision%29))
  (if (Variables|Default|GetIsRotating)
    (CallFunction|EventSmoothTurn (Transformation|GetActorRotation) (Transformation|GetActorLocation (Variables|Default|GetPlayerRef)))))

(fn ConstructionScript
  (|CallParentFunction))

(fn ActivateMortarAttack
  (params (Ability :type Gameplay%20Ability%20Spec%20Handle%20Structure))
  (Class|AbilitySystemComponent|TryActivateAbility (Variables|Default|GetAbilitySystemComponent) (Variables|Default|GetMortarAbility) true))