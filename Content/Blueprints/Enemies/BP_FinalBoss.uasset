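; Final boss enemy that runs a tracked laser attack, detects stomp landings and patrols level tracker points sorted by distance.
; Timers replace Tick, narrowing two warning traces on the player until close or timed out, then lasers fire at the locked position and damage through GAS.
; Capsule hits on blocking volumes, backed by a timed height check, advance the stomp phase via the AI controller.
; StateTree events signal stun and laser end.
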(event OnComponentHit(CapsuleComponent)
  (params (HitComponent :type Primitive%20Component%20Object%20Reference) (OtherActor :type Actor%20Object%20Reference) (OtherComp :type Primitive%20Component%20Object%20Reference) (NormalImpulse :type Vector :default "0, 0, 0") (Hit :type Hit%20Result%20Structure%20%28by%20ref%29))
  (CallFunction|EnterSecondStompPhase OtherActor false))

(event Custom|Event_StartWarnings
  (params (Duration :type Float%20%28double-precision%29))
  ;[0.15 0.15 0.15 0.5] Avoid using tick event
  (bind _returnvalue (Utilities|Time|SetTimerbyEvent (delegate Custom|Event_CheckMultFrames) 0.05 true))
  (Variables|Default|SetUpdateTimer _returnvalue)
  (Variables|/Script/Engine.CharacterMovementComponent|SetMaxWalkSpeed (Variables|Character|GetCharacterMovement) 0.0)
  (CallFunction|TrackPlayerWarningVFX Duration)
  ;[0.15 0.15 0.15 0.5] Prevent warnings from lasting forever if the player keeps moving out of the way
  (Utilities|FlowControl|Delay (Variables|Default|GetWarningTimeout))
  (if (not (Variables|Default|GetIsShootingonfinal)) ; Run once
    (CallFunction|SwitchtoLazers)))

(event Custom|Event_EndLazer
  (if (Variables|Default|GetIsShootingonfinal)
    (Utilities|FlowControl|Delay (Variables|Default|GetLazerDuration))
    (Variables|Default|SetIsShootingonfinal false)
    (CallFunction|DeactivateLazer)
    (CallFunction|EndLazer)))

(event Custom|Event_CheckMultFrames
  ;[0.15 0.15 0.15 0.5] Check if enemy is currently tracking player pos or attacking
  (if (Variables|Default|GetTracking)
    (CallFunction|MoveWarningsTowardPlayer (Utilities|Time|GetWorldDeltaSeconds))
    (elif (Variables|Default|GetIsShootingonfinal)
      (bind _playerhit (CallFunction|LazerAttack))
      (CallFunction|DoDamage _playerhit))))

(event Custom|Event_InternalTick
  (bind _returnvalue (Transformation|GetActorLocation))
  (bind _playerref (Variables|Default|GetPlayerRef))
  (bind _z (Math|Vector|BreakVector _returnvalue))
  (bind _returnvalue_2 (Transformation|GetActorLocation _playerref))
  (bind _z_2 (Math|Vector|BreakVector _returnvalue_2))
  (bind _returnvalue_3 (- _z_2 _z))
  ;[0.15 0.15 0.15 0.5] Backup for testing if enemy has landed
  (if (Math|Float|InRange(Float) (Math|Float|Absolute(Float) _returnvalue_3) 0.0 (Variables|Default|GetMaxRangeForStompLand))
    (CallFunction|EnterSecondStompPhase 0 true :!label _label)
    (elif (< _returnvalue_3 0.0)
      (goto _label))))

(event EventBeginPlay
  (|CallParentFunction)
  (CallFunction|SortTrackersbyDistance)
  (Utilities|Time|SetTimerbyEvent (delegate Custom|Event_InternalTick) 0.3 true) ; Avoid tick
)

(fn ConstructionScript)

(fn DropItems0)

(fn TrackPlayerWarningVFX
  (params (WarningDuration :type Float%20%28double-precision%29))
  (bind _playerref (Variables|Default|GetPlayerRef))
  (bind _returnvalue (Transformation|GetActorLocation _playerref))
  (bind (_x _y _z) (Math|Vector|BreakVector _returnvalue))
  (if (not (Variables|Default|GetIsShootingonfinal)) ; Do not track while shooting
    (Variables|Default|SetWarningDuration WarningDuration)
    (CallFunction|SetWarningVFX (LocalVariables|GetZOffset))
    ;[0.15 0.15 0.15 0.5] Calc offset of warning poses
    (bind _output_get (Variables|Default|SetWarning1Offset (Math|Vector|MakeVector _x (+ _y 2.5e+02) _z)))
    (bind _output_get_2 (Variables|Default|SetWarning2Offset (Math|Vector|MakeVector _x (- _y 2.5e+02) _z)))
    ;[0.15 0.15 0.15 0.5] Set warning VFX location
    (Transformation|SetWorldLocation (Variables|Default|GetNS_FinalBossWarning1) _output_get false false)
    (Transformation|SetWorldLocation (Variables|Default|GetNS_FinalBossWarning2) _output_get_2 false false)))

(fn MoveWarningsTowardPlayer
  (params (DeltaLerp :type Float%20%28double-precision%29))
  (bind _playerref (Variables|Default|GetPlayerRef))
  (bind _playerref_2 (Variables|Default|GetPlayerRef))
  (bind _returnvalue (Transformation|GetActorLocation _playerref))
  (bind _returnvalue_2 (Transformation|GetActorLocation _playerref_2))
  (bind (_x _y _z) (Math|Vector|BreakVector _returnvalue))
  (bind (_x_2 _y_2 _z_2) (Math|Vector|BreakVector _returnvalue_2))
  ;[0.15 0.15 0.15 0.5] Waring 1
  (bind _outhit (Collision|LineTraceByChannel (Transformation|GetActorLocation) (Variables|Default|GetWarning1Offset) "TraceTypeQuery1" false 0 "None"))
  (Niagara|SpawnSystematLocation "/Game/Art/ParticleEffects/Placeholders/NS_FinalBossWarning.NS_FinalBossWarning" (.TraceEnd (Collision|BreakHitResult _outhit))) ; Spawn warning particles
  ;;[0 0 0 0.5] Calculations
  (Variables|Default|SetTimeSinceStartWarning (+ (Variables|Default|GetTimeSinceStartWarning) DeltaLerp))
  (Variables|Default|SetWarning1Offset (Math|Vector|MakeVector _x_2 (Math|Float|Lerp (.Y (Math|Vector|BreakVector (.TraceEnd (Collision|BreakHitResult _outhit)))) _y_2 0.05) _z_2))
  ;[0.15 0.15 0.15 0.5] Waring 2
  (bind _outhit_2 (Collision|LineTraceByChannel (Transformation|GetActorLocation) (Variables|Default|GetWarning2Offset) "TraceTypeQuery1" false 0 "None"))
  (Niagara|SpawnSystematLocation "/Game/Art/ParticleEffects/Placeholders/NS_FinalBossWarning.NS_FinalBossWarning" (.TraceEnd (Collision|BreakHitResult _outhit_2))) ; Spawn warning  particles
  (Variables|Default|SetWarning2Offset (Math|Vector|MakeVector _x (Math|Float|Lerp (.Y (Math|Vector|BreakVector (Variables|Default|GetWarning2Offset))) _y 0.05) _z))
  ;[0.15 0.15 0.15 0.5] Check if narrowed in on player
  (if (Utilities|Operators|EqualEqual (.TraceEnd (Collision|BreakHitResult _outhit_2)) (Transformation|GetActorLocation (Variables|Default|GetPlayerRef)) 1e+01)
    (if (not (Variables|Default|GetIsShootingonfinal)) ; Run once
      (Utilities|Time|ClearandInvalidateTimerbyHandle (Variables|Default|GetUpdateTimer))
      (CallFunction|SwitchtoLazers))))

(fn LazerAttack
  ;[0.15 0.15 0.15 0.5] Lazer 2
  (bind _outhit (Collision|LineTraceByChannel (Transformation|GetWorldLocation (Variables|Default|GetNS_FinalBossLazer2)) (Variables|Default|GetLazerEndPos) "TraceTypeQuery1" false 0 "ForDuration" true "(R=1.000000,G=0.000000,B=0.000000,A=1.000000)" "(R=0.000000,G=1.000000,B=0.000000,A=1.000000)" 1.0)) ; Functio
  (Utilities|Casting|CastToBP_PlayerCharacter (.HitActor (Collision|BreakHitResult _outhit))
    (:then
      (return true))
    (:CastFailed
      ;[0.15 0.15 0.15 0.5] Lazer 1
      (bind _outhit_2 (Collision|LineTraceByChannel (Transformation|GetWorldLocation (Variables|Default|GetNS_FinalBossLazer1)) (Variables|Default|GetLazerEndPos) "TraceTypeQuery1" false 0 "ForOneFrame" true "(R=1.000000,G=0.000000,B=0.000000,A=1.000000)" "(R=0.000000,G=1.000000,B=0.000000,A=1.000000)" 1.0)) ; Functio
      (Utilities|Casting|CastToBP_PlayerCharacter (.HitActor (Collision|BreakHitResult _outhit_2))
        (:then
          (return true))
        (:CastFailed
          (return false))))))

(fn SetLazerVis
  (bind _ns_finalbosslazer2 (Variables|Default|GetNS_FinalBossLazer2))
  (bind _ns_finalbosslazer1 (Variables|Default|GetNS_FinalBossLazer1))
  (bind _ns_finalbosswarning2 (Variables|Default|GetNS_FinalBossWarning2))
  (bind _ns_finalbosswarning1 (Variables|Default|GetNS_FinalBossWarning1))
  ;[0.15 0.15 0.15 0.5] Lazer
  (Rendering|SetVisibility _ns_finalbosslazer2 true false)
  (Rendering|SetVisibility _ns_finalbosslazer1 true false)
  (Components|Activation|Activate _ns_finalbosslazer2 false)
  (Components|Activation|Activate _ns_finalbosslazer1 false)
  ;[0.15 0.15 0.15 0.5] Warnings
  (Rendering|SetVisibility _ns_finalbosswarning1 false false)
  (Rendering|SetVisibility _ns_finalbosswarning2 false false)
  (Components|Activation|Deactivate _ns_finalbosswarning1)
  (Components|Activation|Deactivate _ns_finalbosswarning2))

(fn DoDamage
  (params (ShouldDoDamage :type Boolean))
  (bind _abilitysystemcomponent (Variables|Default|GetAbilitySystemComponent))
  (if ShouldDoDamage
    (bind _outabilityhandles (Class|AbilitySystemComponent|GetAllAbilities _abilitysystemcomponent))
    (Class|AbilitySystemComponent|TryActivateAbility _abilitysystemcomponent (Utilities|Array|Get(acopy) _outabilityhandles) true) ; Activate the damage ability
  ))

(fn DeactivateLazer
  (bind _ns_finalbosslazer2 (Variables|Default|GetNS_FinalBossLazer2))
  (bind _ns_finalbosslazer1 (Variables|Default|GetNS_FinalBossLazer1))
  (Rendering|SetVisibility _ns_finalbosslazer2 false false)
  (Components|Activation|Deactivate _ns_finalbosslazer2)
  (Rendering|SetVisibility _ns_finalbosslazer1 false false)
  (Components|Activation|Deactivate _ns_finalbosslazer1))

(fn GetStunnedfromBomb
  (Gameplay|StateTree|SendStateTreeEvent (Variables|Default|GetAIStateTree) (Utilities|Struct|MakeStateTreeEvent "(TagName=\"Enemy.Stunned\")") :!class /Script/GameplayStateTreeModule.StateTreeComponent))

(fn EndLazer
  (Gameplay|StateTree|SendStateTreeEvent (Variables|Default|GetAIStateTree) (Utilities|Struct|MakeStateTreeEvent "(TagName=\"Enemy.LazerStateEnd\")") :!class /Script/GameplayStateTreeModule.StateTreeComponent))

(fn SetWarningVFX
  (params (Offset :type Float%20%28double-precision%29))
  (bind _ns_finalbosswarning1 (Variables|Default|GetNS_FinalBossWarning1))
  (bind _ns_finalbosswarning2 (Variables|Default|GetNS_FinalBossWarning2))
  ;[0.15 0.15 0.15 0.5] Warning VFX visibility
  (Variables|Default|SetTracking true)
  (Rendering|SetVisibility _ns_finalbosswarning1 true false)
  (Rendering|SetVisibility _ns_finalbosswarning2 true false)
  ;[0.15 0.15 0.15 0.5] VFX activation
  (Components|Activation|Activate _ns_finalbosswarning1 false)
  (Components|Activation|Activate _ns_finalbosswarning2 false))

(fn SwitchtoLazers
  ;[0 0 0 0.5] Switch to lazer attacking portion of task
  (Variables|Default|SetIsShootingonfinal true)
  (Variables|Default|SetTracking false)
  (CallFunction|SetLazerVis)
  (Variables|Default|SetLazerEndPos (Transformation|GetActorLocation (Variables|Default|GetPlayerRef)))
  (CallFunction|EventEndLazer))

(fn SortTrackersbyDistance
  (bind _returnvalue (Transformation|GetActorLocation))
  ;[0.15 0.15 0.15 0.5] Get trackers and set in array
  (bind _outactors (Actor|GetAllActorsOfClass "/Game/Blueprints/Enemies/EnemyParts/BP_FinalBossTracker.BP_FinalBossTracker_C"))
  (bind _output_get (Variables|Default|SetMovementTrackers _outactors))
  ;[0.15 0.15 0.15 0.5] Selection sort points in level based on distance from boss"s starting location
  (for (_ _array_index) _output_get
    (bind _output_get_2 (LocalVariables|SetMinIdx _array_index))
    ;;[0.007292 0.007292 0.007292 0.5] Inner loop
    (for _index (range _output_get_2 (Utilities|Array|LastIndex (Variables|Default|GetMovementTrackers)))
      (if (< (Math|Vector|Distance(Vector) (Transformation|GetActorLocation (Utilities|Array|Get(acopy) (Variables|Default|GetMovementTrackers) _index)) _returnvalue) (Math|Vector|Distance(Vector) _returnvalue (Transformation|GetActorLocation (Utilities|Array|Get(acopy) (Variables|Default|GetMovementTrackers) _output_get_2))))
        (LocalVariables|SetMinIdx _index)))
    ;;[0.7365 0.7365 0.7365 0.5] Outer loop
    (LocalVariables|SetTmp (Utilities|Array|Get(acopy) (Variables|Default|GetMovementTrackers) _array_index))
    (Utilities|Array|SetArrayElem (Variables|Default|GetMovementTrackers) _array_index (Utilities|Array|Get(acopy) (Variables|Default|GetMovementTrackers) (LocalVariables|GetMinIdx)))
    (Utilities|Array|SetArrayElem (Variables|Default|GetMovementTrackers) (LocalVariables|GetMinIdx) (LocalVariables|GetTmp))))

(fn SetNewMovePt
  (if (> (+ (Variables|Default|GetCurrentMovePt) 1) (Utilities|Array|LastIndex (Variables|Default|GetMovementTrackers))) ; Check if at end of array
    (Variables|Default|SetCurrentMovePt 0)
    (else
      (Variables|Default|SetCurrentMovePt (+ (Variables|Default|GetCurrentMovePt) 1)))))

(fn GetCurrentMoveVector
  (bind _returnvalue (Transformation|GetActorLocation))
  (bind _movementtrackers (Variables|Default|GetMovementTrackers))
  (bind _currentmovept (Variables|Default|GetCurrentMovePt))
  (bind _output (Utilities|Array|Get(acopy) _movementtrackers _currentmovept))
  (bind _returnvalue_2 (Transformation|GetActorLocation _output))
  (bind (_x _y) (Math|Vector|BreakVector _returnvalue_2))
  (Utilities|IsValid _output
    (:Is%20Valid
      (return (Math|Vector|MakeVector _x _y (.Z (Math|Vector|BreakVector _returnvalue)))))
    (:Is%20Not%20Valid
      (return _returnvalue) ; Return own position if invalid location found
    )))

(fn EnterSecondStompPhase
  (params (OverlappedObj :type Object%20Object%20Reference) (CalledFromInternalTick :type Boolean))
  (if (Variables|Default|GetIsJumping)
    (Utilities|IsValid OverlappedObj
      (:Is%20Valid
        (Utilities|Casting|CastToBlockingVolume OverlappedObj) ; Check boss hit ground
        (bind _asaic_final_boss_enemy (Utilities|Casting|CastToAIC_FinalBossEnemy (Variables|Default|GetAIController) :!label _label))
        (Default|EventTriggerStompPhaseChange _asaic_final_boss_enemy)
        (Variables|Default|SetIsJumping false)
        (Default|CallPlayLookAnim))
      (:Is%20Not%20Valid
        (if CalledFromInternalTick
          (goto _label))))))