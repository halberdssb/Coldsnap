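; Base enemy Blueprint handling combat, hit reactions, death with bounty and item drops, and director-reported despawning.
; On possession or BeginPlay it caches its AI controller, State Tree, player and director, then grants a GAS attack.
; Hits send a stun event, apply physics knockback and damage, then trigger death or montage and material flash.
; Attacks use temporary collision checks and borrow tokens from the player; helpers toggle activity by player distance.
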(event Custom|Event_ControlMaterialFlash
  ;[0.15 0.15 0.15 0.5] Control color change on hit
  (if (Variables|HitFeedback|GetFadeIn)
    (CallFunction|ColorFlashonHit)
    (Utilities|FlowControl|Delay 0.05)
    (CallFunction|EventControlMaterialFlash)
    (else
      (CallFunction|ColorFlashonHit)
      (Utilities|FlowControl|Delay 0.05)
      (if (Variables|HitFeedback|GetFadeInProgress)
        (CallFunction|EventControlMaterialFlash)))))

(event Custom|OnDamageTaken_Event
  (bind _returnvalue (Ability|GetAbilitySystemComponent 0))
  (bind (_bsuccessfullyfoundattribute _returnvalue_2) (Ability|Attribute|GetFloatAttributefromAbilitySystemComponent _returnvalue "(AttributeName=\"Health\",Attribute=/Script/Coldsnap.HealthAttributeSet:Health,AttributeOwner=\"/Script/CoreUObject.Class'/Script/Coldsnap.HealthAttributeSet'\")"))
  (if _bsuccessfullyfoundattribute
    (if (<= _returnvalue_2 0.0)
      (CallFunction|OnDeath)
      (else
        (CallFunction|VFXonHit)
        (Utilities|IsValid (Variables|Default|GetHitMontage)
          (:Is%20Valid
            (CallFunction|PlayHitAnim)))))
    (else
      (Development|PrintString "ERROR: COULD NOT FIND ENEMY HELATH ATTRIBUTE ON HIT" true true "(R=1.000000,G=0.010033,B=0.000043,A=1.000000)"))))

(event Custom|Event_OpenAttackWindow
  ;[0.15 0.15 0.15 0.5] Enable attacking
  (Variables|Default|SetisAttacking true)
  (Utilities|FlowControl|Delay 3.0) ; Margin of error
  (Variables|Default|SetisAttacking false))

(event Custom|Event_ActivateHitbox
  (params (HitActors :type Array%20of%20Actor%20Object%20References) (HitboxData :type Hitbox%20Data%20Structure))
  ;[0.15 0.15 0.15 0.5] Testing hitbox - not fully functional yet
  (for _array_element HitActors
    (Development|PrintString (Utilities|GetDisplayName _array_element) true true "(R=0.914639,G=0.180610,B=1.000000,A=1.000000)")))

(event Custom|DespawnSetup
  ;[0.15 0.15 0.15 0.5] Despawn functions
  (Variables|DespawnVariables|SetSpawnTime (Utilities|Time|GetGameTimeinSeconds))
  (Variables|DespawnVariables|SetLastCombatTime (Variables|DespawnVariables|GetSpawnTime)))

(event Custom|RequestDespawn
  ;[0.15 0.15 0.15 0.5] Despawn functions
  (Variables|/Game/Blueprints/Systems/DirectorSystem/BP_Director.BP_Director_C|SetWasDespawned (Variables|References|GetDirectorRef) true)
  (Collision|SetCollisionEnabled (Variables|Default|GetCapsuleComponent) "NoCollision")
  (AI|Logic|StopLogic (Variables|Default|GetAIStateTree) "")
  (Actor|DestroyActor (Variables|Default|GetAIController))
  (Actor|DestroyActor))

(event Custom|UpdateLastCombatTime
  ;[0.15 0.15 0.15 0.5] Despawn functions
  (Variables|DespawnVariables|SetLastCombatTime (Utilities|Time|GetGameTimeinSeconds)))

(event EventBeginPlay
  (|CallParentFunction)
  (CallFunction|GetAIController)
  (CallFunction|GetStateTree)
  (CallFunction|AssignAttackTypes)
  (CallFunction|GetReferences)
  (Variables|Default|SetEnemyEnabled true)
  (CallFunction|DespawnSetup))

(event EventHit
  (params (damage :type Float%20%28single-precision%29) (knockbackForce :type Vector :default "0, 0, 0"))
  ;[0.15 0.15 0.15 0.5] Send Stunned Event On Hit
  (Gameplay|StateTree|SendStateTreeEvent (Variables|Default|GetAIStateTree) (Utilities|Struct|MakeStateTreeEvent "(TagName=\"Enemy.Stunned\")") :!class /Script/GameplayStateTreeModule.StateTreeComponent)
  ;[0.15 0.15 0.15 0.5] Enable Physics and Apply Force Next Frame
  (CallFunction|EnablePhysics)
  (Utilities|FlowControl|DelayUntilNextTick)
  (Class|Knockbackable|ApplyKnockback knockbackForce 1.0)
  (Game|Damage|ApplyDamage self 25.0 0 0)
  (CallFunction|OnDamageTakenEvent))

(event Collision|EventHit
  (params (MyComp :type Primitive%20Component%20Object%20Reference) (Other :type Actor%20Object%20Reference) (OtherComp :type Primitive%20Component%20Object%20Reference) (bSelfMoved :type Boolean) (HitLocation :type Vector :default "0, 0, 0") (HitNormal :type Vector :default "0, 0, 0") (NormalImpulse :type Vector :default "0, 0, 0") (Hit :type Hit%20Result%20Structure%20%28by%20ref%29))
  (bind _successfulattack (CallFunction|AttackPlayer Other (* (Variables|Default|GetKnockbackDirection) (Variables|Default|GetKnockbackForce))))
  (if _successfulattack
    (Utilities|FlowControl|Delay (Variables|Default|GetReturnTokenDelay))
    (CallFunction|ReturnAttackToken)))

(event EventTick
  (params (DeltaSeconds :type Float%20%28single-precision%29))
  ;[0.15 0.15 0.15 0.5] Initialize enemy health
  (CallFunction|InitializeHealth))

(event EventDropItemsonDeath
  (CallFunction|DropItems))

(event EventPossessed
  (params (NewController :type Controller%20Object%20Reference))
  (CallFunction|GetAIController)
  (CallFunction|GetStateTree)
  (CallFunction|AssignAttackTypes)
  (CallFunction|GetReferences)
  (Variables|Default|SetEnemyEnabled true)
  (CallFunction|DespawnSetup))

(fn ConstructionScript)

(fn GetReferences
  (bind _returnvalue (Actor|GetActorOfClass "/Game/Blueprints/Player/BP_PlayerCharacter.BP_PlayerCharacter_C"))
  (Variables|References|SetPlayerRef _returnvalue)
  (bind _returnvalue_2 (Actor|GetActorOfClass "/Game/Blueprints/Systems/DirectorSystem/BP_Director.BP_Director_C"))
  (Variables|References|SetDirectorRef _returnvalue_2))

(fn GetStateTree
  (bind _aicontroller (Variables|Default|GetAIController))
  (bind _returnvalue (Actor|GetComponentbyClass _aicontroller "/Script/GameplayStateTreeModule.StateTreeAIComponent"))
  ;[0.15 0.15 0.15 0.5] Get State Tree Reference
  (Utilities|IsValid _returnvalue
    (:Is%20Valid
      (Variables|Default|SetAIStateTree _returnvalue))))

(fn GetAIController
  (bind _self self)
  (bind _returnvalue (AI|GetAIController _self))
  ;[0.15 0.15 0.15 0.5] Get AI Controller Reference
  (Utilities|IsValid _returnvalue
    (:Is%20Valid
      (bind _output_get (Variables|Default|SetAIController _returnvalue))
      (Utilities|IsValid (Variables|/Script/AIModule.AIController|GetBrainComponent _output_get)
        (:Is%20Valid
          (Variables|Default|SetAIBrain (Variables|/Script/AIModule.AIController|GetBrainComponent _output_get)))))))

(fn EnablePhysics
  (Physics|SetSimulatePhysics (Variables|Default|GetCapsuleComponent) true))

(fn DropItems
  (bind _returnvalue (Class|ItemDropTable|CalculateDroppedItem (Variables|Default|GetDropTable)))
  (if (Utilities|IsValidClass _returnvalue)
    (Game|SpawnActorfromClass _returnvalue (Transformation|GetActorTransform) "Undefined" "MultiplyWithRoot" 0 0)
    (Transformation|SetActorLocation (+ (Transformation|GetActorLocation) (* (Math|Random|RandomUnitVector) (Variables|Default|GetItem%20Drop%20RandomRadius))) false false)
    (Audio|Components|Audio|Play (Variables|Default|GetItemDropAudio) 0.0)
    (Development|PrintString "Hello")))

(fn AttackPlayer
  (params (Other :type Actor%20Object%20Reference) (KnockbackForce :type Vector))
  ;[0.15 0.15 0.15 0.5] Temporary, replace with hitbox functionality
  (if (Variables|Default|GetisAttacking)
    (CallFunction|UpdateLastCombatTime)
    (Utilities|Casting|CastToBP_PlayerCharacter Other) ; Check if enemy collided w/player
    (Class|AbilitySystemComponent|TryActivateAbility (Variables|Default|GetAbilitySystemComponent) (Variables|Default|GetBaseEnemyAttack) true)
    (return true)))

(fn AssignAttackTypes
  (bind _returnvalue (GameplayAbilities|GiveAbility (Variables|Default|GetAbilitySystemComponent) "/Game/Blueprints/Enemies/Attacks/GA_BaseEnemyAttack.GA_BaseEnemyAttack_C" 0 -1))
  (Variables|Default|SetBaseEnemyAttack _returnvalue))

(fn InitializeHealth
  (bind _abilitysystemcomponent (Variables|Default|GetAbilitySystemComponent))
  (bind _returnvalue (Ability|GameplayEffect|AssignTagSetbyCallerMagnitude (GameplayEffects|MakeOutgoingSpec :self _abilitysystemcomponent :GameplayEffectClass "/Game/Blueprints/Enemies/Effects/GE_InitializeHealth.GE_InitializeHealth_C" :Level 1.0) "(TagName=\"Health.Initialize\")" (Variables|Default|GetScaledHealth)))
  (GameplayEffects|ApplyGameplayEffectSpecToSelf _abilitysystemcomponent _returnvalue))

(fn ToggleEnemyActive
  (params (Active :type Boolean))
  (bind _self self)
  (bind _aibrain (Variables|Default|GetAIBrain))
  (Actor|Tick|SetActorTickEnabled _self Active)
  (Collision|SetActorEnableCollision _self Active)
  (Rendering|SetActorHiddenInGame false)
  (Components|Activation|SetActive (Variables|Character|GetCharacterMovement) Active false)
  (Components|Activation|SetActive (Variables|Default|GetAbilitySystemComponent) Active false)
  (if Active
    (AI|Logic|StartLogic _aibrain)
    (else
      (AI|Logic|StopLogic _aibrain "")))
  (Variables|Default|SetEnemyEnabled Active))

(fn OnDeath
  (bind _capsulecomponent (Variables|Default|GetCapsuleComponent))
  (if (not (Variables|Default|GetbIsDead))
    (Variables|Default|SetbIsDead true)
    (Default|CallOnKilled self (Variables|Default|GetBounty))
    (Audio|Components|Audio|Play (Variables|Default|GetDeathAudio) 0.0)
    (Physics|SetSimulatePhysics _capsulecomponent false)
    (Collision|SetCollisionEnabled _capsulecomponent "NoCollision")
    (Rendering|SetVisibility (Variables|Character|GetMesh) false false)
    (AI|Logic|StopLogic (Variables|Default|GetAIStateTree) "")
    (CallFunction|DropItems)
    (Actor|DestroyActor)))

(fn VFXonHit
  (Variables|HitFeedback|SetFadeIn true)
  (Variables|HitFeedback|SetFadeInProgress true)
  (CallFunction|EventControlMaterialFlash))

(fn ColorFlashonHit
  (bind _hitflashmat (Variables|HitFeedback|GetHitFlashMat))
  ;[0.15 0.15 0.15 0.5] Simplified
  (bind _returnvalue (Rendering|Material|GetScalarParameterValue (Variables|HitFeedback|GetHitFlashMat) "Opacity_param" :!class /Script/Engine.MaterialInstanceDynamic))
  ;;[0.15 0.15 0.15 0.5] Check if event should continue running
  (Utilities|IsValid (Variables|HitFeedback|GetHitFlashMat)
    (:Is%20Valid
      (if (Variables|HitFeedback|GetFadeInProgress)
        (if (Variables|HitFeedback|GetFadeIn) ; Check if fading in or out
          ;;[0.15 0.15 0.15 0.5] Set opacity
          (Rendering|Material|SetScalarParameterValue _hitflashmat "Opacity_param" (+ _returnvalue (LocalVariables|GetFadeInterval)) :!class /Script/Engine.MaterialInstanceDynamic)
          (if (>= (+ _returnvalue (LocalVariables|GetFadeInterval)) 1.0) ; Check if fade is over
            (Variables|HitFeedback|SetFadeIn false))
          (else
            (Rendering|Material|SetScalarParameterValue _hitflashmat "Opacity_param" (- _returnvalue (LocalVariables|GetFadeInterval)) :!class /Script/Engine.MaterialInstanceDynamic)
            (if (<= (- _returnvalue (LocalVariables|GetFadeInterval)) 0.0) ; Check if fade is over
              (Variables|HitFeedback|SetFadeInProgress false))))))))

(fn AssignHitFlashMat
  (params (SkeletalMeshOnActor :type Skeletal%20Mesh%20Component%20Object%20Reference))
  (bind _returnvalue (Rendering|Material|CreateDynamicMaterialInstance "/Game/Art/Characters/SmallEnemy/Textures/Test/M_EnemyHitDynamic.M_EnemyHitDynamic" "Hit_Highlight_Inst" "None" :!class /Script/Engine.KismetMaterialLibrary))
  (bind _output_get (Variables|HitFeedback|SetHitFlashMat _returnvalue))
  (Rendering|Material|SetOverlayMaterial SkeletalMeshOnActor _output_get :!class /Script/Engine.MeshComponent)
  (return SkeletalMeshOnActor))

(fn ReserveAttackToken
  (params (NumTaken :type Integer))
  (if (<= NumTaken (Variables|/Game/Blueprints/Player/BP_PlayerCharacter.BP_PlayerCharacter_C|GetEnemyTokens (Variables|References|GetPlayerRef)))
    (Default|ChangeTokenAmount (Variables|References|GetPlayerRef) (* (Math|Integer|Absolute(Integer) NumTaken) -1))
    (Variables|Default|SetAttackTokensHeld (+ NumTaken (Variables|Default|GetAttackTokensHeld)))
    (return true)
    (else
      (return false))))

(fn ReturnAttackToken
  (Default|ChangeTokenAmount (Variables|References|GetPlayerRef) (Variables|Default|GetAttackTokensHeld))
  (Variables|Default|SetAttackTokensHeld 0))

(fn UpdateEnemyActiveState
  (params (DeltaTime :type Float%20%28double-precision%29))
  (bind _enemyenabled (Variables|Default|GetEnemyEnabled))
  ;[0.15 0.15 0.15 0.5] Check if Distance To Player is outside of active range
  (if (Utilities|IsEnemyOutOfActiveRange)
    ;[0.15 0.15 0.15 0.5] Turn Enemy Off If On
    (if _enemyenabled
      (CallFunction|ToggleEnemyActive false))
    (else
      ;[0.15 0.15 0.15 0.5] Turn Enemy On If Off
      (if (not _enemyenabled)
        (CallFunction|ToggleEnemyActive true)))))

(fn PlayHitAnim
  (bind _mesh (Variables|Character|GetMesh))
  (bind _hitmontage (Variables|Default|GetHitMontage))
  (bind _returnvalue (Components|SkeletalMesh|GetAnimInstance _mesh))
  ;[0.15 0.15 0.15 0.5] Play Random Hit Anim
  (Class|AnimInstance|MontagePlaywithBlendSettings _returnvalue _hitmontage (LocalVariables|GetDefaultBlendSettings) 1.0 "Duration" 0.0 true)
  (Ability|Animation|MontageJumptoSection _returnvalue (Utilities|GetRandomMontageSectionName _hitmontage) _hitmontage))