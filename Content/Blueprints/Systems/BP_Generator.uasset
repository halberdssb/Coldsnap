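; Heat-powered generator that switches on when hit, if the player allows it, and charges until full, then stays activated.
; While running, heat accrues from player heat-attribute increases in range and a timeline that plays only while the nearby player gains heat.
; Activation and completion notify BP_Director, apply GAS cue effects, recolor lights and update the HUD meter or counter.
; A heat-required widget faces the player camera until activation.
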(event Custom|ActivateHeatTimeline
  (bind _fillmeter (Variables|References|GetFillMeter))
  ;[0.15 0.15 0.15 0.5] GenHeatGainTimeline
  (bind _heatalpha (Timeline|TL_HeatOverTime PlayFromStart)
    (:Update
      (Variables|Default|SetHeatCurrent (Math|Float|Lerp 0.0 (Variables|Default|GetHeatMax) _heatalpha))
      (Utilities|IsValid _fillmeter
        (:Is%20Valid
          (Progress|SetPercent _fillmeter _heatalpha))))
    (:Finished
      (CallFunction|DeactivateGenerator))))

(event Custom|PauseHeatGain
  (bind _fillmeter (Variables|References|GetFillMeter))
  ;[0.15 0.15 0.15 0.5] GenHeatGainTimeline
  (bind _heatalpha (Timeline|TL_HeatOverTime Stop)
    (:Update
      (Variables|Default|SetHeatCurrent (Math|Float|Lerp 0.0 (Variables|Default|GetHeatMax) _heatalpha))
      (Utilities|IsValid _fillmeter
        (:Is%20Valid
          (Progress|SetPercent _fillmeter _heatalpha))))
    (:Finished
      (CallFunction|DeactivateGenerator))))

(event Custom|ContinueHeatGain
  (bind _fillmeter (Variables|References|GetFillMeter))
  ;[0.15 0.15 0.15 0.5] GenHeatGainTimeline
  (bind _heatalpha (Timeline|TL_HeatOverTime Play)
    (:Update
      (Variables|Default|SetHeatCurrent (Math|Float|Lerp 0.0 (Variables|Default|GetHeatMax) _heatalpha))
      (Utilities|IsValid _fillmeter
        (:Is%20Valid
          (Progress|SetPercent _fillmeter _heatalpha))))
    (:Finished
      (CallFunction|DeactivateGenerator))))

(event EventBeginPlay
  (CallFunction|GetReferences))

(event EventTick
  (params (DeltaSeconds :type Float%20%28single-precision%29))
  (bind _heatrequiredui (Variables|Default|GetHeatRequiredUI))
  (Transformation|SetWorldRotation _heatrequiredui (Math|Rotator|FindLookatRotation (Transformation|GetWorldLocation _heatrequiredui) (Transformation|GetWorldLocation (Variables|/Game/Blueprints/Player/BP_PlayerCharacter.BP_PlayerCharacter_C|GetCamera (Variables|References|GetPlayer)))) false false)
  (if (Variables|Default|GetIsRunning)
    (CallFunction|IsPlayerinRange)))

(event EventHit
  (params (damage :type Float%20%28single-precision%29) (knockbackForce :type Vector :default "0, 0, 0"))
  (CallFunction|RecieveHeat))

(fn ConstructionScript)

(fn ActivateGenerator
  (params (InPlayer :type BP%20Player%20Character%20Object%20Reference))
  (if (not (Variables|Default|GetIsRunning))
    (Variables|Default|SetIsRunning true)
    (Variables|Default|SetHeatCurrent 0.0)
    (Default|OnGenActivated (Variables|References|GetDirectorRef) self)
    (bind _returnvalue (GameplayAttributes|GetAttributeSet (Ability|GetAbilitySystemComponent InPlayer) "/Script/Coldsnap.HeatAttributeSet"))
    (bind _output_get (Variables|Default|SetPlayerHeatAttributeSet _returnvalue))
    (EventDispatchers|BindEventtoOnHeatChanged _output_get (EventDispatchers|CreateEvent :!event GainHeatfromPlayer))
    (Rendering|SetVisibility (Variables|Default|GetChargeRadiusMesh) true false)))

(fn UpdateGenHUD
  (params (Player :type Player%20Controller%20Object%20Reference))
  (bind _asbp_hud (Utilities|Casting|CastToBP_HUD (HUD|GetHUD Player)))
  (bind _output_get (Variables|References|SetHUD _asbp_hud))
  (Default|UpdateGeneratorCounter (Variables|/Game/Blueprints/UI/BP_HUD.BP_HUD_C|GetGeneratorUI _output_get)))

(fn RecieveHeat
  (bind _charginglightcolor (Variables|Lighting|GetChargingLightColor))
  (if (not (or (Variables|Default|GetIsActivated) (Variables|Default|GetIsRunning))) ; Is generator already activated?
    (bind _asbp_player_character (Utilities|Casting|CastToBP_PlayerCharacter (Pawn|GetControlledPawn (Game|GetPlayerController 0))))
    (bind _activated (Default|TryActivateGenerator _asbp_player_character)) ; Try to activate the generator
    (if _activated ; Can the generator be turned on?
      (CallFunction|ActivateGenerator _asbp_player_character)
      (GameplayEffects|ApplyGameplayEffectToSelf :self (Ability|GetAbilitySystemComponent (Variables|References|GetPlayer)) :Level 1.0) ; GenStart Cue
      (CallFunction|StartMeterFill (Game|GetPlayerController 0))
      (bind _returnvalue (GameplayEffects|ApplyGameplayEffectToSelf :self (Ability|GetAbilitySystemComponent (Variables|References|GetPlayer)) :Level 1.0)) ; GenCharging Looping Cue
      (Variables|Default|SetGenChargingGE _returnvalue)
      (Rendering|SetVisibility (Variables|Default|GetHeatRequiredUI) false false)
      (Audio|Components|Audio|Play (Variables|Default|GetActivationAudio) 0.0)
      (Rendering|Components|Light|SetLightColor (Variables|Default|GetPointLight) _charginglightcolor true)
      (Rendering|Components|Light|SetLightColor (Variables|Default|GetPointLight1) _charginglightcolor true))))

(fn DeactivateGenerator
  (bind _activatedlightcolor (Variables|Lighting|GetActivatedLightColor))
  (Variables|Default|SetIsRunning false)
  (Variables|Default|SetIsActivated true)
  (Default|CallOnGeneratorDeactivated self)
  (EventDispatchers|UnbindEventfromOnHeatChanged (Variables|Default|GetPlayerHeatAttributeSet) (EventDispatchers|CreateEvent :!event GainHeatfromPlayer))
  (GameplayEffects|RemoveActiveGameplayEffect (Ability|GetAbilitySystemComponent (Variables|References|GetPlayer)) (Variables|Default|GetGenChargingGE) -1)
  (GameplayEffects|ApplyGameplayEffectToSelf :self (Ability|GetAbilitySystemComponent (Variables|References|GetPlayer)) :Level 1.0) ; GenFinishCharging Cue
  (CallFunction|UpdateGenHUD (Game|GetPlayerController 0))
  (Variables|Default|SetHeatCurrent 3e+01)
  (Default|OnGenDeactivated (Variables|References|GetDirectorRef))
  (Widget|SetVisibility (Variables|Default|GetFillElement) "Collapsed")
  (Rendering|Components|Light|SetLightColor (Variables|Default|GetPointLight) _activatedlightcolor true)
  (Rendering|Components|Light|SetLightColor (Variables|Default|GetPointLight1) _activatedlightcolor true)
  (Rendering|SetVisibility (Variables|Default|GetChargeRadiusMesh) false false))

(fn GetReferences
  (bind _returnvalue (Actor|GetActorOfClass "/Game/Blueprints/Systems/DirectorSystem/BP_Director.BP_Director_C"))
  (Variables|References|SetDirectorRef _returnvalue)
  (bind _returnvalue_2 (Actor|GetActorOfClass "/Game/Blueprints/Systems/DifficultyScaling/BP_GameStateDiffScaling.BP_GameStateDiffScaling_C"))
  (Variables|References|SetDiffScaleRef _returnvalue_2)
  (bind _asbp_player_character (Utilities|Casting|CastToBP_PlayerCharacter (Pawn|GetControlledPawn (Game|GetPlayerController 0))))
  (Variables|References|SetPlayer _asbp_player_character))

(fn StartMeterFill
  (params (Player :type Player%20Controller%20Object%20Reference))
  (bind _asbp_hud (Utilities|Casting|CastToBP_HUD (HUD|GetHUD Player)))
  (bind (_fillmeter _fillelement) (Default|ActivateGeneratorFillMeter (Variables|/Game/Blueprints/UI/BP_HUD.BP_HUD_C|GetGeneratorUI _asbp_hud)))
  (Variables|References|SetFillMeter _fillmeter)
  (Variables|Default|SetFillElement _fillelement))

(fn IsPlayerinRange
  (if (<= (Math|Vector|Distance(Vector) (Transformation|GetActorLocation) (Transformation|GetActorLocation (Variables|References|GetPlayer))) (Components|Sphere|GetScaledSphereRadius (Variables|Default|GetChargeRadius))) ; Is player within max charge distance?
    (Variables|Default|SetIsPlayerClose true)
    (if (Variables|/Game/Blueprints/Player/BP_PlayerCharacter.BP_PlayerCharacter_C|GetIsGainingHeat (Variables|References|GetPlayer)) ; Is the player gaining heat?
      (CallFunction|ContinueHeatGain)
      (else
        (CallFunction|PauseHeatGain)))
    (else
      (Variables|Default|SetIsPlayerClose false)
      (CallFunction|PauseHeatGain))))

(fn AddHeattoGenerator
  (params (InHeatGain :type Float%20%28double-precision%29))
  (bind _fillmeter (Variables|References|GetFillMeter))
  (bind _output_get (Variables|Default|SetHeatCurrent (+ InHeatGain (Variables|Default|GetHeatCurrent))))
  (Utilities|IsValid _fillmeter
    (:Is%20Valid
      (Progress|SetPercent _fillmeter (/ _output_get (Variables|Default|GetHeatCurrent))))))

(fn GainHeatfromPlayer
  (params (AttributeSet :type Attribute%20Set%20Object%20Reference) (OldValue :type Float%20%28single-precision%29) (NewValue :type Float%20%28single-precision%29))
  (bind _returnvalue (- NewValue OldValue))
  (if (Variables|Default|GetIsRunning) ; Is the generator running?
    (if (Variables|Default|GetIsPlayerClose) ; Is the player close by?
      ;[0.15 0.15 0.15 0.5] Update Meter using 0-1 percentage value
      (bind _output_get (Variables|Default|SetHeatCurrent (+ (Math|Float|Clamp(Float) _returnvalue 0.0 _returnvalue) (Variables|Default|GetHeatCurrent))))
      (Progress|SetPercent (Variables|References|GetFillMeter) (/ _output_get (Variables|Default|GetHeatMax)))
      (if (>= (/ _output_get (Variables|Default|GetHeatMax)) 1.0) ; Is the heat gauge full?
        (CallFunction|DeactivateGenerator)))))