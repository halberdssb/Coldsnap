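; BP_LowGravityVolume is a spherical volume that lowers gravity for any Character inside it.
; On overlap it saves the character's original GravityScale in a map keyed by character and applies LowGravityScale; on exit it restores the saved value and removes the entry.
; The Construction Script sizes the sphere from the Radius variable, and entering or leaving prints a debug message.
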(event OnComponentBeginOverlap(Sphere)
  (params (OverlappedComponent :type Primitive%20Component%20Object%20Reference) (OtherActor :type Actor%20Object%20Reference) (OtherComp :type Primitive%20Component%20Object%20Reference) (OtherBodyIndex :type Integer) (bFromSweep :type Boolean) (SweepResult :type Hit%20Result%20Structure%20%28by%20ref%29))
  (bind _ascharacter (Utilities|Casting|CastToCharacter OtherActor))
  (if (not (Utilities|Map|Contains (Variables|Default|GetOriginalGravityByCharacter) _ascharacter))
    (Utilities|Map|Add (Variables|Default|GetOriginalGravityByCharacter) _ascharacter (Variables|/Script/Engine.CharacterMovementComponent|GetGravityScale (Variables|/Script/Engine.Character|GetCharacterMovement _ascharacter)))
    (Variables|/Script/Engine.CharacterMovementComponent|SetGravityScale (Variables|/Script/Engine.Character|GetCharacterMovement _ascharacter) (Variables|Default|GetLowGravityScale))
    (Development|PrintString "Entering gravity volume" true true "(R=0.610680,G=0.000000,B=1.000000,A=1.000000)")))

(event OnComponentEndOverlap(Sphere)
  (params (OverlappedComponent :type Primitive%20Component%20Object%20Reference) (OtherActor :type Actor%20Object%20Reference) (OtherComp :type Primitive%20Component%20Object%20Reference) (OtherBodyIndex :type Integer))
  (bind _ascharacter (Utilities|Casting|CastToCharacter OtherActor))
  (if (Utilities|Map|Contains (Variables|Default|GetOriginalGravityByCharacter) _ascharacter)
    (Variables|/Script/Engine.CharacterMovementComponent|SetGravityScale (Variables|/Script/Engine.Character|GetCharacterMovement _ascharacter) (.Value (Utilities|Map|Find (Variables|Default|GetOriginalGravityByCharacter) _ascharacter)))
    (Utilities|Map|Remove (Variables|Default|GetOriginalGravityByCharacter) _ascharacter)
    (Development|PrintString "Leaving gravity volume" true true "(R=0.000000,G=0.004400,B=1.000000,A=1.000000)")))

(event EventBeginPlay)

(event Collision|EventActorBeginOverlap
  (params (OtherActor :type Actor%20Object%20Reference)))

(event EventTick
  (params (DeltaSeconds :type Float%20%28single-precision%29)))

(fn ConstructionScript
  (Components|Sphere|SetSphereRadius (Variables|Default|GetSphere) (Variables|Default|GetRadius) true))