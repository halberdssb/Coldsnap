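; Game state that scales difficulty from a running total of enemy kills, using base health and damage read from the player at BeginPlay.
; Recalculation functions combine exponential multipliers and flat bonuses into a global difficulty, pushing damage scaling to the player via a SetByCaller GameplayEffect.
; The player variant dampens damage growth and uses constant flat bonuses.
; Helpers provide milestone progress and linear spawn-rate growth; "50/150" tiers currently step every 2/6 kills.
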(event Custom|OnEnemyKilled
  ;[0.15 0.15 0.15 0.5] Total Kill Counter
  (bind _output_get (Variables|Default|SetTotalKills (+ (Variables|Default|GetTotalKills) 1)))
  (Development|PrintString (Utilities|String|Append "Total Kills: " (Utilities|String|ToString(Integer) _output_get))))

(event EventBeginPlay
  (CallFunction|SetBases))

(fn ConstructionScript)

(fn RecalculateDiff
  (bind _totalkills (Variables|Default|GetTotalKills))
  (Development|PrintString "Recalculating")
  (LocalVariables|SetNum50 (/ _totalkills 2)) ; 50 kills?
  (LocalVariables|SetNum150 (/ _totalkills 6)) ; 150 kills?
  (bind _output_get (Variables|Default|SetCurrentHealthMult (Math|Float|Power (Variables|Default|GetHealthPer50Mult) (Math|Conversions|ToFloat(Integer) (LocalVariables|GetNum50)))))
  ;[0.15 0.15 0.15 0.5] Remove when debug is finished!!
  (Development|PrintString (Utilities|String|Append "CurrentHealthMult: " (Utilities|String|ToString(Float) _output_get)) true true "(R=0.077190,G=1.000000,B=0.000000,A=1.000000)" 5.0)
  (bind _output_get_2 (Variables|Default|SetCurrentDamMult (Math|Float|Power (Variables|Default|GetDamPer50Mult) (Math|Conversions|ToFloat(Integer) (LocalVariables|GetNum50)))))
  (Development|PrintString (Utilities|String|Append "CurrentDamageMult: " (Utilities|String|ToString(Float) _output_get_2)) true true "(R=1.000000,G=0.004793,B=0.000000,A=1.000000)" 5.0)
  (Variables|Default|SetCurrentFlatHealthBonus (* (Math|Conversions|ToFloat(Integer) (LocalVariables|GetNum150)) (Variables|Default|GetFlatHealthPer150)))
  (Variables|Default|SetCurrentFlatDamBonus (* (Math|Conversions|ToFloat(Integer) (LocalVariables|GetNum150)) (Variables|Default|GetFlatDamPer150)))
  (Variables|Default|SetRefHealthMult (* (+ (Variables|Default|GetBaseHealth) (Variables|Default|GetCurrentFlatHealthBonus)) (Variables|Default|GetCurrentHealthMult)))
  (bind _output_get_3 (Variables|Default|SetRefDmgMult (* (+ (Variables|Default|GetBaseDamage) (Variables|Default|GetCurrentFlatDamBonus)) (Variables|Default|GetCurrentDamMult))))
  (Development|PrintString (Utilities|String|Append "RefDmgMult: " (Utilities|String|ToString(Float) _output_get_3)) true true "(R=1.000000,G=0.000000,B=0.835145,A=1.000000)" 5.0)
  (Variables|Default|SetGlobalDiff (+ (/ (Variables|Default|GetRefHealthMult) (Variables|Default|GetBaseHealth)) (/ (Variables|Default|GetRefDmgMult) (Variables|Default|GetBaseDamage))))
  (if (== _output_get_3 0.0)
    (bind _output_get_4 (Variables|Default|SetRefDmgMult 1.0))
    (CallFunction|UpdatePlayerDmgScaling _output_get_4)
    (return (Variables|Default|GetGlobalDiff))
    (else
      (CallFunction|UpdatePlayerDmgScaling _output_get_3)
      (return (Variables|Default|GetGlobalDiff)))))

(fn GetDiffMilestones
  (bind _totalkills (Variables|Default|GetTotalKills))
  (LocalVariables|SetMilestoneIndex (/ _totalkills 6))
  (LocalVariables|SetSubIndex (/ (Math|Integer|%(Integer) _totalkills 6) 2))
  (return (LocalVariables|GetMilestoneIndex) (LocalVariables|GetSubIndex) (Class|KismetSystemLibrary|MakeLiteralInteger 3)))

(fn AdjustSpawnRates
  ;[0.15 0.15 0.15 0.5] Linear growth for spawn rate
  (bind _output_get (Variables|Default|SetSpawnRateMult (+ (* (Math|Conversions|ToFloat(Integer) (Variables|Default|GetTotalKills)) (Variables|Default|GetSpawnRateGainPerKill)) (Math|Float|MakeLiteralFloat 1.0)))) ; y
  (Development|PrintString (Utilities|String|Append "SpawnRateMult: " (Utilities|String|ToString(Float) _output_get)))
  (return _output_get))

(fn SetBases
  (bind _returnvalue (Actor|GetActorOfClass "/Game/Blueprints/Player/BP_PlayerCharacter.BP_PlayerCharacter_C"))
  (Utilities|IsValid _returnvalue
    (:Is%20Valid
      (Variables|Default|SetBaseHealth (Math|Float|Truncate (.ReturnValue (Ability|Attribute|GetFloatAttributefromAbilitySystemComponent (Ability|GetAbilitySystemComponent 0) "(AttributeName=\"MaxHealth\",Attribute=/Script/Coldsnap.HealthAttributeSet:MaxHealth,AttributeOwner=\"/Script/CoreUObject.Class'/Script/Coldsnap.HealthAttributeSet'\")"))))
      (Variables|Default|SetBaseDamage (Math|Float|Truncate (Variables|/Game/Blueprints/Player/BP_PlayerCharacter.BP_PlayerCharacter_C|GetDamage _returnvalue))))))

(fn UpdatePlayerDmgScaling
  (params (NewDamageMult :type Float%20%28double-precision%29))
  (bind _returnvalue (Game|GetPlayerCharacter 0))
  (bind _returnvalue_2 (Ability|GetAbilitySystemComponent _returnvalue))
  (bind _returnvalue_3 (Ability|GameplayEffect|AssignTagSetbyCallerMagnitude (GameplayEffects|MakeOutgoingSpec :self _returnvalue_2 :GameplayEffectClass "/Game/Blueprints/Systems/DifficultyScaling/GE_UpdateDamageMult.GE_UpdateDamageMult_C" :Level 1.0) "(TagName=\"Damage.Mult\")" NewDamageMult))
  (GameplayEffects|ApplyGameplayEffectSpecToSelf _returnvalue_2 _returnvalue_3))

(fn RecalculateDiffPlayer
  (bind _totalkills (Variables|Default|GetTotalKills))
  (Development|PrintString "Recalculating")
  (LocalVariables|SetNum50 (/ _totalkills 2)) ; 50 kills?
  (LocalVariables|SetNum150 (/ _totalkills 6)) ; 150 kills?
  (bind _output_get (Variables|Default|SetCurrentHealthMult (Math|Float|Power (Variables|Default|GetHealthPer50Mult) (Math|Conversions|ToFloat(Integer) (LocalVariables|GetNum50)))))
  ;[0.15 0.15 0.15 0.5] Remove when debug is finished!!
  (Development|PrintString (Utilities|String|Append "CurrentHealthMult: " (Utilities|String|ToString(Float) _output_get)) true true "(R=0.077190,G=1.000000,B=0.000000,A=1.000000)" 5.0)
  (bind _output_get_2 (Variables|Default|SetCurrentDamMult (Math|Float|Power (Variables|Default|GetDamPer50Mult) (* (Math|Conversions|ToFloat(Integer) (LocalVariables|GetNum50)) 0.01))))
  (Development|PrintString (Utilities|String|Append "CurrentDamageMult: " (Utilities|String|ToString(Float) _output_get_2)) true true "(R=1.000000,G=0.004793,B=0.000000,A=1.000000)" 5.0)
  (Variables|Default|SetCurrentFlatHealthBonus (Variables|Default|GetFlatHealthPer150))
  (Variables|Default|SetCurrentFlatDamBonus (Variables|Default|GetFlatDamPer150))
  (Variables|Default|SetRefHealthMult (* (+ (Variables|Default|GetBaseHealth) (Variables|Default|GetCurrentFlatHealthBonus)) (Variables|Default|GetCurrentHealthMult)))
  (bind _output_get_3 (Variables|Default|SetRefDmgMult (* (+ (Variables|Default|GetBaseDamage) (Variables|Default|GetCurrentFlatDamBonus)) (Variables|Default|GetCurrentDamMult))))
  (Development|PrintString (Utilities|String|Append "RefDmgMult: " (Utilities|String|ToString(Float) _output_get_3)) true true "(R=1.000000,G=0.000000,B=0.835145,A=1.000000)" 5.0)
  (Variables|Default|SetGlobalDiff (+ (/ (Variables|Default|GetRefHealthMult) (Variables|Default|GetBaseHealth)) (/ (Variables|Default|GetRefDmgMult) (Variables|Default|GetBaseDamage))))
  (if (== _output_get_3 0.0)
    (bind _output_get_4 (Variables|Default|SetRefDmgMult 1.0))
    (CallFunction|UpdatePlayerDmgScaling _output_get_4)
    (return (Variables|Default|GetGlobalDiff))
    (else
      (CallFunction|UpdatePlayerDmgScaling _output_get_3)
      (return (Variables|Default|GetGlobalDiff)))))