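; Hittable crate that takes knockback when hit and returns to its starting position after a delay.
; BeginPlay stores the mesh's world location, and the Hit event passes the incoming force vector to ApplyKnockback and restarts the timer.
; Tick counts time since the last hit and, once RespawnTime elapses, teleports the actor to the stored location with zero rotation.
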(event EventBeginPlay
  (Variables|Default|SetSpawnPos (Transformation|GetWorldLocation (Variables|Character|GetMesh))))

(event Collision|EventActorBeginOverlap
  (params (OtherActor :type Actor%20Object%20Reference)))

(event EventTick
  (params (DeltaSeconds :type Float%20%28single-precision%29))
  (if (Variables|Default|GetHasBeenHit)
    (bind _output_get (Variables|Default|SetTimeSinceLastHit (+ DeltaSeconds (Variables|Default|GetTimeSinceLastHit))))
    (if (>= _output_get (Variables|Default|GetRespawnTime))
      (Transformation|Teleport (Variables|Default|GetSpawnPos) "0, 0, 0")
      (Variables|Default|SetHasBeenHit false)
      (Variables|Default|SetTimeSinceLastHit 0.0))))

(event EventHit
  (params (damage :type Float%20%28single-precision%29) (knockbackForce :type Vector :default "0, 0, 0"))
  (Class|Knockbackable|ApplyKnockback knockbackForce 1.0)
  (Variables|Default|SetHasBeenHit true)
  (Variables|Default|SetTimeSinceLastHit 0.0))

(fn ConstructionScript)