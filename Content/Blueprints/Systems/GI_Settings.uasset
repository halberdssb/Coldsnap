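; Game instance that holds the player's volume and sensitivity settings and persists them through a COLDSNAPSaveGame.
; On Init it loads the save slot and caches both values, or creates and immediately saves a new save object if none exists.
; Setters update the cache and save object only, with debug prints if it is invalid.
; SaveGame writes to disk separately, and ReturnSettings exposes the cached values.
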(event EventInit
  (CallFunction|LoadorCreateSaveObject))

(fn SetVolume
  (params (NewVolume :type Float%20%28double-precision%29))
  (bind _saveobject (Variables|Default|GetSaveObject))
  (bind _output_get (Variables|Default|SetVolumeInst NewVolume))
  (Utilities|IsValid _saveobject
    (:Is%20Valid
      (Variables|/Script/Coldsnap.COLDSNAPSaveGame|SetVolume _saveobject _output_get)
      (Development|PrintString "Volume saved to save data"))
    (:Is%20Not%20Valid
      (CallFunction|PrintSaveIssueDebug "Volume"))))

(fn SetSensitivity
  (params (NewSensitivity :type Float%20%28double-precision%29))
  (bind _saveobject (Variables|Default|GetSaveObject))
  (bind _output_get (Variables|Default|SetSensitivityInst NewSensitivity))
  (Utilities|IsValid _saveobject
    (:Is%20Valid
      (Variables|/Script/Coldsnap.COLDSNAPSaveGame|SetSensitivity _saveobject _output_get))
    (:Is%20Not%20Valid
      (CallFunction|PrintSaveIssueDebug "Settings"))))

(fn ReturnSettings
  (return (Variables|Default|GetVolumeInst) (Variables|Default|GetSensitivityInst)))

(fn SaveGame
  (SaveGame|SaveGametoSlot (Variables|Default|GetSaveObject) (Variables|Default|GetSaveSlotName) (Variables|Default|GetSaveSlot))
  (Development|PrintString "Game saved!" true true "(R=1.000000,G=0.169219,B=0.895486,A=1.000000)"))

(fn LoadorCreateSaveObject
  (bind _returnvalue (SaveGame|DoesSaveGameExist (Variables|Default|GetSaveSlotName) (Variables|Default|GetSaveSlot)))
  (if _returnvalue
    (bind _returnvalue_2 (SaveGame|LoadGamefromSlot (Variables|Default|GetSaveSlotName) (Variables|Default|GetSaveSlot)))
    (bind _ascoldsnapsave_game (Utilities|Casting|CastToCOLDSNAPSaveGame _returnvalue_2)
      (:then
        (Variables|Default|SetSaveObject _ascoldsnapsave_game)
        (CallFunction|LoadSettings))
      (:CastFailed
        (Development|PrintString "ERROR: Save Object loaded in GI_Settings is not of type COLDSNAPSaveGame " true true "(R=1.000000,G=0.000000,B=0.006521,A=1.000000)" 5.0)))
    (else
      (bind _returnvalue_3 (SaveGame|CreateSaveGameObject "/Script/Coldsnap.COLDSNAPSaveGame"))
      (bind _output_get (Variables|Default|SetSaveObject _returnvalue_3))
      (SaveGame|SaveGametoSlot _output_get (Variables|Default|GetSaveSlotName) (Variables|Default|GetSaveSlot)))))

(fn LoadSettings
  (bind _saveobject (Variables|Default|GetSaveObject))
  (Variables|Default|SetVolumeInst (Variables|/Script/Coldsnap.COLDSNAPSaveGame|GetVolume _saveobject))
  (Variables|Default|SetSensitivityInst (Variables|/Script/Coldsnap.COLDSNAPSaveGame|GetSensitivity _saveobject)))

(fn PrintSaveIssueDebug
  (params (ErrorSaveFieldName :type String))
  (Development|PrintString (Utilities|String|Append (Utilities|String|Append (LocalVariables|GetErrorStringPreName) ErrorSaveFieldName) (LocalVariables|GetErrorStringPostName)) true true "(R=1.000000,G=0.000000,B=0.004068,A=1.000000)" 6.0))