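; BP_CoreLevelEndHandler ends the core level once its minibosses are gone, returning the game to the menu scene.
; On BeginPlay it disables tick, waits a second for the Director to spawn, then caches all BP_MinibossEnemy actors.
; Each tick it checks whether the first two cached minibosses are invalid and, if both are, EndGame opens the menu level.
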(event EventBeginPlay
  (Actor|Tick|SetActorTickEnabled false) ; Wait for Director To Spawn Generators
  (Utilities|FlowControl|Delay 1.0)
  (Actor|Tick|SetActorTickEnabled true) ; Wait for Director To Spawn Generators
  (bind _outactors (Actor|GetAllActorsOfClass "/Game/Blueprints/Enemies/BP_MinibossEnemy.BP_MinibossEnemy_C"))
  (Variables|Default|SetMinibosses _outactors)
  (Variables|Default|Setinitialized true))

(event Collision|EventActorBeginOverlap
  (params (OtherActor :type Actor%20Object%20Reference)))

(event EventTick
  (params (DeltaSeconds :type Float%20%28single-precision%29))
  (if (Variables|Default|Getinitialized)
    (Utilities|IsValid (Utilities|Array|Get(acopy) (Variables|Default|GetMinibosses))
      (:Is%20Not%20Valid
        (Utilities|IsValid (Utilities|Array|Get(acopy) (Variables|Default|GetMinibosses) 1)
          (:Is%20Not%20Valid
            (CallFunction|EndGame)))))))

(fn ConstructionScript)

(fn EndGame
  (Game|OpenLevel(byObjectReference) "/Game/Maps/Build/MenuScene.MenuScene"))