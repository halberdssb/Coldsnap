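; AI director that spends credit budgets to spawn enemies and randomly culls level generators at start.
; Looping timers pick affordable, stage-eligible enemy table entries, placing waves at spawn points or the active drill and ambient enemies on traced navmesh points around anchors.
; Kill bounties refill both budgets and update difficulty scaling.
; Spawn interval derives from difficulty, active generators and drill phase, with the wave timer restarted on generator changes.
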(event Custom|RegisterEnemy
  (params (Enemy :type Actor%20Object%20Reference))
  (bind _boundenemies (Variables|Default|GetBoundEnemies))
  (bind _asbp_base_enemy (Utilities|Casting|CastToBP_BaseEnemy Enemy))
  (if (Utilities|Array|ContainsItem _boundenemies _asbp_base_enemy)
    _
    (else
      (Utilities|Array|Add _boundenemies _asbp_base_enemy)))
  (EventDispatchers|BindEventtoOnKilled _asbp_base_enemy (delegate Custom|Director_OnKilled))
  (Utilities|Array|Add (Variables|Default|GetBoundEnemies) _asbp_base_enemy))

(event Custom|Director_OnKilled
  (params (EnemyRef :type BP%20Base%20Enemy%20Object%20Reference) (Bounty :type Integer))
  (CallFunction|OnKillAddCredits Bounty)
  (CallFunction|DiffCalculation))

(event Custom|DiffCalculation
  (bind _diffscalingref (Variables|References|GetDiffScalingRef))
  (Default|OnEnemyKilled _diffscalingref)
  (Default|RecalculateDiff _diffscalingref)
  (bind _actualspawnrate (CallFunction|GetActualSpawnRate))
  (bind _output_get (Variables|Default|SetActual%20Spawn%20Rate _actualspawnrate))
  (Development|PrintString (Utilities|String|ToString(Float) _output_get)))

(event Custom|TEMP_RegisterPresetEnemies
  (bind _outactors (Actor|GetAllActorsOfClass "/Game/Blueprints/Enemies/BP_BaseEnemy.BP_BaseEnemy_C"))
  (for _array_element _outactors
    (CallFunction|RegisterEnemy _array_element)))

(event Custom|PickThreeRandomSpawners
  (params (RandomIdx :type Integer) (SpawnerArray :type Array%20of%20BP%20Spawn%20Point%20Object%20References))
  (bind _returnvalue (Math|Random|RandomIntegerinRange 0 RandomIdx))
  ;[0.15 0.15 0.15 0.5] Picks three random spawners (called in PickRandomSpawner)
  (Utilities|Array|Add (Variables|SpwnPtArrayVariables|GetSpawnersResult) (Utilities|Array|Get(acopy) SpawnerArray _returnvalue))
  (Utilities|Array|RemoveIndex SpawnerArray _returnvalue))

(event EventBeginPlay
  (CallFunction|TEMPRegisterPresetEnemies)
  (CallFunction|GetReferences)
  (Variables|AmbientEnemies|SetAmbientCredits 2e+01)
  (Variables|Default|SetCredits 2e+01)
  (Utilities|Time|SetTimerbyFunctionName 0 "TrySpawnOnce" (Variables|Default|GetActual%20Spawn%20Rate) true)
  (CallFunction|RandomSpawnGenerators)
  (if (Variables|AmbientEnemies|GetbAmbientEnabled)
    (Utilities|Time|SetTimerbyFunctionName 0 "TryAmbSpawnOnce" (Variables|AmbientEnemies|GetAmbientSpawnInterval) true)))

(fn ConstructionScript)

(fn OnKillAddCredits
  (params (Bounty :type Integer))
  (Variables|Default|SetCredits (Math|Float|Clamp(Float) (+ (Variables|Default|GetCredits) (* (Variables|Default|GetDifficultyMult) (Math|Conversions|ToFloat(Integer) Bounty))) 0.0 (Variables|Default|GetBudgetCap)))
  (Variables|AmbientEnemies|SetAmbientCredits (Math|Float|Clamp(Float) (+ (Variables|AmbientEnemies|GetAmbientCredits) (* (Variables|Default|GetDifficultyMult) (Math|Conversions|ToFloat(Integer) Bounty))) 0.0 (Variables|Default|GetBudgetCap))))

(fn TrySpawnOnce
  (if (> (Variables|Default|GetCredits) 0.0) ; Does the director have credits?
    ;[0.15 0.15 0.15 0.5] The director looks for potential enemy candidates
    (Utilities|Array|Clear (Variables|TrySpawnOnceVariable|GetCandiates))
    (Variables|TrySpawnOnceVariable|SetTotalWeight 0.0)
    (for _index (range 0 (- (Utilities|Array|Length (Variables|Default|GetEnemyTable)) 1)) ; Looking for candidates
      (CallFunction|LookingforCandidates _index))
    ;[0.15 0.15 0.15 0.5] Director chooses a candidate to spawn
    (if (> (Utilities|Array|Length (Variables|TrySpawnOnceVariable|GetCandiates)) 0) ; Does the director have at least one candidate to choose from?
      (Variables|TrySpawnOnceVariable|SetRoll (Math|Random|RandomFloatinRange 0.0 (Variables|TrySpawnOnceVariable|GetTotalWeight)))
      (Variables|TrySpawnOnceVariable|SetAccumulatedWeight (Variables|TrySpawnOnceVariable|GetTotalWeight))
      (bind (_array_element _array_index) (Utilities|Array|ForEachLoopwithBreak (Variables|TrySpawnOnceVariable|GetCandiates) :!label _label) ; Choosing one candidate
        (:LoopBody
          (CallFunction|ChoosingOneCandidate _array_index _array_element)
          (goto _label Break))
        (:Completed
          ;[0.15 0.15 0.15 0.5] Spawning
          (if (>= (Variables|TrySpawnOnceVariable|GetChosenIndex) 0) ; Has the director chosen at least one candidate?
            (if (Variables|DrillSpawnVariables|GetDrillPhaseActive) ; Is the drill activated?
              ;;[0.15 0.15 0.15 0.5] Handles drill spawning
              (Development|PrintString "Drill is active, checking for suitable location" true true "(R=0.709414,G=0.000000,B=1.000000,A=1.000000)")
              (bind (_spawnlocation _foundlocation) (Default|FindSpawnLocation (Variables|References|GetDrillRef)))
              (if _foundlocation ; Is there a suitable spawn location?
                (CallFunction|SpawnDrillEnemy _spawnlocation) ; There is, spawn enemy at drill
                (Development|PrintString "Spawning drill enemy" true true "(R=0.139215,G=1.000000,B=0.000000,A=1.000000)")
                (else
                  (CallFunction|SpawnEnemy) ; There is not, spawn enemy normally
                  (Development|PrintString "Spawning enemy normally" true true "(R=1.000000,G=0.046970,B=0.000000,A=1.000000)")))
              (else
                (CallFunction|SpawnEnemy)
                (Development|PrintString "Drill isn't activated so spawn normally" true true "(R=1.000000,G=0.963110,B=0.000000,A=1.000000)"))))))
      (else
        (Development|PrintString "No candidates this wave")))))

(fn GetReferences
  (bind _returnvalue (Actor|GetActorOfClass "/Game/Blueprints/Enemies/BP_BaseEnemy.BP_BaseEnemy_C"))
  (Variables|References|SetEnemy%20Ref _returnvalue)
  (bind _returnvalue_2 (Actor|GetActorOfClass "/Game/Blueprints/Systems/DifficultyScaling/BP_GameStateDiffScaling.BP_GameStateDiffScaling_C"))
  (Variables|References|SetDiffScalingRef _returnvalue_2)
  (bind _outactors (Actor|GetAllActorsOfClass "/Game/Blueprints/Systems/DirectorSystem/BP_SpawnPoint.BP_SpawnPoint_C"))
  (Variables|SpwnPtArrayVariables|SetSpawners _outactors)
  (bind _returnvalue_3 (Actor|GetActorOfClass "/Game/Blueprints/Systems/DrillSystems/BP_DrillSystem.BP_DrillSystem_C"))
  (Variables|References|SetDrillRef _returnvalue_3))

(fn GetActualSpawnRate
  (bind _spawnratemult (Default|AdjustSpawnRates (Variables|References|GetDiffScalingRef)))
  (bind _genspawnratemult (CallFunction|RecalcGenBonuses))
  (bind _drillspawnratemult (CallFunction|RecalcDrillBonuses (* _spawnratemult _genspawnratemult)))
  (if (> _drillspawnratemult 1.0)
    (return (/ (Variables|Default|GetSpawnInterval) _drillspawnratemult))
    (else
      (return (* (Variables|Default|GetSpawnInterval) _drillspawnratemult)))))

(fn RecalcGenBonuses
  (bind _output_get (Variables|GenSpawnVariables|SetGenSpawnRateMult (+ (* (Variables|GenSpawnVariables|GetActiveGenCount) (Variables|GenSpawnVariables|GetGenSpawnRateBonus)) 1.0)))
  (return _output_get))

(fn OnGenActivated
  (params (GenRef :type BP%20Generator%20Object%20Reference))
  (Math|Integer|IncrementInt (Variables|GenSpawnVariables|GetActiveGenCount)
    (:%20%20
      (Variables|Default|SetCredits (+ (Variables|Default|GetCredits) (Variables|GenSpawnVariables|GetActiveGenCreditBonus)))
      (bind _actualspawnrate (CallFunction|GetActualSpawnRate))
      (Development|PrintString (Utilities|String|Append "Active spawn rate: " (Utilities|String|ToString(Float) _actualspawnrate)) true true "(R=0.000000,G=0.660000,B=1.000000,A=1.000000)" 1e+01)
      (Development|PrintString "Director got credit bonus, gen is activated" true true "(R=0.000000,G=1.000000,B=0.034383,A=1.000000)")
      (Utilities|Time|ClearTimerbyFunctionName 0 "TrySpawnOnce")
      (Utilities|Time|SetTimerbyFunctionName 0 "TrySpawnOnce" _actualspawnrate true))))

(fn OnGenDeactivated
  (params (GenRef :type BP%20Generator%20Object%20Reference))
  (bind _result (Math|Integer|DecrementInt (Variables|GenSpawnVariables|GetActiveGenCount))
    (:%20%20
      (Variables|GenSpawnVariables|SetActiveGenCount (Math|Integer|Clamp(Integer) _result 0 10))
      (Math|Integer|IncrementInt (Variables|GenSpawnVariables|GetDeactiveGenCount)
        (:%20%20
          (bind _actualspawnrate (CallFunction|GetActualSpawnRate))
          (Development|PrintString (Utilities|String|Append "Deactive spawnrate: " (Utilities|String|ToString(Float) _actualspawnrate)) true true "(R=0.000000,G=0.660000,B=1.000000,A=1.000000)" 1e+01)
          (Development|PrintString "Gen is deactivated" true true "(R=0.000000,G=1.000000,B=0.034383,A=1.000000)")
          (Utilities|Time|ClearTimerbyFunctionName 0 "TrySpawnOnce")
          (Utilities|Time|SetTimerbyFunctionName 0 "TrySpawnOnce" _actualspawnrate true))))))

(fn SpawnEnemy
  (bind _output_get (Variables|TrySpawnOnceVariable|SetChosenEntry (Utilities|Array|Get(acopy) (Variables|Default|GetEnemyTable) (Variables|TrySpawnOnceVariable|GetChosenIndex))))
  (Variables|Default|SetCredits (Math|Float|Clamp(Float) (- (Variables|Default|GetCredits) (.cost _output_get)) 0.0 (Variables|Default|GetBudgetCap)))
  (bind _selectedspawners (CallFunction|PickRandomSpawners (Variables|SpwnPtArrayVariables|GetMaxSpawnersPerWave)))
  (bind _array_element (Utilities|Array|ForEachLoopwithBreak _selectedspawners)
    (:LoopBody
      (bind _returnvalue (Game|SpawnActorfromClass (.enemyclass _output_get) (Math|Transform|MakeTransform (Transformation|GetWorldLocation (Variables|/Game/Blueprints/Systems/DirectorSystem/BP_SpawnPoint.BP_SpawnPoint_C|GetDefaultSceneRoot _array_element))) "AdjustIfPossibleButAlwaysSpawn" "MultiplyWithRoot" 0 (.bounty _output_get) 0))
      (bind _output_get_2 (Variables|Default|SetSpawnedEnemy _returnvalue))
      (CallFunction|RegisterEnemy _output_get_2)
      (GameplayEffects|ApplyGameplayEffectToSelf :self (Ability|GetAbilitySystemComponent _output_get_2) :GameplayEffectClass "/Game/GameplayCues/CueGameplayEffects/GE_EnemySpawning.GE_EnemySpawning_C" :Level 1.0)
      ;[0.15 0.15 0.15 0.5] Enemy Spawning Debug
      (Rendering|Debug|DrawDebugSphere (.Location (Math|Transform|BreakTransform (Math|Transform|MakeTransform (Transformation|GetWorldLocation (Variables|/Game/Blueprints/Systems/DirectorSystem/BP_SpawnPoint.BP_SpawnPoint_C|GetDefaultSceneRoot _array_element))))) 1e+02 12 "(R=1.000000,G=0.031257,B=0.000000,A=1.000000)" 1e+01 4.0)
      (Transformation|SetActorLocation (Game|GetPlayerCharacter 0) (+ (.Location (Math|Transform|BreakTransform (Math|Transform|MakeTransform (Transformation|GetWorldLocation (Variables|/Game/Blueprints/Systems/DirectorSystem/BP_SpawnPoint.BP_SpawnPoint_C|GetDefaultSceneRoot _array_element))))) "0.000000,0.000000,200.000000") false false))))

(fn LookingforCandidates
  (params (EnemyTableIndex :type Integer))
  (bind _enemytable (Variables|Default|GetEnemyTable))
  (bind _output (Utilities|Array|Get(acopy) _enemytable EnemyTableIndex))
  (if (<= (.cost _output) (Variables|Default|GetCredits)) ; Affordable?
    (if (>= (Variables|Default|GetStageIndex) (.minstage _output)) ; Correct stage?
      (Utilities|Array|Add (Variables|TrySpawnOnceVariable|GetCandiates) EnemyTableIndex)
      (Variables|TrySpawnOnceVariable|SetTotalWeight (+ (Variables|TrySpawnOnceVariable|GetTotalWeight) (Math|Float|Clamp(Float) (.weight _output) 0.0 1e+02))))))

(fn ChoosingOneCandidate
  (params (ArrayIndex :type Integer) (ArrayElement :type Integer))
  (bind _output_get (Variables|TrySpawnOnceVariable|SetRoll (- (Variables|TrySpawnOnceVariable|GetRoll) (.weight (Utilities|Array|Get(acopy) (Variables|Default|GetEnemyTable) ArrayElement)))))
  (if (<= _output_get 0.0)
    (Variables|TrySpawnOnceVariable|SetChosenIndex ArrayIndex)))

(fn PickRandomSpawners
  (params (MaxToPick :type Integer))
  (bind _output_get (LocalVariables|SetTempArray (Variables|SpwnPtArrayVariables|GetSpawners)))
  (bind _output_get_2 (LocalVariables|SetSpawnersAvailable (Utilities|Array|Length _output_get)))
  (Utilities|Array|Clear (Variables|SpwnPtArrayVariables|GetSpawnersResult))
  (for _index (range 0 (- (Math|Integer|Clamp(Integer) _output_get_2 (Math|Integer|Min(Integer) (Variables|SpwnPtArrayVariables|GetMaxSpawnersPerWave) (LocalVariables|GetSpawnersAvailable)) 0) 1)) ; Pick 3 random spawners
    (CallFunction|PickThreeRandomSpawners (- (Utilities|Array|Length (LocalVariables|GetTempArray)) 1) (LocalVariables|GetTempArray)))
  (return (Variables|SpwnPtArrayVariables|GetSpawnersResult)))

(fn SpawnDrillEnemy
  (params (SpawnTransform :type Transform))
  (bind _output_get (Variables|TrySpawnOnceVariable|SetChosenEntry (Utilities|Array|Get(acopy) (Variables|Default|GetEnemyTable) (Variables|TrySpawnOnceVariable|GetChosenIndex))))
  (Variables|Default|SetCredits (Math|Float|Clamp(Float) (- (Variables|Default|GetCredits) (.cost _output_get)) 0.0 (Variables|Default|GetBudgetCap)))
  (bind _returnvalue (Game|SpawnActorfromClass (.enemyclass _output_get) SpawnTransform "AdjustIfPossibleButAlwaysSpawn" "MultiplyWithRoot" 0 (.bounty _output_get) 0))
  (bind _output_get_2 (Variables|Default|SetSpawnedEnemy _returnvalue))
  (CallFunction|RegisterEnemy _output_get_2))

(fn RecalcDrillBonuses
  (params (CurrentSpawnRate :type Float%20%28double-precision%29))
  (if (Variables|DrillSpawnVariables|GetDrillPhaseActive) ; Is the drill active?
    (return (* CurrentSpawnRate 2.5))
    (else
      (return (* CurrentSpawnRate 1.0)))))

(fn RandomSpawnGenerators
  (bind _outactors (Actor|GetAllActorsOfClass "/Game/Blueprints/Systems/BP_Generator.BP_Generator_C"))
  (LocalVariables|SetGeneratorsInScene _outactors)
  (if (> (Utilities|Array|Length _outactors) 3)
    (bind _output_get (LocalVariables|SetInitialNumGenerators (- (Utilities|Array|Length _outactors) 4)))
    (for _index (range 0 _output_get)
      (bind _output_get_2 (LocalVariables|SetDrillToDestroy (Utilities|Array|Get(acopy) (LocalVariables|GetGeneratorsInScene) (Math|Random|RandomInteger (Utilities|Array|Length (LocalVariables|GetGeneratorsInScene))))))
      (Utilities|Array|RemoveItem (LocalVariables|GetGeneratorsInScene) _output_get_2)
      (Actor|DestroyActor _output_get_2))))

(fn TryAmbSpawnOnce
  (Development|PrintString "Trying to spawn ambient enemies" true true "(R=1.000000,G=0.735559,B=0.000000,A=1.000000)")
  (if (< (Variables|AmbientEnemies|GetAmbientAlive) (Variables|AmbientEnemies|GetMaxAmbientAlive))
    (bind _output_get (Variables|AmbientEnemies|SetAmbientCredits (+ (Variables|AmbientEnemies|GetAmbientCredits) (Variables|AmbientEnemies|GetAmbientCreditsPerTick))))
    (if (> _output_get 0.0) ; Is AmbientCredits greater than 0?
      (Utilities|Array|Clear (Variables|TrySpawnOnceVariable|GetCandiates))
      (Variables|TrySpawnOnceVariable|SetTotalWeight 0.0)
      (for _index (range 0 (- (Utilities|Array|Length (Variables|Default|GetEnemyTable)) 1)) ; Looking for candidates
        (CallFunction|LookingforCandidates _index))
      (if (> (Utilities|Array|Length (Variables|TrySpawnOnceVariable|GetCandiates)) 0) ; Does the director have at least one candidate to choose from?
        (Variables|TrySpawnOnceVariable|SetRoll (Math|Random|RandomFloatinRange 0.0 (Variables|TrySpawnOnceVariable|GetTotalWeight)))
        (Variables|TrySpawnOnceVariable|SetAccumulatedWeight (Variables|TrySpawnOnceVariable|GetTotalWeight))
        (bind (_array_element _array_index) (Utilities|Array|ForEachLoopwithBreak (Variables|TrySpawnOnceVariable|GetCandiates) :!label _label) ; Choosing one candidate
          (:LoopBody
            (CallFunction|ChoosingOneCandidate _array_index _array_element)
            (goto _label Break))
          (:Completed
            (if (>= (Variables|TrySpawnOnceVariable|GetChosenIndex) 0) ; Has the director chosen at least one candidate?
              (CallFunction|SpawnAmbEnemy))))
        (else
          (Development|PrintString "No candidates this wave")))
      (else
        (Development|PrintString "Need more AmbCredits")
        (return)))
    (else
      (return))))

(fn SpawnAmbEnemy
  (bind _output_get (Variables|TrySpawnOnceVariable|SetChosenEntry (Utilities|Array|Get(acopy) (Variables|Default|GetEnemyTable) (Variables|TrySpawnOnceVariable|GetChosenIndex))))
  (Variables|AmbientEnemies|SetAmbientCredits (- (Variables|AmbientEnemies|GetAmbientCredits) (.cost _output_get)))
  (bind _spawntransform (CallFunction|FindAmbientSpawnTransform))
  (bind _returnvalue (Game|SpawnActorfromClass (.enemyclass _output_get) _spawntransform "AdjustIfPossibleButAlwaysSpawn" "MultiplyWithRoot" 0 (.bounty _output_get) 0))
  (bind _output_get_2 (Variables|Default|SetSpawnedEnemy _returnvalue))
  (CallFunction|RegisterEnemy _output_get_2)
  (Development|PrintString "General enemy spawned " true true "(R=0.050979,G=1.000000,B=0.000000,A=1.000000)" 5.0))

(fn FindAmbientSpawnTransform
  (bind _outactors (Actor|GetAllActorsOfClass "/Game/Blueprints/Systems/DirectorSystem/BP_GenSpawnCenter.BP_GenSpawnCenter_C" :!label _label))
  (bind _output_get (Variables|AmbientEnemies|SetAmbientAnchors _outactors))
  (if (.ReturnValue (AI|Navigation|GetRandomReachablePointinRadius (.Location (Math|Transform|BreakTransform (Transformation|GetActorTransform (Utilities|Array|Get(acopy) _output_get (Math|Random|RandomIntegerinRange 0 (Utilities|Array|Length _output_get)))))) (Math|Random|RandomFloatinRange (Variables|AmbientEnemies|GetAmbMinSpawnRadius) (Variables|AmbientEnemies|GetAmbMaxSpawnRadius)) 0 0))
    (bind (_outhit _returnvalue) (Collision|LineTraceByChannel (+ (.RandomLocation (AI|Navigation|GetRandomReachablePointinRadius (.Location (Math|Transform|BreakTransform (Transformation|GetActorTransform (Utilities|Array|Get(acopy) _output_get (Math|Random|RandomIntegerinRange 0 (Utilities|Array|Length _output_get)))))) (Math|Random|RandomFloatinRange (Variables|AmbientEnemies|GetAmbMinSpawnRadius) (Variables|AmbientEnemies|GetAmbMaxSpawnRadius)) 0 0)) "0.000000,0.000000,1000.000000") (- (.RandomLocation (AI|Navigation|GetRandomReachablePointinRadius (.Location (Math|Transform|BreakTransform (Transformation|GetActorTransform (Utilities|Array|Get(acopy) _output_get (Math|Random|RandomIntegerinRange 0 (Utilities|Array|Length _output_get)))))) (Math|Random|RandomFloatinRange (Variables|AmbientEnemies|GetAmbMinSpawnRadius) (Variables|AmbientEnemies|GetAmbMaxSpawnRadius)) 0 0)) "0.000000,0.000000,5000.000000") "TraceTypeQuery1" false (Variables|AmbientEnemies|GetAmbientAnchors) "None"))
    (if _returnvalue
      (bind _output_get_2 (LocalVariables|SetSpawn (Math|Transform|MakeTransform (.ImpactPoint (Collision|BreakHitResult _outhit)) "0, 0, 0" "1.000000,1.000000,1.000000")))
      (return _output_get_2)
      (else
        (goto _label)))
    (else
      (goto _label))))

(fn SpawnStaticDrillEnemies
  (params (SpawnTransform :type Transform))
  (bind _output_get (Variables|TrySpawnOnceVariable|SetChosenEntry (Utilities|Array|Get(acopy) (Variables|Default|GetEnemyDrillTable) (Class|KismetSystemLibrary|MakeLiteralInteger 4))))
  (Variables|Default|SetCredits (Math|Float|Clamp(Float) (- (Variables|Default|GetCredits) (.cost _output_get)) 0.0 (Variables|Default|GetBudgetCap)))
  (bind _returnvalue (Game|SpawnActorfromClass (.enemyclass _output_get) SpawnTransform "AdjustIfPossibleButAlwaysSpawn" "MultiplyWithRoot" 0 (.bounty _output_get) 0))
  (bind _output_get_2 (Variables|Default|SetSpawnedEnemy _returnvalue))
  (CallFunction|RegisterEnemy _output_get_2)
  (GameplayEffects|ApplyGameplayEffectToSelf :self (Ability|GetAbilitySystemComponent _output_get_2) :GameplayEffectClass "/Game/GameplayCues/CueGameplayEffects/GE_EnemySpawning.GE_EnemySpawning_C" :Level 1.0))