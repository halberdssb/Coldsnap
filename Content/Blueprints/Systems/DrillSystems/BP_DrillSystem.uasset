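; Drill objective actor that runs a timed drill phase once the director's generator count reaches the number of generators in the level.
; Tick polls that count, then disables itself, flags the phase on BP_Director and grants it bonus credits.
; After a delay, it destroys cached debris, activates the assigned hole and clears the phase.
; A separate function searches the navmesh for drill-facing spawn transforms beyond a minimum radius.
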(event Custom|PickRandomOffset
  (bind _returnvalue (Math|Random|RandomFloatinRange 0.0 3.6e+02))
  (bind _spawnradiusmin (Variables|Default|GetSpawnRadiusMin))
  (bind _spawnradiusmax (Variables|Default|GetSpawnRadiusMax))
  (bind _returnvalue_2 (Math|Trig|DegreesToRadians _returnvalue))
  (bind _returnvalue_3 (Math|Random|RandomFloatinRange _spawnradiusmin _spawnradiusmax))
  ;[0.15 0.15 0.15 0.5] Pick random spawn location offset
  (Variables|Default|SetSpawnLocationOffset (+ (Transformation|GetActorLocation) (Math|Vector|MakeVector (* (Math|Trig|Cos(Radians) _returnvalue_2) _returnvalue_3) (* (Math|Trig|Sin(Radians) _returnvalue_2) _returnvalue_3) 0.0))))

(event EventBeginPlay
  (CallFunction|GetReferences)
  (Variables|Default|SetDrillActive false)
  (Actor|Tick|SetActorTickEnabled true))

(event EventTick
  (params (DeltaSeconds :type Float%20%28single-precision%29))
  (if (not (Variables|Default|GetDrillActive)) ; Is the drill active?
    (if (>= (Variables|/Game/Blueprints/Systems/DirectorSystem/BP_Director.BP_Director_C|GetDeactiveGenCount (Variables|Default|GetDirectorRef)) (Utilities|Array|Length (Variables|Default|GetGenerators))) ; Are all generators activated?
      (CallFunction|StartDrill)
      (Utilities|FlowControl|Delay (Variables|Default|GetDrillActivationTime))
      (CallFunction|FinishDrill))))

(fn ConstructionScript)

(fn GetReferences
  (bind _asbp_hud (Utilities|Casting|CastToBP_HUD (HUD|GetHUD (Game|GetPlayerController 0))))
  (Variables|Default|SetHUD_Ref _asbp_hud)
  (bind _outactors (Actor|GetAllActorsOfClass "/Game/Blueprints/Systems/BP_Generator.BP_Generator_C"))
  (Variables|Default|SetGenerators _outactors)
  (bind _outactors_2 (Actor|GetAllActorsOfClass "/Game/Blueprints/Systems/DrillSystems/BP_Debris.BP_Debris_C"))
  (Variables|Default|SetDebris _outactors_2)
  (bind _returnvalue (Actor|GetActorOfClass "/Game/Blueprints/Systems/DirectorSystem/BP_Director.BP_Director_C"))
  (Variables|Default|SetDirectorRef _returnvalue))

(fn StartDrill
  (bind _directorref (Variables|Default|GetDirectorRef))
  (Variables|Default|SetDrillActive true)
  (Variables|/Game/Blueprints/Systems/DirectorSystem/BP_Director.BP_Director_C|SetDrillPhaseActive (Variables|Default|GetDirectorRef) true)
  (Actor|Tick|SetActorTickEnabled false)
  (Variables|/Game/Blueprints/Systems/DirectorSystem/BP_Director.BP_Director_C|SetCredits _directorref (+ (Variables|/Game/Blueprints/Systems/DirectorSystem/BP_Director.BP_Director_C|GetCredits _directorref) 2e+02))
  (Development|PrintString "Drill has started"))

(fn FinishDrill
  (bind _holeref (Variables|Default|GetHoleRef))
  (for (_array_element _array_index) (Variables|Default|GetDebris)
    (Utilities|IsValid _array_element
      (:Is%20Valid
        (Actor|DestroyActor (Utilities|Array|Get(acopy) (Variables|Default|GetDebris) _array_index)))))
  (Utilities|IsValid _holeref
    (:Is%20Valid
      (Default|ActivateHole _holeref)
      (Variables|Default|SetDrillActive false)
      (Variables|/Game/Blueprints/Systems/DirectorSystem/BP_Director.BP_Director_C|SetDrillPhaseActive (Variables|Default|GetDirectorRef) false)
      (Development|PrintString "Drill finished"))
    (:Is%20Not%20Valid
      (Development|PrintString "Assign hole ref in details panel"))))

(fn FindSpawnLocation
  (bind _returnvalue (Transformation|GetActorLocation))
  (bind _returnvalue_2 (Transformation|GetActorLocation))
  (bind _returnvalue_3 (Class|NavigationSystemV1|GetNavigationSystem))
  (bind _spawnradiusmax (Variables|Default|GetSpawnRadiusMax))
  (bind (_randomlocation _returnvalue_4) (AI|Navigation|GetRandomReachablePointinRadius _returnvalue_3 _returnvalue_2 _spawnradiusmax 0 0))
  (bind _returnvalue_5 (Math|Vector|Distance(Vector) _randomlocation _returnvalue))
  (Utilities|FlowControl|ForLoopwithBreak 0 (- (Variables|Default|GetMaxSpawnAttempts) 1)
    (:LoopBody
      (Development|PrintString (Utilities|String|Append "Navmesh found: " (Utilities|String|ToString(Boolean) _returnvalue_4)) true true "(R=0.053466,G=1.000000,B=0.000000,A=1.000000)" 5.0)
      (if _returnvalue_4 ; Was a spawn location found?
        (Development|PrintString (Utilities|String|ToString(Float) _returnvalue_5) true true "(R=0.725616,G=0.000000,B=1.000000,A=1.000000)" 5.0)
        (Variables|Default|SetSpawnLocation _randomlocation)
        (Development|PrintString "Spawn point found" true true "(R=0.526088,G=0.000626,B=1.000000,A=1.000000)" 5.0)
        (if (>= _returnvalue_5 (Variables|Default|GetSpawnRadiusMin)) ; Is the spawn location too close to the drill?
          (Development|PrintString "Spawn point was far enough" true true "(R=0.000000,G=1.000000,B=0.629042,A=1.000000)" 5.0)
          (Variables|Default|SetSpawnLocation (+ (Variables|Default|GetSpawnLocation) (Variables|Default|GetSpawnLocationOffset)))
          (Variables|Default|SetSpawnRotation (Math|Rotator|FindLookatRotation (Variables|Default|GetSpawnLocationOffset) (Transformation|GetActorLocation)))
          (Development|PrintString "A spawn location was found, attempting spawn" true true "(R=0.002263,G=1.000000,B=0.331225,A=1.000000)")
          (return (Math|Transform|MakeTransform (Variables|Default|GetSpawnLocation) (Variables|Default|GetSpawnRotation)) true))))
    (:Completed
      (Development|PrintString "Viable location not found" false true "(R=1.000000,G=0.000000,B=0.047463,A=1.000000)")
      (return "" false))))