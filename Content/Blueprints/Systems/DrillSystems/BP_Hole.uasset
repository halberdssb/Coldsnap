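; BP_Hole is a level exit trigger in the drill systems that sends the player on to the next stage.
; It disables its box collision on BeginPlay, then immediately activates itself as a query-only trigger.
; On player overlap it saves GAS data, run data and an incremented BP_Director stage index to the game instance.
; It then opens LevelToLoad, carrying progress across the level change.
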(event OnComponentBeginOverlap(Box)
  (params (OverlappedComponent :type Primitive%20Component%20Object%20Reference) (OtherActor :type Actor%20Object%20Reference) (OtherComp :type Primitive%20Component%20Object%20Reference) (OtherBodyIndex :type Integer) (bFromSweep :type Boolean) (SweepResult :type Hit%20Result%20Structure%20%28by%20ref%29))
  (bind _asbp_player_character (Utilities|Casting|CastToBP_PlayerCharacter OtherActor))
  (if (Variables|Default|GetIsActive)
    (Class|GASDataPersistenceHandler|SaveGASDatatoGameInstance (Variables|/Script/Coldsnap.PlayerCharacter|GetDataPersistenceHandler _asbp_player_character))
    (bind _asbp_game_state_diff_scaling (Utilities|Casting|CastToBP_GameStateDiffScaling (Game|GetGameState)))
    (Default|SaveRunDatatoInstance _asbp_game_state_diff_scaling)
    (Development|PrintString "Go to next level")
    (bind _returnvalue (Actor|GetActorOfClass "/Game/Blueprints/Systems/DirectorSystem/BP_Director.BP_Director_C"))
    (Variables|/Game/Blueprints/Systems/DirectorSystem/BP_Director.BP_Director_C|SetStageIndex _returnvalue (+ (Variables|/Game/Blueprints/Systems/DirectorSystem/BP_Director.BP_Director_C|GetStageIndex _returnvalue) 1))
    (Default|SaveStageIndextoInstance _returnvalue)
    (Game|OpenLevel(byObjectReference) (Variables|Default|GetLevelToLoad))))

(event Custom|ActivateHole
  (Variables|Default|SetIsActive true)
  (Collision|SetCollisionEnabled (Variables|Default|GetBox) "QueryOnly"))

(event EventBeginPlay
  (Variables|Default|SetIsActive false)
  (Collision|SetCollisionEnabled (Variables|Default|GetBox) "NoCollision")
  (CallFunction|ActivateHole))

(fn ConstructionScript)