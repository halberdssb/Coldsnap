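; BP_LavaPool is a temporary hazard that burns enemies standing in it and destroys itself after its lifetime.
; Sphere overlap events maintain a list of BP_BaseEnemy actors inside the pool.
; A looping timer applies GE_LavaPoolBurn to each listed enemy through GAS, passing damage via a SetByCaller tag with effect context from the player's ability system.
; Each application also prints debug text.
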(event OnComponentBeginOverlap(Sphere)
  (params (OverlappedComponent :type Primitive%20Component%20Object%20Reference) (OtherActor :type Actor%20Object%20Reference) (OtherComp :type Primitive%20Component%20Object%20Reference) (OtherBodyIndex :type Integer) (bFromSweep :type Boolean) (SweepResult :type Hit%20Result%20Structure%20%28by%20ref%29))
  (bind _overlappingenemies (Variables|Default|GetOverlappingEnemies))
  ;[0.8333 0.1259 0.1359 0.5] Track enemies standing in lava pool
  (Utilities|IsValid OtherActor
    (:Is%20Valid
      (bind _asbp_base_enemy (Utilities|Casting|CastToBP_BaseEnemy OtherActor))
      (if (not (Utilities|Array|ContainsItem _overlappingenemies _asbp_base_enemy))
        (Utilities|Array|Add _overlappingenemies _asbp_base_enemy)))))

(event OnComponentEndOverlap(Sphere)
  (params (OverlappedComponent :type Primitive%20Component%20Object%20Reference) (OtherActor :type Actor%20Object%20Reference) (OtherComp :type Primitive%20Component%20Object%20Reference) (OtherBodyIndex :type Integer))
  ;[0.8333 0.1259 0.1359 0.5] Track enemies standing in lava pool
  (Utilities|IsValid OtherActor
    (:Is%20Valid
      (Utilities|Array|RemoveItem (Variables|Default|GetOverlappingEnemies) OtherActor))))

(event Custom|ApplyBurnToEnemies
  (bind _playerref (Variables|References|GetPlayerRef))
  (bind _returnvalue (Ability|GetAbilitySystemComponent _playerref))
  (for _array_element (Variables|Default|GetOverlappingEnemies)
    (Utilities|IsValid _array_element
      (:Is%20Valid
        (Utilities|IsValid (Ability|GetAbilitySystemComponent _array_element)
          (:Is%20Valid
            (bind _output_get (Variables|Default|SetBurnEffect (GameplayEffects|MakeOutgoingSpec (Ability|GetAbilitySystemComponent _array_element) "/Game/Blueprints/Systems/LavaPool/GE_LavaPoolBurn.GE_LavaPoolBurn_C" 1.0 (GameplayEffects|MakeEffectContext (Ability|GetAbilitySystemComponent (Variables|References|GetPlayerRef))))))
            (bind _returnvalue_2 (Ability|GameplayEffect|AssignTagSetbyCallerMagnitude _output_get "(TagName=\"Damage.Apply\")" (Variables|Default|GetBurnDamage)))
            (bind _returnvalue_3 (GameplayEffects|ApplyGameplayEffectSpecToTarget _returnvalue _returnvalue_2 (Ability|GetAbilitySystemComponent _array_element)))
            (bind _returnvalue_4 (Class|AbilitySystemBlueprintLibrary|GetActiveGameplayEffectTotalDuration _returnvalue_3))
            (Utilities|FlowControl|DelayUntilNextTick)
            (if (GameplayTags|HasMatchingGameplayTag _returnvalue "(TagName=\"Event.DebugBurn\")")
              (Development|PrintString "DEALING DAMAGE" true true "(R=1.000000,G=0.037018,B=0.003498,A=1.000000)")
              (else
                (Development|PrintString (Utilities|String|ToString(Float) _returnvalue_4)))))))
      (:Is%20Not%20Valid
        (Utilities|Array|RemoveItem (Variables|Default|GetOverlappingEnemies) _array_element)))))

(event EventBeginPlay
  (CallFunction|GetReferences)
  (Utilities|Time|SetTimerbyEvent (delegate Custom|ApplyBurnToEnemies) (Variables|Default|GetBurnApplyRate) true)
  (Utilities|FlowControl|Delay (Variables|Default|GetPoolLifeTime))
  (Actor|DestroyActor))

(fn ConstructionScript)

(fn GetReferences
  (bind _returnvalue (Actor|GetActorOfClass "/Game/Blueprints/Player/BP_PlayerCharacter.BP_PlayerCharacter_C"))
  (Variables|References|SetPlayerRef _returnvalue)
  (bind _returnvalue_2 (Actor|GetActorOfClass "/Game/Blueprints/Systems/DirectorSystem/BP_Director.BP_Director_C"))
  (Variables|References|SetDirectorRef _returnvalue_2)
  (Variables|References|SetPlayerASC_Ref (Ability|GetAbilitySystemComponent (Variables|References|GetPlayerRef))))