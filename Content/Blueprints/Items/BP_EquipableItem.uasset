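; BP_EquipableItem is a world item that the player can approach and equip through its own UI.
; Overlap events, plus a sphere check on BeginPlay for a player already in range, set or clear it as the player's nearby upgrade and toggle the HUD interact prompt.
; OpenItemEquipUI pauses the game and focuses EquipUI with a mouse cursor; FocusOnGame restores gameplay, optionally reshowing the prompt.
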(event EventBeginPlay
  (CallFunction|GetPlayerandHUD)
  (CallFunction|CheckforPlayerinInteractRadius))

(event Collision|EventActorBeginOverlap
  (params (OtherActor :type Actor%20Object%20Reference))
  (CallFunction|SetNearbyEquipableforPlayer OtherActor))

(event EventTick
  (params (DeltaSeconds :type Float%20%28single-precision%29)))

(event Collision|EventActorEndOverlap
  (params (OtherActor :type Actor%20Object%20Reference))
  (CallFunction|RemoveNearbyEquipableforPlayer OtherActor))

(fn ConstructionScript)

(fn GetItemName
  (return (Utilities|GetDisplayName self)))

(fn SetNearbyEquipableforPlayer
  (params (OverlappedObject :type Object%20Object%20Reference))
  ;[0.15 0.15 0.15 0.5] Set Player Nearby Upgrade To This
  (if (== OverlappedObject (Variables|Default|GetPlayer))
    (Default|SetNearbyUpgrade (Variables|Default|GetPlayer) self)
    ;[0.15 0.15 0.15 0.5] Show Interact UI
    (CallFunction|DisplayItemInteractUI true)))

(fn DisplayItemInteractUI
  (params (TurnOn :type Boolean))
  (bind _hud (Variables|Default|GetHUD))
  (bind _iteminteractui (Variables|/Game/Blueprints/UI/BP_HUD.BP_HUD_C|GetItemInteractUI _hud))
  (if TurnOn
    (Widget|SetVisibility _iteminteractui "Visible")
    (bind _itemname (CallFunction|GetItemName))
    (Default|SetInteractText _iteminteractui (Utilities|String|Append "Equip " _itemname))
    (else
      (Widget|SetVisibility _iteminteractui "Hidden"))))

(fn GetPlayerandHUD
  ;[0.15 0.15 0.15 0.5] Get Player and HUD References
  (bind _asbp_player_character (Utilities|Casting|CastToBP_PlayerCharacter (Game|GetPlayerCharacter 0)))
  (Variables|Default|SetPlayer _asbp_player_character)
  (bind _asbp_hud (Utilities|Casting|CastToBP_HUD (HUD|GetHUD (Game|GetPlayerController 0))))
  (Variables|Default|SetHUD _asbp_hud))

(fn FocusonItemEquipUI
  (bind _returnvalue (Game|GetPlayerController 0))
  (CallFunction|DisplayItemInteractUI false)
  (Widget|SetVisibility (Variables|Default|GetEquipUI) "Visible")
  (Utilities|Casting|CastToBP_HUD (HUD|GetHUD _returnvalue))
  (Input|SetInputModeUIOnly _returnvalue (Variables|Default|GetEquipUI) "DoNotLock" true)
  (Variables|/Script/Engine.PlayerController|SetbShowMouseCursor _returnvalue true))

(fn OpenItemEquipUI
  (Game|SetGamePaused true)
  (CallFunction|FocusonItemEquipUI))

(fn RemoveNearbyEquipableforPlayer
  (params (Overlapped%20Actor :type Object%20Object%20Reference))
  (bind _player (Variables|Default|GetPlayer))
  ;[0.15 0.15 0.15 0.5] Remove This As Player Nearby Upgrade
  (if (== Overlapped%20Actor _player)
    (Default|SetNearbyUpgrade _player)
    ;[0.15 0.15 0.15 0.5] Hide Interact UI
    (CallFunction|DisplayItemInteractUI false)))

(fn CheckforPlayerinInteractRadius
  (bind _interactradius (Variables|Default|GetInteractRadius))
  (bind _returnvalue (Collision|SphereOverlapActors (Transformation|GetWorldLocation _interactradius) (Components|Sphere|GetScaledSphereRadius _interactradius) (LocalVariables|GetObjectTypes) "/Game/Blueprints/Player/BP_PlayerCharacter.BP_PlayerCharacter_C"))
  (if _returnvalue
    (CallFunction|SetNearbyEquipableforPlayer (Variables|Default|GetPlayer))))

(fn FocusonGame
  (params (ShowInteractUI :type Boolean))
  (bind _returnvalue (Game|GetPlayerController 0))
  (if ShowInteractUI
    (CallFunction|DisplayItemInteractUI true))
  (Variables|/Script/UMG.Widget|SetVisibility (Variables|Default|GetEquipUI) "Hidden")
  (Input|SetInputModeGameOnly _returnvalue true)
  (Variables|/Script/Engine.PlayerController|SetbShowMouseCursor _returnvalue false)
  (Game|SetGamePaused false))