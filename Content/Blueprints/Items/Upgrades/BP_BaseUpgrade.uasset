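; Base upgrade item actor that offers gameplay effects for arms, legs, torso and fuel slots, equipped through the HUD's upgrade UI.
; On BeginPlay it constructs effect objects from classes in UpgradeComp, with fuel holding an array, and exposes them through getters.
; It caches the HUD's equip UI a tick later.
; Opening the equip UI runs the parent logic, then sets this item as the current upgrade.
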(event EventBeginPlay
  (|CallParentFunction)
  ;[0.6251 0.1069 0.7604 0.5] Instantiate Gameplay Effect References
  (CallFunction|GetArmsEffectObjectReference)
  (CallFunction|GetLegsEffectObjectReference)
  (CallFunction|GetTorsoEffectObjectReference)
  (CallFunction|GetFuelEffectObjectReference)
  ;[0.4948 0.361 0.03608 0.287] Get Equip UI Reference
  (Utilities|FlowControl|DelayUntilNextTick)
  (Variables|Default|SetEquipUI (Variables|/Game/Blueprints/UI/BP_HUD.BP_HUD_C|GetUpgradeEquipUI (Variables|Default|GetHUD))))

(event Collision|EventActorBeginOverlap
  (params (OtherActor :type Actor%20Object%20Reference))
  (|CallParentFunction OtherActor))

(event EventTick
  (params (DeltaSeconds :type Float%20%28single-precision%29)))

(event Collision|EventActorEndOverlap
  (params (OtherActor :type Actor%20Object%20Reference))
  (|CallParentFunction OtherActor))

(fn ConstructionScript)

(fn GetArmsEffectObjectReference
  (bind _returnvalue (Game|ConstructObjectfromClass (Variables|/Script/Coldsnap.Upgrade|GetarmsGameplayEffect (Variables|Default|GetUpgrade_Comp))))
  (Variables|Default|SetArmsGameplayEffect _returnvalue))

(fn GetLegsEffectObjectReference
  (bind _returnvalue (Game|ConstructObjectfromClass (Variables|/Script/Coldsnap.Upgrade|GetlegsGameplayEffect (Variables|Default|GetUpgrade_Comp))))
  (Variables|Default|SetLegsGameplayEffect _returnvalue))

(fn GetTorsoEffectObjectReference
  (bind _returnvalue (Game|ConstructObjectfromClass (Variables|/Script/Coldsnap.Upgrade|GettorsoGameplayEffect (Variables|Default|GetUpgrade_Comp))))
  (Variables|Default|SetTorsoGameplayEffect _returnvalue))

(fn GetFuelEffectObjectReference
  (bind _fuelupgradeeffectobjects (LocalVariables|GetFuelUpgradeEffectObjects))
  (for _array_element (Variables|/Script/Coldsnap.Upgrade|GetfuelGameplayEffects (Variables|Default|GetUpgrade_Comp))
    (bind _returnvalue (Game|ConstructObjectfromClass _array_element))
    (Utilities|Array|Add _fuelupgradeeffectobjects _returnvalue))
  (Variables|Default|SetFuelGameplayEffect _fuelupgradeeffectobjects))

(fn GetItemName
  (return (Variables|/Script/Coldsnap.Upgrade|GetUpgradeName (Variables|Default|GetUpgrade_Comp))))

(fn OpenItemEquipUI
  (|CallParentFunction)
  ;[0.4948 0.361 0.03608 0.287] Set current upgrade in UI to this one
  (Default|SetCurrentUpgrade (Variables|/Game/Blueprints/UI/BP_HUD.BP_HUD_C|GetUpgradeEquipUI (Variables|Default|GetHUD)) self))

(fn GetArmsGameplayEffect
  (return (Variables|Default|GetArmsGameplayEffect)))

(fn GetLegsGameplayEffect
  (return (Variables|Default|GetLegsGameplayEffect)))

(fn GetTorsoGameplayEffect
  (return (Variables|Default|GetTorsoGameplayEffect)))

(fn GetFuelGameplayEffect
  (return (Variables|Default|GetFuelGameplayEffect)))