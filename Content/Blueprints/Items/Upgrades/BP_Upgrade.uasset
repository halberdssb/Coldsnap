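; BP_Upgrade is an upgrade item that carries separate gameplay effects for arms, legs and fuel.
; On BeginPlay it constructs effect objects from the classes on its UpgradeComp and caches the HUD's upgrade equip UI.
; Overlap handling defers to the parent, while OpenItemEquipUI extends the parent to set itself as that UI's current upgrade.
; The item name also comes from UpgradeComp.
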(event EventBeginPlay
  (|CallParentFunction)
  ;[0.15 0.15 0.15 0.5] Instantiate Gameplay Effect References
  (CallFunction|GetArmsEffectObjectReference)
  (CallFunction|GetLegsEffectObjectReference)
  (CallFunction|GetFuelEffectObjectReference)
  (Variables|Default|SetEquipUI (Variables|/Game/Blueprints/UI/BP_HUD.BP_HUD_C|GetUpgradeEquipUI (Variables|Default|GetHUD))))

(event Collision|EventActorBeginOverlap
  (params (OtherActor :type Actor%20Object%20Reference))
  (|CallParentFunction OtherActor))

(event EventTick
  (params (DeltaSeconds :type Float%20%28single-precision%29)))

(event Collision|EventActorEndOverlap
  (params (OtherActor :type Actor%20Object%20Reference))
  (|CallParentFunction OtherActor))

(fn ConstructionScript)

(fn GetArmsEffectObjectReference
  (bind _returnvalue (Game|ConstructObjectfromClass (Variables|/Script/Coldsnap.Upgrade|GetarmsGameplayEffect (Variables|Default|GetUpgrade_Comp))))
  (Variables|Default|SetArmsGameplayEffect _returnvalue))

(fn GetLegsEffectObjectReference
  (bind _returnvalue (Game|ConstructObjectfromClass (Variables|/Script/Coldsnap.Upgrade|GetlegsGameplayEffect (Variables|Default|GetUpgrade_Comp))))
  (Variables|Default|SetLegsGameplayEffect _returnvalue))

(fn GetFuelEffectObjectReference
  (bind _returnvalue (Game|ConstructObjectfromClass (Variables|/Script/Coldsnap.Upgrade|GetfuelGameplayEffect (Variables|Default|GetUpgrade_Comp))))
  (Variables|Default|SetFuelGameplayEffect _returnvalue))

(fn GetItemName
  (return (Variables|/Script/Coldsnap.Upgrade|GetUpgradeName (Variables|Default|GetUpgrade_Comp))))

(fn OpenItemEquipUI
  (|CallParentFunction)
  (Default|SetCurrentUpgrade (Variables|/Game/Blueprints/UI/BP_HUD.BP_HUD_C|GetUpgradeEquipUI (Variables|Default|GetHUD)) self))