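; Base Blueprint for item pickups that grant an equipable ability.
; The construction script instantiates an Ability object from AbilityClass, which also supplies the item's display name.
; OpenItemEquipUI is overridden for the single-slot vertical slice: it registers the pickup with the HUD's equip UI and equips straight to slot 1 without showing the UI.
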(event EventBeginPlay
  (|CallParentFunction)
  (Variables|Default|SetEquipUI (Variables|/Game/Blueprints/UI/BP_HUD.BP_HUD_C|GetEquipableAbilityEquipUI (Variables|Default|GetHUD))))

(event Collision|EventActorBeginOverlap
  (params (OtherActor :type Actor%20Object%20Reference))
  (|CallParentFunction OtherActor) ; This node is disabled and will not be called.\nDrag off pins to build functionality.
)

(event EventTick
  (params (DeltaSeconds :type Float%20%28single-precision%29))
  (|CallParentFunction DeltaSeconds) ; This node is disabled and will not be called.\nDrag off pins to build functionality.
)

(fn ConstructionScript
  (|CallParentFunction)
  (bind _returnvalue (Game|ConstructObjectfromClass (Variables|Default|GetAbilityClass)))
  (Variables|Default|SetAbility _returnvalue))

(fn OpenItemEquipUI
  (bind _hud (Variables|Default|GetHUD))
  (bind _equipableabilityequipui (Variables|/Game/Blueprints/UI/BP_HUD.BP_HUD_C|GetEquipableAbilityEquipUI _hud))
  ;[0.15 0.15 0.15 0.5] Override for Vertical Slice - Only One Ability Slot, so directly equip to slot without showing UI
  (Default|SetCurrentEquipableAbility _equipableabilityequipui self)
  (Default|EquipAbilitytoSlot _equipableabilityequipui 1))

(fn GetItemName
  (return (Variables|/Script/Coldsnap.EquipableAbility|GetAbilityName (Variables|Default|GetAbility))))