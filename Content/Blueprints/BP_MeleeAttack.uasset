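; BP_MeleeAttack is a gameplay ability that performs a melee attack, launching nearby knockbackable targets upward.
; On activation it calls CreateMeleeHitbox at the owner's location with debug drawing on, then loops over the returned elements.
; Each Knockbackable gets a strong vertical knockback, separate from the hitbox's own knockback inputs, and has its name printed.
; A Hittable branch is disconnected, and the graph never calls EndAbility.
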(event Ability|EventActivateAbility
  (bind _returnvalue (Class|MeleeAttackGameplayAbility|CreateMeleeHitbox (Transformation|GetWorldLocation (Variables|/Script/Engine.Actor|GetRootComponent (Components|GetOwner (Ability|GetAbilitySystemComponentfromActorInfo)))) 9e+02 "0.000000,1.000000,0.000000" 5e+01 60 true))
  (for _array_element _returnvalue
    (bind _asknockbackable (Utilities|Casting|CastToKnockbackable _array_element))
    (Class|Knockbackable|ApplyKnockback _asknockbackable "0.000000,0.000000,1.000000" 2e+05)
    (Development|PrintString (Utilities|GetDisplayName _array_element))))

(event Ability|EventOnEndAbility
  (params (bWasCancelled :type Boolean)))