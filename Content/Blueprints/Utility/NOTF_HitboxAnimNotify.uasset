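; Anim notify state that creates attack hitboxes during an animation from its HitboxFrameData entries, carrying damage, knockback, stun and launch settings.
; Each tick converts every entry's offset, rotation and capsule size using the mesh's transform, assuming uniform scale.
; It passes the result to the owner's AttackHitboxManager component, optionally drawing debug capsules for montage authoring.
; Begin records the attack duration and End resets elapsed notify time.
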(fn ReceivedNotifyTick
  (params (MeshComp :type Skeletal%20Mesh%20Component%20Object%20Reference) (Animation :type Anim%20Sequence%20Base%20Object%20Reference) (FrameDeltaTime :type Float%20%28single-precision%29) (EventReference :type Anim%20Notify%20Event%20Reference%20Structure%20%28by%20ref%29))
  (bind _returnvalue (Components|GetOwner MeshComp))
  (bind _returnvalue_2 (Actor|GetComponentbyClass _returnvalue "/Script/Coldsnap.AttackHitboxManager"))
  ;[0.6251 0.1069 0.7604 0.5] Create each hitbox active this frame
  (for _array_element (Variables|Default|GetHitbox%20Frame%20Data)
    ;[0.276 0.01853 0.01294 0.6522] Set Hitbox Data of hitbox spawned based on data from notify state fields
    (Utilities|FlowControl|Sequence
      (:then_0
        ;;[0.15 0.15 0.15 0.5] Get Transform Values of Hitbox
        (bind _localoffset (CallFunction|GetLocalOffset MeshComp (.PositionOffset (Utilities|Struct|BreakHitboxData _array_element)))))
      (:then_1
        (bind _local_rotation (CallFunction|GetLocalRotation MeshComp (.Rotation (Utilities|Struct|BreakHitboxData _array_element)))))
      (:then_2
        (bind (_height _radius) (CallFunction|GetLocalScale MeshComp (.Height (Utilities|Struct|BreakHitboxData _array_element)) (.Radius (Utilities|Struct|BreakHitboxData _array_element)))))
      (:then_3
        ;[1 0.4799 0.1042 0.2957] Create Hitbox
        (if (Variables|Default|GetDrawDebugHitboxes)
          (CallFunction|DrawDebugHitbox (Utilities|Struct|MakeHitboxData _localoffset _height _radius _local_rotation (.KnockbackDirection (Utilities|Struct|BreakHitboxData _array_element)) (.KnockbackForce (Utilities|Struct|BreakHitboxData _array_element)) (.Damage (Utilities|Struct|BreakHitboxData _array_element)) (.ShouldStun (Utilities|Struct|BreakHitboxData _array_element)) (.StunTime (Utilities|Struct|BreakHitboxData _array_element)) (.PlayerLaunchForce (Utilities|Struct|BreakHitboxData _array_element))) MeshComp))
        (Utilities|IsValid _returnvalue_2
          (:Is%20Valid
            (Class|AttackHitboxManager|CreateAttackHitbox _returnvalue_2 (Utilities|Struct|MakeHitboxData _localoffset _height _radius _local_rotation (.KnockbackDirection (Utilities|Struct|BreakHitboxData _array_element)) (.KnockbackForce (Utilities|Struct|BreakHitboxData _array_element)) (.Damage (Utilities|Struct|BreakHitboxData _array_element)) (.ShouldStun (Utilities|Struct|BreakHitboxData _array_element)) (.StunTime (Utilities|Struct|BreakHitboxData _array_element)) (.PlayerLaunchForce (Utilities|Struct|BreakHitboxData _array_element)))))))))
  (return true))

(fn GetLocalOffset
  (params (Owning%20Actor :type Scene%20Component%20Object%20Reference) (OffsetFromOwner :type Vector))
  ;[0.6251 0.1069 0.7604 0.5] Ad offset of hitbox to world position of player to stay relative to player location
  (return (+ (+ (Transformation|GetWorldLocation Owning%20Actor) (Math|Vector|RotateVector OffsetFromOwner (Transformation|GetWorldRotation Owning%20Actor))) (Variables|/Script/Engine.SceneComponent|GetRelativeLocation Owning%20Actor))))

(fn GetLocalRotation
  (params (Player%20Actor :type Scene%20Component%20Object%20Reference) (HitboxRotation :type Rotator))
  ;[0.6251 0.1069 0.7604 0.5] Rotate hitbox rotation by current player rotation
  (return (Math|Transform|TransformRotation (Transformation|GetWorldTransform Player%20Actor) HitboxRotation)))

(fn GetLocalScale
  (params (Player%20Actor :type Scene%20Component%20Object%20Reference) (HitboxHeight :type Float%20%28double-precision%29) (HitboxRadius :type Float%20%28double-precision%29))
  (bind _returnvalue (Transformation|GetWorldScale Player%20Actor))
  (bind _x (Math|Vector|BreakVector _returnvalue))
  ;[0.6251 0.1069 0.7604 0.5] Scale hitbox relative to scale of player - ensure matching size in game as seen in montage viewport
  (return (* _x HitboxHeight) (* _x HitboxRadius)))

(fn DrawDebugHitbox
  (params (HitboxData :type Hitbox%20Data%20Structure%20%28by%20ref%29) (OwningActor :type Scene%20Component%20Object%20Reference))
  (bind (_positionoffset _height _radius _rotation) (Utilities|Struct|BreakHitboxData HitboxData))
  ;[0.6251 0.1069 0.7604 0.5] Used for visualizing hitboxes - intended for montage viewport use only when creating hitboxes, or in debug view
  (Rendering|Debug|DrawDebugCapsule OwningActor _positionoffset (/ _height 2.0) _radius _rotation "(R=1.000000,G=0.000000,B=0.009150,A=1.000000)" 0.0 3.0))

(fn ReceivedNotifyBegin
  (params (MeshComp :type Skeletal%20Mesh%20Component%20Object%20Reference) (Animation :type Anim%20Sequence%20Base%20Object%20Reference) (TotalDuration :type Float%20%28single-precision%29) (EventReference :type Anim%20Notify%20Event%20Reference%20Structure%20%28by%20ref%29))
  (Class|HitboxAnimNotify|SetAttackDuration TotalDuration)
  (return false))

(fn ReceivedNotifyEnd
  (params (MeshComp :type Skeletal%20Mesh%20Component%20Object%20Reference) (Animation :type Anim%20Sequence%20Base%20Object%20Reference) (EventReference :type Anim%20Notify%20Event%20Reference%20Structure%20%28by%20ref%29))
  (Class|HitboxAnimNotify|ResetElapsedNotifyTime)
  (return false))