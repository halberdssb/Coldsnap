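; HitboxAnimNotify is an animation notify state that visualizes a hitbox during an animation; it performs no overlap or damage checks.
; Each tick it draws a red debug capsule at the owning actor's CapsuleComponent location plus a position offset, sized and rotated by its variables, with Height doubled as the half-height.
; It also prints a "Hello" debug string every tick, and its notify time-ratio lookup is unused.
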(fn ReceivedNotifyTick
  (params (MeshComp :type Skeletal%20Mesh%20Component%20Object%20Reference) (Animation :type Anim%20Sequence%20Base%20Object%20Reference) (FrameDeltaTime :type Float%20%28single-precision%29) (EventReference :type Anim%20Notify%20Event%20Reference%20Structure%20%28by%20ref%29))
  (bind _returnvalue (Components|GetOwner MeshComp))
  (Rendering|Debug|DrawDebugCapsule _returnvalue (+ (Transformation|GetWorldLocation (Actor|GetComponentbyClass _returnvalue "/Script/Engine.CapsuleComponent")) (Variables|Default|GetPosition%20Offset)) (* (Variables|Default|GetHeight) 2.0) (Variables|Default|GetRadius) (Variables|Default|GetRotation) "(R=1.000000,G=0.000000,B=0.009150,A=1.000000)" 0.0 3.0)
  (Development|PrintString 0)
  (return true))