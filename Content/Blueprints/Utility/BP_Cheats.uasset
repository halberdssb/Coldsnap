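; BP_Cheats is a debug utility with cheat functions for the level's generators.
; ActivateAllGenerators and ActivateNextGenerator both call a shared helper, ActivateGeneratorFlexible, with a flag for all or one.
; The helper finds BP_Director, loops over its GensInScene list and, on each inactive generator, calls ActivateGenerator immediately followed by DeactivateGenerator.
; In single mode it stops after the first inactive generator.
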(fn ActivateAllGenerators
  (CallFunction|ActivateGeneratorFlexible true))

(fn ActivateNextGenerator
  (CallFunction|ActivateGeneratorFlexible false))

(fn ActivateGeneratorFlexible
  (params (ActivateAll :type Boolean))
  (bind _returnvalue (Actor|GetActorOfClass "/Game/Blueprints/Systems/DirectorSystem/BP_Director.BP_Director_C"))
  (bind _array_element (Utilities|Array|ForEachLoopwithBreak (Variables|/Game/Blueprints/Systems/DirectorSystem/BP_Director.BP_Director_C|GetGensInScene _returnvalue) :!label _label)
    (:LoopBody
      (if (not (Variables|/Game/Blueprints/Systems/BP_Generator.BP_Generator_C|GetIsActivated _array_element))
        (Default|ActivateGenerator _array_element)
        (Default|DeactivateGenerator _array_element)
        (if (not ActivateAll)
          (goto _label Break))))))