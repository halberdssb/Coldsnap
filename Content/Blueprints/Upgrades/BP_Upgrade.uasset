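; Upgrade pickup actor that lets the player open an equip menu for arms, legs and fuel gameplay effects.
; On BeginPlay it caches player and HUD references and constructs effect objects from the classes in UpgradeComp.
; Overlap registers it as the player's nearby upgrade and toggles a named interact prompt.
; Opening the equip UI passes itself to the HUD widget, with helpers switching opacity, input mode and cursor between menu and game.
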(event EventBeginPlay
  ;[0.15 0.15 0.15 0.5] Get Player and HUD References
  (bind _asbp_player_character (Utilities|Casting|CastTo (Game|GetPlayerCharacter 0)))
  (Variables|Default|SetPlayer 0 _asbp_player_character)
  (bind _asbp_hud (Utilities|Casting|CastToBP_HUD (HUD|GetHUD (Game|GetPlayerController 0))))
  (Variables|Default|SetHUD _asbp_hud)
  ;[0.15 0.15 0.15 0.5] Instantiate Gameplay Effect References
  (CallFunction|GetArmsEffectObjectReference)
  (CallFunction|GetLegsEffectObjectReference)
  (CallFunction|GetFuelEffectObjectReference))

(event Collision|EventActorBeginOverlap
  (params (OtherActor :type Actor%20Object%20Reference))
  ;[0.15 0.15 0.15 0.5] Set Player Nearby Upgrade To This
  (if (== OtherActor (.Player (Variables|Default|GetPlayer)))
    (CallFunction|SetNearbyUpgrade (.Player (Variables|Default|GetPlayer)) self)
    ;[0.15 0.15 0.15 0.5] Show Interact UI
    (CallFunction|DisplayUpgradeInteractUI true)))

(event EventTick
  (params (DeltaSeconds :type Float%20%28single-precision%29)))

(event Collision|EventActorEndOverlap
  (params (OtherActor :type Actor%20Object%20Reference))
  ;[0.15 0.15 0.15 0.5] Remove This As Player Nearby Upgrade
  (if (== OtherActor (.Player (Variables|Default|GetPlayer)))
    (CallFunction|SetNearbyUpgrade (.Player (Variables|Default|GetPlayer)))
    ;[0.15 0.15 0.15 0.5] Hide Interact UI
    (CallFunction|DisplayUpgradeInteractUI false)))

(fn ConstructionScript)

(fn GetArmsEffectObjectReference
  (bind _returnvalue (Game|ConstructObjectfromClass (Variables|Default|GetarmsGameplayEffect (Variables|Default|GetUpgrade_Comp))))
  (Variables|Default|SetArmsGameplayEffect 0 _returnvalue))

(fn GetLegsEffectObjectReference
  (bind _returnvalue (Game|ConstructObjectfromClass (Variables|Default|GetlegsGameplayEffect (Variables|Default|GetUpgrade_Comp))))
  (Variables|Default|SetLegsGameplayEffect 0 _returnvalue))

(fn GetFuelEffectObjectReference
  (bind _returnvalue (Game|ConstructObjectfromClass (Variables|Default|GetfuelGameplayEffect (Variables|Default|GetUpgrade_Comp))))
  (Variables|Default|SetFuelGameplayEffect 0 _returnvalue))

(fn FocusonEquipUI
  (bind _returnvalue (Game|GetPlayerController 0))
  (CallFunction|DisplayUpgradeInteractUI false)
  (Variables|/Script/UMG.Widget|SetRenderOpacity (Variables|Default|GetUpgradeUI) 1.0)
  (Utilities|Casting|CastToBP_HUD (HUD|GetHUD _returnvalue))
  (Input|SetInputModeUIOnly _returnvalue (Variables|/Game/Blueprints/UI/WB_UpgradeEquipUI.WB_UpgradeEquipUI_C|GetLegsButton (Variables|/Game/Blueprints/UI/BP_HUD.BP_HUD_C|GetUpgradeEquipUI (Variables|Default|GetHUD))) "DoNotLock" true)
  (Variables|/Script/Engine.PlayerController|SetbShowMouseCursor _returnvalue true))

(fn FocusonGame
  (params (ShowInteractUI :type Boolean))
  (bind _returnvalue (Game|GetPlayerController 0))
  (if ShowInteractUI
    (CallFunction|DisplayUpgradeInteractUI true))
  (Variables|/Script/UMG.Widget|SetRenderOpacity (Variables|Default|GetUpgradeUI) 0.0)
  (Input|SetInputModeGameOnly _returnvalue true)
  (Variables|/Script/Engine.PlayerController|SetbShowMouseCursor _returnvalue false))

(fn OpenUpgradeEquipUI
  (Default|SetCurrentUpgrade (Variables|/Game/Blueprints/UI/BP_HUD.BP_HUD_C|GetUpgradeEquipUI (Variables|Default|GetHUD)) self)
  (Variables|Default|SetUpgradeUI (Variables|/Game/Blueprints/UI/BP_HUD.BP_HUD_C|GetUpgradeEquipUI (Variables|Default|GetHUD)))
  (CallFunction|FocusonEquipUI))

(fn DisplayUpgradeInteractUI
  (params (TurnOn :type Boolean))
  (bind _hud (Variables|Default|GetHUD))
  (bind _upgradeinteractui (Variables|/Game/Blueprints/UI/BP_HUD.BP_HUD_C|GetUpgradeInteractUI _hud))
  (if TurnOn
    (Variables|/Script/UMG.Widget|SetRenderOpacity _upgradeinteractui 1.0)
    (Default|SetInteractText _upgradeinteractui (Utilities|String|Append "Equip " (Variables|Default|GetUpgradeName (Variables|Default|GetUpgrade_Comp))))
    (else
      (Variables|/Script/UMG.Widget|SetRenderOpacity _upgradeinteractui 0.0))))