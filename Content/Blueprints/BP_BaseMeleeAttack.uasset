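; Base Gameplay Ability for melee attacks that spawns a hitbox in front of the owning actor.
; On activation it places a debug-drawn sphere hitbox along the owner's forward vector, using only the length of HitboxOffset.
; Each returned actor receives Hit through a Hittable cast, with a printed warning on failure.
; Knockback settings feed the hitbox; the separate Knockbackable helper is uncalled here, and the graph never ends the ability.
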(event Ability|EventActivateAbility
  ;[0.15 0.15 0.15 0.5] Create Hitbox and Get Overlapped Hittables
  (bind _localspaceoffset (CallFunction|GetHitboxOffsetinPlayerSpace (Variables|/Script/Engine.Actor|GetRootComponent (Components|GetOwner (Ability|GetAbilitySystemComponentfromActorInfo)))))
  (bind _returnvalue (Class|MeleeAttackGameplayAbility|CreateMeleeHitbox _localspaceoffset (Variables|Default|GetHitboxRadius) (Variables|Default|GetKnockback%20Direction) (Variables|Default|GetKnockback%20Force) 60 true))
  (for _array_element _returnvalue
    (CallFunction|HitActor _array_element)))

(event Ability|EventOnEndAbility
  (params (bWasCancelled :type Boolean)))

(fn GetHitboxOffsetinPlayerSpace
  (params (PlayerSceneComponent :type Scene%20Component%20Object%20Reference))
  (return (+ (Transformation|GetWorldLocation PlayerSceneComponent) (* (Math|Vector|VectorLength (Variables|Default|GetHitboxOffset)) (Math|Vector|Normalize (Math|Vector|GetForwardVector PlayerSceneComponent))))))

(fn ApplyKnockbacktoActor
  (params (Actor :type Object%20Object%20Reference))
  (bind _asknockbackable (Utilities|Casting|CastToKnockbackable Actor)
    (:then
      (Class|Knockbackable|ApplyKnockback _asknockbackable (Variables|Default|GetKnockback%20Direction) (Variables|Default|GetKnockback%20Force)))
    (:CastFailed
      (Development|PrintString (LocalVariables|GetWarningText)))))

(fn HitActor
  (params (Actor :type Object%20Object%20Reference))
  (bind _ashittable (Utilities|Casting|CastToHittable Actor)
    (:then
      (Class|Hittable|Hit _ashittable))
    (:CastFailed
      (Development|PrintString (LocalVariables|GetWarningText)))))